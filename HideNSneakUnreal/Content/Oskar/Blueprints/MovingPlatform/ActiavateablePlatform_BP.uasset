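; Platform Blueprint that moves its MovingPlatform component in a straight line from its start toward EndPoint while IsActivated is set.
; Tick steps it along a cached direction by Speed, then clears the flag and disables ticking on arrival.
; Clicking either button retargets to that button's location, but only Button2 recalculates direction.
; The logic that would reactivate it toward the start is unconnected, so nothing here turns activation on.
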(event OnClicked(Button1)
  (params (TouchedComponent :type Primitive%20Component%20Object%20Reference) (ButtonPressed :type Key%20Structure))
  ;[1 1 1] Author: Oskar Johansson
  (Variables|Default|SetTargetPosition (Transformation|GetWorldLocation TouchedComponent)))

(event OnClicked(Button2)
  (params (TouchedComponent :type Primitive%20Component%20Object%20Reference) (ButtonPressed :type Key%20Structure))
  ;[1 1 1] Author: Oskar Johansson
  (CallFunction|SetDirectionandTargetPosition TouchedComponent))

(event EventBeginPlay
  ;[1 1 1] Author: Oskar Johansson
  (bind _output_get (Variables|Default|SetEndPosition (Transformation|GetWorldLocation (Variables|Default|GetEnd_point))))
  (bind _output_get_2 (Variables|Default|SetTargetPosition _output_get))
  (bind _output_get_3 (Variables|Default|SetStartPosition (Transformation|GetWorldLocation (Variables|Default|GetMovingPlatform))))
  (bind _output_get_4 (Variables|Default|SetCurrentPosition _output_get_3))
  (Variables|Default|SetDirection (Math|Vector|Normalize (Math|Vector|GetUnitDirection(Vector) _output_get_4 _output_get_2))))

(event EventTick
  (params (DeltaSeconds :type Float%20%28single-precision%29))
  ;[1 1 1] Author: Oskar Johansson
  (if (Variables|Default|Getis%20activated)
    (bind _output_get (Variables|Default|SetCurrentPosition (Transformation|GetWorldLocation (Variables|Default|GetMovingPlatform))))
    (if (Math|Vector|NotEqual(Vector) _output_get (Variables|Default|GetTargetPosition) 1.0) ; checks if (targetposition == currentposition)
      (Transformation|SetRelativeLocation (Variables|Default|GetMovingPlatform) (+ _output_get (* (Variables|Default|GetDirection) (* (Variables|Default|GetSpeed) DeltaSeconds))) false false)
      (else
        (Variables|Default|Setis%20activated false)
        (Actor|Tick|SetActorTickEnabled false)))))

(fn ConstructionScript)

(fn SetDirectionandTargetPosition
  (params (self2 :type Scene%20Component%20Object%20Reference))
  (bind _output_get (Variables|Default|SetTargetPosition (Transformation|GetWorldLocation self2)))
  (Variables|Default|SetDirection (Math|Vector|Normalize (Math|Vector|GetUnitDirection(Vector) (Variables|Default|GetCurrentPosition) _output_get))))