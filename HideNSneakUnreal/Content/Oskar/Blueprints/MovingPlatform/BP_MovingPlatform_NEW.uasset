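; Moving platform actor that shuttles back and forth between its starting location and an End point, pausing at each end.
; StartPlatform derives speed and direction through MovingPlatform helpers, then after a delay the authority asks BP_RoundController to start the elevator.
; Tick moves the platform while Moving is set; on arrival it swaps target, stops, waits, and the authority requests the next start from the controller.
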(event Custom|StartPlatform
  (bind _movingplatform (Variables|Default|GetMovingPlatform))
  (bind _output_get (Variables|Default|SetStartPosition (Transformation|GetWorldLocation (Variables|Default|GetPlatform))))
  (bind _output_get_2 (Variables|Default|SetEndPosition (Transformation|GetWorldLocation (Variables|Default|GetEnd))))
  (bind _output_get_3 (Variables|Default|SetTargetPosition _output_get_2))
  (bind _returnvalue (Class|MovingPlatform|SetSpeed _movingplatform (Variables|Default|GetTravelTime) (Math|Vector|Distance(Vector) _output_get_2 _output_get)))
  (Variables|Default|SetMovementSpeed _returnvalue)
  (bind _movementvector (Class|MovingPlatform|SetMovementVector _movingplatform _output_get _output_get_3 0.0))
  (Variables|Default|SetMovementVector _movementvector)
  (Utilities|FlowControl|Delay 5.0)
  (if (Ability|HasAuthority)
    (bind _outactors (Actor|GetAllActorsOfClass "/Game/Blueprints/BP_RoundController.BP_RoundController_C"))
    (bind _output_get_4 (Variables|Default|SetRoundController (Utilities|Array|Get(acopy) _outactors)))
    (Default|ServerStartElevator _output_get_4 self)))

(event EventBeginPlay)

(event EventTick
  (params (DeltaSeconds :type Float%20%28single-precision%29))
  (bind _movementspeed (Variables|Default|GetMovementSpeed))
  (if (Variables|Default|GetMoving)
    (bind _output_get (Variables|Default|SetCurrentPosition (Transformation|GetWorldLocation (Variables|Default|GetPlatform))))
    (bind (_targetpositionout _movementvectorout _returnvalue) (Class|MovingPlatform|MovePlatform (Variables|Default|GetMovingPlatform) (Variables|Default|GetTargetPosition) _output_get (Variables|Default|GetEndPosition) (Variables|Default|GetStartPosition) _movementspeed))
    (if _returnvalue
      (Variables|Default|SetTargetPosition _targetpositionout)
      (Variables|Default|SetMovementVector _movementvectorout)
      (Variables|Default|SetMoving false)
      (Utilities|FlowControl|Delay (Variables|Default|GetTime%20at%20ends))
      (if (Ability|HasAuthority)
        (Default|ServerStartElevator (Variables|Default|GetRoundController) self))
      (else
        (Transformation|AddRelativeLocation (Variables|Default|GetPlatform) (* (Variables|Default|GetMovementVector) (* _movementspeed DeltaSeconds)) false false)))))

(fn ConstructionScript)

(fn SetTickandStartPosition
  (params (TargetPosition :type Vector))
  (if (not (Class|Actor|IsActorTickEnabled))
    (Variables|Default|SetTargetPosition TargetPosition)
    (Actor|Tick|SetActorTickEnabled true)))