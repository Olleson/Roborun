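; Elevator platform that travels between its start location and an End marker when the player character overlaps a start, end or platform trigger.
; Triggers enable tick and can set the target; a MovingPlatform helper computes speed from travel time and detects arrival.
; Tick moves the platform along the movement vector, switching off some collision while moving.
; On arrival it adopts the next target, stops ticking, then restores collision after a delay.
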(event OnComponentBeginOverlap(PlayerTouchStart)
  (params (OverlappedComponent :type Primitive%20Component%20Object%20Reference) (OtherActor :type Actor%20Object%20Reference) (OtherComp :type Primitive%20Component%20Object%20Reference) (OtherBodyIndex :type Integer) (bFromSweep :type Boolean) (SweepResult :type Hit%20Result%20Structure%20%28by%20ref%29))
  (Utilities|Casting|CastToHideNSneakCPPCharacter OtherActor)
  (CallFunction|SetTickandStartPosition (Variables|Default|GetStartPosition))
  (Variables|Default|SetMoving true))

(event OnComponentBeginOverlap(PlayerTouchEnd)
  (params (OverlappedComponent :type Primitive%20Component%20Object%20Reference) (OtherActor :type Actor%20Object%20Reference) (OtherComp :type Primitive%20Component%20Object%20Reference) (OtherBodyIndex :type Integer) (bFromSweep :type Boolean) (SweepResult :type Hit%20Result%20Structure%20%28by%20ref%29))
  (Utilities|Casting|CastToHideNSneakCPPCharacter OtherActor)
  (CallFunction|SetTickandStartPosition (Variables|Default|GetEndPosition))
  (Variables|Default|SetMoving true))

(event OnComponentBeginOverlap(PlayerTouchPlatform)
  (params (OverlappedComponent :type Primitive%20Component%20Object%20Reference) (OtherActor :type Actor%20Object%20Reference) (OtherComp :type Primitive%20Component%20Object%20Reference) (OtherBodyIndex :type Integer) (bFromSweep :type Boolean) (SweepResult :type Hit%20Result%20Structure%20%28by%20ref%29))
  (Utilities|Casting|CastToHideNSneakCPPCharacter OtherActor)
  (if (not (Class|Actor|IsActorTickEnabled))
    (Actor|Tick|SetActorTickEnabled true)
    (Variables|Default|SetMoving true)))

(event EventBeginPlay
  (bind _movingplatform (Variables|Default|GetMovingPlatform))
  (bind _output_get (Variables|Default|SetStartPosition (Transformation|GetWorldLocation (Variables|Default|GetPlatform))))
  (bind _output_get_2 (Variables|Default|SetEndPosition (Transformation|GetWorldLocation (Variables|Default|GetEnd))))
  (bind _output_get_3 (Variables|Default|SetTargetPosition _output_get_2))
  (bind _returnvalue (Class|MovingPlatform|SetSpeed _movingplatform (Variables|Default|GetTravelTime) (Math|Vector|Distance(Vector) _output_get _output_get_2)))
  (Variables|Default|SetMovementSpeed _returnvalue)
  (bind _movementvector (Class|MovingPlatform|SetMovementVector _movingplatform _output_get _output_get_3 0.0))
  (Variables|Default|SetMovementVector _movementvector))

(event EventTick
  (params (DeltaSeconds :type Float%20%28single-precision%29))
  (bind _movementspeed (Variables|Default|GetMovementSpeed))
  (if (Variables|Default|GetMoving)
    (CallFunction|TurnOffCollisiononStart/end))
  (bind _output_get (Variables|Default|SetCurrentPosition (Transformation|GetWorldLocation (Variables|Default|GetPlatform))))
  (bind (_targetpositionout _movementvectorout _returnvalue) (Class|MovingPlatform|MovePlatform (Variables|Default|GetMovingPlatform) (Variables|Default|GetTargetPosition) _output_get (Variables|Default|GetEndPosition) (Variables|Default|GetStartPosition) _movementspeed))
  (if _returnvalue
    (Variables|Default|SetTargetPosition _targetpositionout)
    (Variables|Default|SetMovementVector _movementvectorout)
    (Actor|Tick|SetActorTickEnabled false)
    (Utilities|FlowControl|Delay (Variables|Default|GetTime%20at%20ends))
    (Collision|SetCollisionEnabled "QueryAndPhysics")
    (Collision|SetCollisionEnabled "QueryAndPhysics")
    (else
      (Transformation|AddRelativeLocation (Variables|Default|GetPlatform) (* (Variables|Default|GetMovementVector) (* _movementspeed DeltaSeconds)) false false))))

(fn ConstructionScript)

(fn SetTickandStartPosition
  (params (TargetPosition :type Vector))
  (if (not (Class|Actor|IsActorTickEnabled))
    (Variables|Default|SetTargetPosition TargetPosition)
    (Actor|Tick|SetActorTickEnabled true)))

(fn TurnOffCollisiononStart/end
  (Collision|SetCollisionEnabled "NoCollision")
  (Collision|SetCollisionEnabled "NoCollision")
  (Variables|Default|SetMoving false))