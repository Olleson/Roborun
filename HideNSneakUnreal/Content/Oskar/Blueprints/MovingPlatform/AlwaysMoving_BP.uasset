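; AlwaysMoving_BP is a moving platform that continuously shuttles back and forth between its starting position and an EndPoint component.
; BeginPlay caches both world positions and the unit direction toward the end.
; Each Tick offsets MovingPlatform along that direction at Speed, without sweep.
; A dot product detects when the platform passes its target, then flips the direction and swaps the target between start and end.
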(event EventBeginPlay
  ;[1 1 1] Author: Oskar Johansson
  (bind _output_get (Variables|Default|SetEndPosition (Transformation|GetWorldLocation (Variables|Default|GetEndPoint))))
  (bind _output_get_2 (Variables|Default|SetTargetPosition _output_get))
  (bind _output_get_3 (Variables|Default|SetStartPosition (Transformation|GetWorldLocation (Variables|Default|GetMovingPlatform))))
  (bind _output_get_4 (Variables|Default|SetCurrentPosition _output_get_3))
  (Variables|Default|SetDirection (Math|Vector|Normalize (Math|Vector|GetUnitDirection(Vector) _output_get_4 _output_get_2))))

(event EventTick
  (params (DeltaSeconds :type Float%20%28single-precision%29))
  (bind _endposition (Variables|Default|GetEndPosition))
  ;[1 1 1] Author: Oskar Johansson
  (bind _output_get (Variables|Default|SetCurrentPosition (Transformation|GetWorldLocation (Variables|Default|GetMovingPlatform))))
  (if (>= (Math|Vector|DotProduct (- (Variables|Default|GetTargetPosition) _output_get) (Variables|Default|GetDirection)) 0.0) ; checks if (targetposition == currentposition)
    (Transformation|AddWorldOffset (Variables|Default|GetMovingPlatform) (* (Variables|Default|GetDirection) (* (Variables|Default|GetSpeed) DeltaSeconds)) false false)
    (else
      ;;[1 1 1] Changes the direction and target position depending on where it is
      (Variables|Default|SetDirection (* (Variables|Default|GetDirection) -1))
      (if (Math|Vector|Equal(Vector) (Variables|Default|GetTargetPosition) _endposition 1.0)
        (Variables|Default|SetTargetPosition (Variables|Default|GetStartPosition))
        (else
          (Variables|Default|SetTargetPosition _endposition))))))

(fn ConstructionScript)