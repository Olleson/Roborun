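; A returning moving platform that travels toward an end point while its PlayerTouch volume is overlapped and reverses when the overlap ends.
; On BeginPlay it stores the world locations of MovingPlatform and EndPoint.
; Overlap events play or reverse a timeline that lerps between those positions, without filtering the overlapping actor.
; The stored world-space positions are applied through SetRelativeLocation, with no sweep.
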(event OnComponentBeginOverlap(PlayerTouch)
  (params (OverlappedComponent :type Primitive%20Component%20Object%20Reference) (OtherActor :type Actor%20Object%20Reference) (OtherComp :type Primitive%20Component%20Object%20Reference) (OtherBodyIndex :type Integer) (bFromSweep :type Boolean) (SweepResult :type Hit%20Result%20Structure%20%28by%20ref%29))
  ;[1 1 1] Author: Oskar Johansson
  (bind _newtrack_0 (Timeline|Timeline_0 Play)
    (:Update
      (Transformation|SetRelativeLocation (Variables|Default|GetMovingPlatform) (Math|Vector|Lerp(Vector) (Variables|Default|GetStartPosition) (Variables|Default|GetEndPosition) _newtrack_0) false false))))

(event OnComponentEndOverlap(PlayerTouch)
  (params (OverlappedComponent :type Primitive%20Component%20Object%20Reference) (OtherActor :type Actor%20Object%20Reference) (OtherComp :type Primitive%20Component%20Object%20Reference) (OtherBodyIndex :type Integer))
  ;[1 1 1] Author: Oskar Johansson
  (bind _newtrack_0 (Timeline|Timeline_0 Reverse)
    (:Update
      (Transformation|SetRelativeLocation (Variables|Default|GetMovingPlatform) (Math|Vector|Lerp(Vector) (Variables|Default|GetStartPosition) (Variables|Default|GetEndPosition) _newtrack_0) false false))))

(event EventBeginPlay
  ;[1 1 1] Author: Oskar Johansson
  (Variables|Default|SetStartPosition (Transformation|GetWorldLocation (Variables|Default|GetMovingPlatform)))
  (Variables|Default|SetEndPosition (Transformation|GetWorldLocation (Variables|Default|GetEndPoint))))

(fn ConstructionScript)