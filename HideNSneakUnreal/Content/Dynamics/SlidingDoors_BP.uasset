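; Sliding double door actor that opens while a CPP_Character stands in its trigger box.
; Box overlap begin plays the Doors timeline and overlap end reverses it, ignoring other actors.
; The timeline track, scaled by Length, drives the relative Y of LeftDoor and RightDoor in opposite directions.
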(event OnComponentBeginOverlap(Box)
  (params (OverlappedComponent :type Primitive%20Component%20Object%20Reference) (OtherActor :type Actor%20Object%20Reference) (OtherComp :type Primitive%20Component%20Object%20Reference) (OtherBodyIndex :type Integer) (bFromSweep :type Boolean) (SweepResult :type Hit%20Result%20Structure%20%28by%20ref%29))
  (Utilities|Casting|CastToCPP_Character OtherActor)
  (bind _newtrack_0 (Timeline|Doors Play)
    (:Update
      (Transformation|SetRelativeLocation (Variables|Default|GetLeftDoor) (Math|Vector|MakeVector 0.0 (* (* _newtrack_0 (Math|Conversions|ToFloat(Integer) (Variables|Default|GetLength))) -1.0) 0.0) false false)
      (Transformation|SetRelativeLocation (Variables|Default|GetRightDoor) (Math|Vector|MakeVector 0.0 (* _newtrack_0 (Math|Conversions|ToFloat(Integer) (Variables|Default|GetLength))) 0.0) false false))))

(event OnComponentEndOverlap(Box)
  (params (OverlappedComponent :type Primitive%20Component%20Object%20Reference) (OtherActor :type Actor%20Object%20Reference) (OtherComp :type Primitive%20Component%20Object%20Reference) (OtherBodyIndex :type Integer))
  (Utilities|Casting|CastToCPP_Character OtherActor)
  (bind _newtrack_0 (Timeline|Doors Reverse)
    (:Update
      (Transformation|SetRelativeLocation (Variables|Default|GetLeftDoor) (Math|Vector|MakeVector 0.0 (* (* _newtrack_0 (Math|Conversions|ToFloat(Integer) (Variables|Default|GetLength))) -1.0) 0.0) false false)
      (Transformation|SetRelativeLocation (Variables|Default|GetRightDoor) (Math|Vector|MakeVector 0.0 (* _newtrack_0 (Math|Conversions|ToFloat(Integer) (Variables|Default|GetLength))) 0.0) false false))))

(event EventBeginPlay)

(event Collision|EventActorBeginOverlap
  (params (OtherActor :type Actor%20Object%20Reference)))

(event EventTick
  (params (DeltaSeconds :type Float%20%28single-precision%29)))

(fn ConstructionScript)