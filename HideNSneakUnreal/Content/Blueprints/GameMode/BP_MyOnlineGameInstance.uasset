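; BP_MyOnlineGameInstance is a game instance that persists player settings through a BP_SaveSettings save object.
; On Init it creates a default settings object, then loads the saved slot over it, or writes the defaults to a new slot if no valid save is found.
; On Shutdown it saves the current settings object back to the slot, keyed by the first player controller's ID, and prints status messages throughout.
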(event EventInit
  (bind _returnvalue (SaveGame|CreateSaveGameObject "/Game/Blueprints/UI/BP_SaveSettings.BP_SaveSettings_C"))
  (Variables|Default|SetSettingsObj _returnvalue)
  (Development|PrintString "Loading settings...")
  (CallFunction|LoadPlayerSettings))

(event EventShutdown
  (CallFunction|SavePlayerSettings))

(fn SavePlayerSettings
  (bind _returnvalue (SaveGame|SaveGametoSlot (Variables|Default|GetSettingsObj) (Variables|Default|GetSettingsSlotName) (Class|GameplayStatics|GetPlayerControllerID (Game|GetPlayerController 0))))
  (if _returnvalue
    (Development|PrintString "Settings saved successfully!")
    (else
      (Development|PrintString "Error: Failed to save settings"))))

(fn LoadPlayerSettings
  (bind _returnvalue (SaveGame|LoadGamefromSlot (Variables|Default|GetSettingsSlotName) (Class|GameplayStatics|GetPlayerControllerID (Game|GetPlayerController 0))))
  (bind _asbp_save_settings (Utilities|Casting|CastToBP_SaveSettings _returnvalue)
    (:then
      (Variables|Default|SetSettingsObj _asbp_save_settings)
      (Development|PrintString "Settings loaded successfully!"))
    (:CastFailed
      (bind _returnvalue_2 (SaveGame|SaveGametoSlot (Variables|Default|GetSettingsObj) (Variables|Default|GetSettingsSlotName) (Class|GameplayStatics|GetPlayerControllerID (Game|GetPlayerController 0))))
      (if _returnvalue_2
        (Development|PrintString "No Save found. New Save Slot created!")
        (else
          (Development|PrintString "Error: Failed to load settings"))))))