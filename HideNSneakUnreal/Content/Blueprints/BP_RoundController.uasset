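; Round manager for a hide-and-seek game that starts rounds, counts down time and detects when they end.
; On authority, BeginPlay caches a character to host the Start button and stores the round time.
; StartRound checks player count, resets and teleports players, picks a random Seeker, freezes them briefly and starts a looping one-second timer.
; Tick ends rounds when time expires or Hiders hit the minimum, except solo, showing Play Again.
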(event Custom|StartRound
  (bind _randomisedseeker (Variables|Default|GetRandomisedSeeker))
  (bind _randomisedseeker_2 (Variables|Default|GetRandomisedSeeker))
  (bind _charactermovement (Variables|/Script/Engine.Character|GetCharacterMovement _randomisedseeker_2))
  ;[1 1 1] Starts the round, makes a random person the Seeker, starts the timer
  (Utilities|FlowControl|Delay 0.01)
  (CallFunction|StartRound)
  (Utilities|FlowControl|Delay 0.01)
  (if (Utilities|IsValid _randomisedseeker)
    (Class|HideNSneakCPPCharacter|ServerBecomeSeeker _randomisedseeker)
    (Utilities|FlowControl|Sequence
      (:then_0
        (Utilities|Time|SetTimerbyFunctionName 0 "Detract1FromTimerEverySecond" 1.0 true))
      (:then_1
        (if (Class|HideNSneakCPPCharacter|IsSeeker _randomisedseeker_2)
          (Utilities|FlowControl|Sequence
            (:then_0
              (Pawn|Components|CharacterMovement|DisableMovement _charactermovement))
            (:then_1
              (Utilities|FlowControl|Delay (Variables|Default|GetSeekerWaitAtStartTime))
              (Pawn|Components|CharacterMovement|SetMovementMode _charactermovement "MOVE_Walking" 0))))))))

(event Custom|SetStartButton
  (CallFunction|MakeButtonVisible (Variables|/Game/Blueprints/BP_HideNSneakCPPCharacter.BP_HideNSneakCPPCharacter_C|GetThisPlayersStartRoundButton (Variables|Default|GetCharacterWithAuthority))))

(event EventBeginPlay
  (Networking|SwitchHasAuthority
    (:Authority
      (Variables|RoundController|SetOrigimalRoundTime (Variables|RoundController|GetRoundTime))
      (bind _outactors (Actor|GetAllActorsOfClass "/Game/Blueprints/BP_HideNSneakCPPCharacter.BP_HideNSneakCPPCharacter_C"))
      (for _array_element _outactors
        (if (Ability|HasAuthority _array_element)
          (Variables|Default|SetCharacterWithAuthority _array_element)
          (Utilities|FlowControl|Delay 3.0)
          (CallFunction|SetStartButton))))))

(event EventTick
  (params (DeltaSeconds :type Float%20%28single-precision%29))
  (bind _characterwithauthority (Variables|Default|GetCharacterWithAuthority))
  (bind _thisplayersplayagainbutton (Variables|/Game/Blueprints/BP_HideNSneakCPPCharacter.BP_HideNSneakCPPCharacter_C|GetThisPlayersPlayAgainButton _characterwithauthority))
  (if (and (or (< (Variables|RoundController|GetRoundTime) 1) (== (Utilities|Array|Length (Variables|Default|GetHiders)) (Variables|Default|GetMinimumAmountOfPlayers))) (!= (Utilities|Array|Length (Variables|Default|GetPlayers)) 1))
    (Variables|RoundController|SetIsRoundActive false)
    (Widget|SetVisibility _thisplayersplayagainbutton "Visible")
    (Variables|/Script/Engine.PlayerController|SetbShowMouseCursor (Class|GameplayStatics|GetPlayerControllerfromID) true)
    (if (UserInterface|Viewport|IsinViewport _thisplayersplayagainbutton)
      (Widget|SetVisibility _thisplayersplayagainbutton "Visible")
      (else
        (UserInterface|Viewport|AddtoViewport _thisplayersplayagainbutton 0)))))

(fn ConstructionScript)

(fn Detract1fromTimerEverySecond
  ;[1 1 1] Checks if the round is over or not
  (if (Variables|RoundController|GetIsRoundActive)
    ;[1 1 1] Detracts 1 from the Round Time
    (Variables|RoundController|SetRoundTime (- (Variables|RoundController|GetRoundTime) 1))
    (else
      (return))))

(fn MakeButtonVisible
  (params (InputPin :type Start%20Round%20Button%20Object%20Reference))
  (Widget|SetVisibility InputPin "Visible")
  (Variables|/Script/Engine.PlayerController|SetbShowMouseCursor (Class|GameplayStatics|GetPlayerControllerfromID) true)
  (Variables|Default|SetStartRoundButton InputPin)
  (if (UserInterface|Viewport|IsinViewport InputPin)
    (Widget|SetVisibility InputPin "Visible")
    (else
      (UserInterface|Viewport|AddtoViewport InputPin 0))))

(fn RandomisePlayerinArrayPlayers
  (bind _players (Variables|Default|GetPlayers))
  (bind _output_get (Variables|Default|SetRandom%20Number (Math|Random|RandomIntegerinRange 0 (- (Utilities|Array|Length _players) 1))))
  (for (_array_element _array_index) _players
    (if (== _array_index _output_get)
      (bind _asbp_hide_nsneak_cppcharacter (Utilities|Casting|CastToBP_HideNSneakCPPCharacter _array_element))
      (Variables|Default|SetRandomisedSeeker _asbp_hide_nsneak_cppcharacter)))
  (return))

(fn StartRound
  (bind _returnvalue (Utilities|Time|GetGameTimeinSeconds))
  (bind _characterwithauthority (Variables|Default|GetCharacterWithAuthority))
  (if (>= (Utilities|Array|Length (Variables|Default|GetPlayers)) (Variables|Default|GetAmountOfPlayersToStart))
    (Utilities|FlowControl|Sequence
      (:then_0
        (Variables|RoundController|SetRoundTime (Variables|RoundController|GetOrigimalRoundTime)))
      (:then_1
        (Variables|RoundController|SetIsRoundActive true))
      (:then_2
        (bind _asplayer_controller (Utilities|Casting|CastToPlayerController (Pawn|GetController (Variables|Default|GetCharacterWithAuthority))))
        (Variables|/Script/Engine.PlayerController|SetbShowMouseCursor _asplayer_controller false)
        (Class|HideNSneakCPPCharacter|ServerResetPlayerstoHiders _characterwithauthority)
        (Widget|SetVisibility (Variables|/Game/Blueprints/BP_HideNSneakCPPCharacter.BP_HideNSneakCPPCharacter_C|GetThisPlayersStartRoundButton _characterwithauthority) "Collapsed"))
      (:then_3
        (CallFunction|RandomisePlayerinArrayPlayers)
        (Actor|Tick|SetActorTickEnabled true))
      (:then_4
        (for _array_element (Variables|Default|GetPlayers)
          (bind _asbp_hide_nsneak_cppcharacter (Utilities|Casting|CastToBP_HideNSneakCPPCharacter _array_element))
          (Utilities|FlowControl|Sequence
            (:then_0
              (Variables|/Game/Blueprints/BP_HideNSneakCPPCharacter.BP_HideNSneakCPPCharacter_C|SetTimeWhenHiderAbilityCanBeUsed _asbp_hide_nsneak_cppcharacter _returnvalue))
            (:then_1
              (Variables|/Game/Blueprints/BP_HideNSneakCPPCharacter.BP_HideNSneakCPPCharacter_C|SetTimeWhenSeekerAbilityCanBeUsed _asbp_hide_nsneak_cppcharacter _returnvalue))
            (:then_2
              (Transformation|SetActorLocation _asbp_hide_nsneak_cppcharacter (Variables|/Game/Blueprints/BP_HideNSneakCPPCharacter.BP_HideNSneakCPPCharacter_C|GetPlayerSpawnLocation _asbp_hide_nsneak_cppcharacter) false false)
              (Transformation|SetActorRotation _asbp_hide_nsneak_cppcharacter (Variables|/Game/Blueprints/BP_HideNSneakCPPCharacter.BP_HideNSneakCPPCharacter_C|GetPlayerSpawnRotation _asbp_hide_nsneak_cppcharacter)))))))
    (else
      (CallFunction|SetStartButton))))