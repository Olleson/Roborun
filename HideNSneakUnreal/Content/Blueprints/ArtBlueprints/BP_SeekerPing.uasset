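; BP_SeekerPing is a short-lived visual ping: a sphere that animates in scale and material on spawn, then destroys itself.
; The construction script creates a dynamic M_PulseBall instance on material slot 1 and also assigns it to slot 0.
; On BeginPlay, one timeline drives the sphere's world scale from its Size track and the material's Multiplier parameter from its Transparency track.
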(event EventBeginPlay
  (bind (_direction _transparency _size) (Timeline|Timeline_0 Play)
    (:Update
      (Utilities|FlowControl|Sequence
        (:then_0
          (Transformation|SetWorldScale3D (Variables|Default|GetSphere) _size))
        (:then_1
          (Rendering|Material|SetScalarParameterValue (Variables|Default|GetMaterialMultiplier) "Multiplier" _transparency :!class /Script/Engine.MaterialInstanceDynamic))))
    (:Finished
      (Actor|DestroyActor))))

(fn ConstructionScript
  (bind _returnvalue (Rendering|Material|CreateDynamicMaterialInstance (Variables|Default|GetSphere) 1 "/Game/Art/VFX/Shaders/M_PulseBall.M_PulseBall" "None" :!class /Script/Engine.PrimitiveComponent))
  (bind _output_get (Variables|Default|SetMaterialMultiplier _returnvalue))
  (Rendering|Material|SetMaterial (Variables|Default|GetSphere) 0 _output_get))