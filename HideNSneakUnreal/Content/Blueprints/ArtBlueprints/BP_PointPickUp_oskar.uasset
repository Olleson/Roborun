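; Point pickup for the hide-and-seek game that plays a looping animation until a character touches it.
; On overlap it awards points to non-decoy hiders, passing the round controller's score multiplier, but is consumed by any HideNSneak character.
; It then hides, disables collision and fires a nuts-and-bolts particle burst, updating an attractor parameter on Tick so particles home in on the collector before delayed destruction.
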(event OnComponentBeginOverlap(Collider)
  (params (OverlappedComponent :type Primitive%20Component%20Object%20Reference) (OtherActor :type Actor%20Object%20Reference) (OtherComp :type Primitive%20Component%20Object%20Reference) (OtherBodyIndex :type Integer) (bFromSweep :type Boolean) (SweepResult :type Hit%20Result%20Structure%20%28by%20ref%29))
  (bind _p_nutsnboltscollide (Variables|Default|GetP_NutsNBoltsCollide))
  ;[1 1 1] Author: Fredrik Marcus
  ; Co-Author: Oskar Johansson
  ;;[1 1 1] On comp overlap
  (bind _asbp_hide_nsneak_cppcharacter (Utilities|Casting|CastToBP_HideNSneakCPPCharacter OtherActor))
  (Utilities|FlowControl|Sequence
    (:then_0
      ;;;[1 1 1] Check if its a hider and if it is then give him points
      (if (not (Class|HideNSneakCPPCharacter|IsSeeker _asbp_hide_nsneak_cppcharacter))
        (if (not (Variables|/Script/HideNSneakUnreal.HideNSneakCPPCharacter|GetIsDecoy _asbp_hide_nsneak_cppcharacter))
          (Default|AddScore _asbp_hide_nsneak_cppcharacter (Variables|Default|GetPointValue) (Variables|/Script/HideNSneakUnreal.RoundController|GetScoreMultiplier (Variables|Default|GetRoundController))))))
    (:then_1
      ;;;[1 1 1] Set player Reference and start ticking
      (Variables|Default|SetPlayerVar _asbp_hide_nsneak_cppcharacter)
      (Actor|Tick|SetActorTickEnabled true))
    (:then_2
      (Rendering|SetVisibility (Variables|Default|GetI_PointPickUp_anim) false false)
      (Collision|SetCollisionEnabled (Variables|Default|GetCollider) "NoCollision")
      (Components|Activation|Activate _p_nutsnboltscollide false)
      (Effects|Components|ParticleSystem|SetVectorParameter _p_nutsnboltscollide "PointAttractorPos" (Transformation|GetActorLocation (Variables|Default|GetPlayerVar)))
      (Utilities|FlowControl|Delay 5.0)
      (Actor|DestroyActor))))

(event EventBeginPlay
  ;[1 1 1] Author: Fredrik Marcus
  ; Co-Author: Oskar Johansson
  ;;[1 1 1] Get a reference to the roundcontroller and start the animation
  (Utilities|FlowControl|Sequence
    (:then_0
      (bind _outactors (Actor|GetAllActorsOfClass "/Game/Blueprints/BP_RoundController.BP_RoundController_C"))
      (for _array_element _outactors
        (Variables|Default|SetRoundController _array_element)))
    (:then_1
      (Components|Animation|PlayAnimation (Variables|Default|GetI_PointPickUp_anim) "/Game/Art/3D/ACTUALWORLD/PointPickUp/I_PointPickUp_anim_Anim.I_PointPickUp_anim_Anim" true))))

(event EventTick
  (params (DeltaSeconds :type Float%20%28single-precision%29))
  ;[1 1 1] Author: Fredrik Marcus
  ; Co-Author: Oskar Johansson
  ;;[1 1 1] Update the player location in the particle system so the particles comes to the player
  (Effects|Components|ParticleSystem|SetVectorParameter (Variables|Default|GetP_NutsNBoltsCollide) "PointAttractorPos" (Transformation|GetWorldLocation (Variables|/Script/Engine.Actor|GetRootComponent (Variables|Default|GetPlayerVar)))))

(fn ConstructionScript)