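; A placed spawn marker that creates a dummy hider character for training mode in the hide-and-seek game.
; One second after BeginPlay it finds the round controller and checks whether training is on.
; In training it spawns a BP_HideNSneakCPPCharacter at its own transform and adds it to the controller's Hiders list; otherwise it destroys itself.
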(event Custom|SpawnDummy
  (bind _returnvalue (Game|SpawnActorfromClass "/Game/Blueprints/BP_HideNSneakCPPCharacter.BP_HideNSneakCPPCharacter_C" (Transformation|GetActorTransform) "Undefined" 0 0))
  (Utilities|Array|Add (Variables|/Script/HideNSneakUnreal.RoundController|GetHiders (Variables|Default|GetRoundController)) _returnvalue))

(event EventBeginPlay
  (Utilities|FlowControl|Delay 1.0)
  (bind _outactors (Actor|GetAllActorsOfClass "/Game/Blueprints/BP_RoundController.BP_RoundController_C"))
  (bind _output_get (Variables|Default|SetRoundController (Utilities|Array|Get(acopy) _outactors)))
  (if (Variables|/Game/Blueprints/BP_RoundController.BP_RoundController_C|GetIsTraining _output_get) ; If the game is in training mode, spawn a dummy, otherwise delete this actor
    (CallFunction|SpawnDummy)
    (else
      (Actor|DestroyActor))))

(fn ConstructionScript)