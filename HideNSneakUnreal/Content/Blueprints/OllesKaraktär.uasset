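; Player character Blueprint for a hide-and-seek game, switching between hider and seeker roles.
; It registers with the RoundController and creates a play-again button.
; When IsSeeker replicates, it switches team, body colour and speed, and a timeline changes camera boom length toward first person for seekers.
; Seekers press E on a cooldown to temporarily give in-range hiders a see-through-walls material, then restore their dynamic materials.
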(event EventBeginPlay
  ;[1 1 1] Creates a unique play button for each player
  (bind _returnvalue (UserInterface|CreateWidget "/Game/Blueprints/UI/PlayAgainButton.PlayAgainButton_C"))
  (bind _output_get (Variables|Default|SetThisPlayersPlayAgainButton _returnvalue))
  (Widget|SetVisibility _output_get "Collapsed")
  ;[1 1 1] Sets the Round Controller for the character
  (bind _outactors (Actor|GetAllActorsOfClass "/Script/HideNSneakUnreal.RoundController"))
  (for _array_element _outactors
    (bind _output_get_2 (Variables|Default|SetRoundControllerInScene _array_element))
    (Class|RoundController|BPAddHidertoHiderTeam _output_get_2 self)))

(event EventOnRepIsSeeker
  (bind _playermaterial (Variables|Default|GetPlayerMaterial))
  (bind _charactermovement (Variables|Character|GetCharacterMovement))
  ;[1 1 1] Changes colour of character, moves camera to first person
  (if (Variables|Default|GetbIsSeeker)
    (Class|RoundController|BPAddHidertoSeekerTeam (Variables|Default|GetRoundControllerInScene) self)
    (Rendering|Material|SetVectorParameterValue _playermaterial "BodyColor" (Variables|Default|GetSeekerColour) :!class /Script/Engine.MaterialInstanceDynamic)
    (Variables|/Script/Engine.CharacterMovementComponent|SetMaxWalkSpeed _charactermovement (Variables|Default|GetSeekerSpeed))
    (bind _newtrack_0 (Timeline|CameraSwitch Play)
      (:Update
        (Variables|/Script/Engine.SpringArmComponent|SetTargetArmLength (Variables|Default|GetCameraBoom) (Math|Float|Lerp 3e+02 (Variables|Default|GetCameraDistanceAsSeeker) _newtrack_0))))
    (else
      (Class|RoundController|BPAddHidertoHiderTeam (Variables|Default|GetRoundControllerInScene) self)
      (Rendering|Material|SetVectorParameterValue _playermaterial "BodyColor" (Variables|Default|GetHiderColour) :!class /Script/Engine.MaterialInstanceDynamic)
      (Variables|/Script/Engine.CharacterMovementComponent|SetMaxWalkSpeed _charactermovement (Variables|Default|GetHiderSpeed))
      (Timeline|CameraSwitch Reverse))))

(event Input|KeyboardEvents|E
  (params (Key :type Key%20Structure :default "None"))
  (:Pressed
    (if (Class|HideNSneakCPPCharacter|IsSeeker)
      ;[1 1 1] Change Hiders material to one that can be seen through walls, reset back to original after delay
      (Math|Float|CompareFloat (Variables|Default|GetTimeWhenSeekerAbilityCanBeUsed) (Utilities|Time|GetGameTimeinSeconds)
        (:<
          (CallFunction|MakeHidersSeeableThroughWalls)
          (Utilities|FlowControl|Delay (Variables|Default|GetHiderAbilityDuration))
          (CallFunction|SetBackHidersMaterial)
          (Variables|Default|SetTimeWhenSeekerAbilityCanBeUsed (+ (Utilities|Time|GetGameTimeinSeconds) (Variables|Default|GetSeekerAbilityCooldown))))))))

(fn ConstructionScript
  (bind _mesh (Variables|Character|GetMesh))
  ;[1 1 1] Setup dynamic material instance to change color during gameplay
  (bind _returnvalue (Rendering|Material|CreateDynamicMaterialInstance _mesh 0 (Rendering|Material|GetMaterial _mesh 0) "None" :!class /Script/Engine.PrimitiveComponent))
  (Variables|Default|SetPlayerMaterial _returnvalue))

(fn MakeHidersSeeableThroughWalls
  ;[1 1 1] For all Hiders, set their material to M_SeeThroughWalls
  (bind _outactors (Actor|GetAllActorsOfClass "/Game/Blueprints/BP_HideNSneakCPPCharacter.BP_HideNSneakCPPCharacter_C"))
  (for _array_element _outactors
    (if (not (Class|HideNSneakCPPCharacter|IsSeeker _array_element))
      (if (<= (Math|Vector|VectorLength (- (Transformation|GetActorLocation _array_element) (Transformation|GetActorLocation))) (Variables|Default|GetSekerAbilityRange))
        (Rendering|Material|SetMaterial (Variables|/Script/Engine.Character|GetMesh _array_element) 0 "/Game/Art/Materials/M_SeeThroughWalls.M_SeeThroughWalls")))))

(fn SetBackHidersMaterial
  (bind _outactors (Actor|GetAllActorsOfClass "/Game/Blueprints/BP_HideNSneakCPPCharacter.BP_HideNSneakCPPCharacter_C"))
  (for _array_element _outactors
    (Rendering|Material|SetMaterial (Variables|/Script/Engine.Character|GetMesh _array_element) 0 (Variables|/Game/Blueprints/BP_HideNSneakCPPCharacter.BP_HideNSneakCPPCharacter_C|GetPlayerMaterial _array_element))))