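; Player character for a multiplayer hide-and-seek game, playing as hider, seeker or decoy.
; BeginPlay registers it with the RoundController and local UI/minimap; OnRepIsSeeker destroys decoys or awards tag points and swaps speed, animation, materials, lights and camera.
; Hiders deploy decoys; seekers temporarily reveal nearby hiders through walls via material swaps.
; It also handles minimap pings, power-up icons, chat, pause, elevators, emotes and colour-blind modes.
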(event OnComponentHit(CapsuleComponent)
  (params (HitComponent :type Primitive%20Component%20Object%20Reference) (OtherActor :type Actor%20Object%20Reference) (OtherComp :type Primitive%20Component%20Object%20Reference) (NormalImpulse :type Vector :default "0, 0, 0") (Hit :type Hit%20Result%20Structure%20%28by%20ref%29))
  ;[1 1 1 1 50] Author:
  ; Co-Authors:
  ; Secondary Authors: Simon Makdesi
  ;;[1 1 1] changed + set the variable hasnt collided to be true at start
  (bind _asbp_hide_nsneak_cppcharacter (Utilities|Casting|CastToBP_HideNSneakCPPCharacter OtherActor))
  (if (Math|Boolean|ANDBoolean (not (Variables|/Script/HideNSneakUnreal.HideNSneakCPPCharacter|GetbIsSeeker _asbp_hide_nsneak_cppcharacter)) (Variables|Default|GetbIsSeeker) (Variables|Misc.|GetHasntCollidedWithAnotherPlayer))
    (Variables|Misc.|SetHasntCollidedWithAnotherPlayer false)
    (Utilities|FlowControl|Delay 1.0)
    (Variables|Misc.|SetHasntCollidedWithAnotherPlayer true)
    (if (<= (Utilities|Array|Length (Variables|/Script/HideNSneakUnreal.RoundController|GetSeekers (Variables|Misc.|GetRoundControllerInScene))) 3)
      ;;;[1 1 1] almost works it just gived points duoble sometime or the ui doesnt update
      (Variables|Default|SetScore (+ (Variables|Default|GetScore) 6))
      (else
        (Variables|Default|SetScore (+ (Variables|Default|GetScore) 3))))))

(event OnComponentBeginOverlap(Box)
  (params (OverlappedComponent :type Primitive%20Component%20Object%20Reference) (OtherActor :type Actor%20Object%20Reference) (OtherComp :type Primitive%20Component%20Object%20Reference) (OtherBodyIndex :type Integer) (bFromSweep :type Boolean) (SweepResult :type Hit%20Result%20Structure%20%28by%20ref%29))
  ;[1 1 1] Sets Chased face material
  (if (not (Class|HideNSneakCPPCharacter|IsSeeker))
    (bind _asbp_hide_nsneak_cppcharacter (Utilities|Casting|CastToBP_HideNSneakCPPCharacter OtherActor))
    (if (Class|HideNSneakCPPCharacter|IsSeeker _asbp_hide_nsneak_cppcharacter)
      (Rendering|Material|SetMaterial (Variables|Character|GetMesh) 2 "/Game/Art/3D/Character/Material/Faces/Hider/M_Hider_Chased_Face.M_Hider_Chased_Face")
      (Collision|AssignOnComponentEndOverlap (Variables|Default|GetBox) (delegate Custom|OnComponentEndOverlap_Event_0)))))

(event Custom|AddToUI
  (params (WidgetToShow :type User%20Widget%20Class%20Reference))
  ;[1 1 1 1 50] Author:
  ; Co-Authors:
  ; Secondary Authors: Simon Makdesi
  ;;[1 1 1] Add element to player UI
  (bind _returnvalue (UserInterface|CreateWidget WidgetToShow))
  (UserInterface|Viewport|AddtoViewport _returnvalue 0))

(event Custom|PingAllPlayers
  (params (PingDuration :type Float%20%28single-precision%29))
  ;[1 1 1 1 50] Author:
  ; Co-Authors:
  ; Secondary Authors: Simon Makdesi
  ;;[1 1 1] PING
  (bind _uiwidget (CallFunction|GetLocalPlayerUIWidget))
  (Utilities|IsValid _uiwidget
    (:Is%20Valid
      (Default|SetPointOfInterestVisibility (Variables|/Game/Blueprints/Widgets/BPW_Player_UI.BPW_Player_UI_C|GetBPW_Minimap _uiwidget) self true)
      (Utilities|FlowControl|Delay PingDuration)
      (CallFunction|StopPingingAllPlayers))))

(event Custom|ActivateObject
  (params (Elevator :type Elevator%20with%20Buttons%20BP%20Object%20Reference))
  ;[1 1 1 1 50] Author:
  ; Co-Authors:
  ; Secondary Authors: Simon Makdesi
  ;;[1 1 1] Moving platform interaction
  (Variables|Misc.|SetElevatorReference Elevator))

(event Custom|InitializePlayerSettings
  (params (HiderBaseSpeed :type Float%20%28single-precision%29) (SeekerBaseSpeed :type Float%20%28single-precision%29) (PlayerBaseJumpHeight :type Float%20%28single-precision%29))
  ;[1 1 1 1 50] Author:
  ; Co-Authors:
  ; Secondary Authors: Simon Makdesi
  ;;[1 1 1] Initialize Player Settings
  (bind _output_get (Variables|Default|SetHiderBaseSpeed HiderBaseSpeed))
  (Variables|/Script/Engine.CharacterMovementComponent|SetMaxWalkSpeed (Variables|Character|GetCharacterMovement) _output_get)
  (Variables|Default|SetSeekerBaseSpeed SeekerBaseSpeed)
  (bind _output_get_2 (Variables|Default|SetBaseJumpHeight PlayerBaseJumpHeight))
  (Variables|/Script/Engine.CharacterMovementComponent|SetJumpZVelocity (Variables|Character|GetCharacterMovement) _output_get_2))

(event Custom|ClientPingAllPlayers
  (params (PingDuration :type Float%20%28single-precision%29))
  ;[1 1 1 1 50] Author:
  ; Co-Authors:
  ; Secondary Authors: Simon Makdesi
  ;;[1 1 1] PING
  (CallFunction|PingAllPlayers PingDuration))

(event Custom|StopPingingAllPlayers
  ;[1 1 1 1 50] Author:
  ; Co-Authors:
  ; Secondary Authors: Simon Makdesi
  ;;[1 1 1] PING
  (bind _uiwidget (CallFunction|GetLocalPlayerUIWidget))
  (Default|SetPointOfInterestVisibility (Variables|/Game/Blueprints/Widgets/BPW_Player_UI.BPW_Player_UI_C|GetBPW_Minimap _uiwidget) self false))

(event Custom|RemovePauseMenu
  ;[1 1 1 1 50] Author:
  ; Co-Authors:
  ; Secondary Authors: Simon Makdesi
  (bind _foundwidgets (Widget|GetAllWidgetsOfClass "/Game/Blueprints/Widgets/BPW_PauseMenu.BPW_PauseMenu_C" true))
  (Widget|RemovefromParent _foundwidgets)
  (Variables|Misc.|SetIsInPauseMenu false))

(event Custom|RemoveSettingsMenu
  ;[1 1 1 1 50] Author:
  ; Co-Authors:
  ; Secondary Authors: Simon Makdesi
  (bind _foundwidgets (Widget|GetAllWidgetsOfClass "/Game/Blueprints/Widgets/BPW_Settings.BPW_Settings_C" true))
  (Widget|RemovefromParent _foundwidgets))

(event Custom|Spawn%20emitter
  (params (Emitter :type Particle%20System%20Object%20Reference) (Location :type Vector))
  ;[1 1 1 1 50] Author:
  ; Co-Authors:
  ; Secondary Authors: Simon Makdesi
  ;;[1 1 1] Spawn emitter & sound
  (Effects|SpawnEmitteratLocation Emitter Location))

(event Custom|ResetColorBlindMode
  ;[1 1 1 1 50] Author:
  ; Co-Authors:
  ; Secondary Authors: Simon Makdesi
  (Rendering|Material|SetScalarParameterValue "/Game/Materials/ColorBlind_MatParam_Collection.ColorBlind_MatParam_Collection" "CB_Protanopia" 0.0 :!class /Script/Engine.KismetMaterialLibrary)
  (Rendering|Material|SetScalarParameterValue "/Game/Materials/ColorBlind_MatParam_Collection.ColorBlind_MatParam_Collection" "CB_Deuteranopia" 0.0 :!class /Script/Engine.KismetMaterialLibrary)
  (Rendering|Material|SetScalarParameterValue "/Game/Materials/ColorBlind_MatParam_Collection.ColorBlind_MatParam_Collection" "CB_Tritanopia" 0.0 :!class /Script/Engine.KismetMaterialLibrary)
  (Rendering|Material|SetScalarParameterValue "/Game/Materials/ColorBlind_MatParam_Collection.ColorBlind_MatParam_Collection" "CB_Monochromacy" 0.0 :!class /Script/Engine.KismetMaterialLibrary))

(event Custom|Spawn%20sound
  (params (Sound :type Sound%20Base%20Object%20Reference) (Location :type Vector) (VolumeMultiplier :type Float%20%28single-precision%29))
  ;[1 1 1 1 50] Author:
  ; Co-Authors:
  ; Secondary Authors: Simon Makdesi
  ;;[1 1 1] Spawn emitter & sound
  (Audio|SpawnSoundatLocation Sound Location "0, 0, 0" VolumeMultiplier 1.0 0.0 0 0))

(event Custom|MulticastMeshVisibility
  (params (inVisibility :type Boolean))
  (bind _mesh (Variables|Character|GetMesh))
  ;[1 1 1 1 50] Author:
  ; Co-Authors:
  ; Secondary Authors: Simon Makdesi
  ;;[1 1 1] Toggle Mesh Visibility
  (if inVisibility
    (if (Class|HideNSneakCPPCharacter|IsSeeker)
      (Rendering|Material|SetMaterial _mesh 0 "/Game/Art/3D/Character/Material/M_SeekerBody.M_SeekerBody")
      (Rendering|Material|SetMaterial _mesh 1 "/Game/Art/3D/Character/Material/M_Siren.M_Siren")
      (Rendering|Material|SetMaterial _mesh 2 "/Game/Art/3D/Character/Material/Faces/Seeker/M_Seeker_Default_Face.M_Seeker_Default_Face")
      (else
        (Rendering|Material|SetMaterial _mesh 0 "/Game/Art/3D/Character/Material/M_HiderBody.M_HiderBody")
        (Rendering|Material|SetMaterial _mesh 1 "/Game/Art/3D/Character/Material/M_Siren.M_Siren")
        (Rendering|Material|SetMaterial _mesh 2 "/Game/Art/3D/Character/Material/Faces/Hider/M_Hider_Default_Face.M_Hider_Default_Face")))
    (else
      (Rendering|Material|SetMaterial _mesh 0 "/Game/Art/VFX/Shaders/M_Invisibility_1.M_Invisibility_1")
      (Rendering|Material|SetMaterial _mesh 1 "/Game/Art/VFX/Shaders/M_Invisibility_1.M_Invisibility_1")
      (Rendering|Material|SetMaterial _mesh 2 "/Game/Art/VFX/Shaders/M_Invisibility_1.M_Invisibility_1"))))

(event Custom|ServerSendMessage
  (params (Player :type BP%20Hide%20N%20Sneak%20CPP%20Character%20Object%20Reference) (PlayerName :type Text) (Message :type Text))
  ;[1 1 1 1 50] Author:
  ; Co-Authors:
  ; Secondary Authors: Simon Makdesi
  ;;[1 1 1] Owning client replicates players' messages
  (bind _asbp_round_controller (Utilities|Casting|CastToBP_RoundController (Variables|Misc.|GetRoundControllerInScene)))
  (Default|SendMessage _asbp_round_controller Player PlayerName Message))

(event Custom|SetSilentFootsteps_1
  (params (inSilentFootsteps :type Boolean))
  ;[1 1 1 1 50] Author:
  ; Co-Authors:
  ; Secondary Authors: Simon Makdesi
  ;;[1 1 1] Toggles footsteps to be audible or silent
  (bind _ashider_anim_bp (Utilities|Casting|CastToHider_Anim_BP (Components|SkeletalMesh|GetAnimInstance (Variables|Character|GetMesh))))
  (Variables|/Game/Art/3D/Character/Animations/BP/Hider_Anim_BP.Hider_Anim_BP_C|SetHasSilentFootsteps _ashider_anim_bp inSilentFootsteps))

(event Custom|FocusOnGame
  ;[1 1 1 1 50] Author:
  ; Co-Authors:
  ; Secondary Authors: Simon Makdesi
  (Class|WidgetBlueprintLibrary|SetFocustoGameViewport)
  (Input|SetInputModeGameOnly (Game|GetPlayerController 0)))

(event Custom|OnComponentEndOverlap_Event_0
  (params (OverlappedComponent :type Primitive%20Component%20Object%20Reference) (OtherActor :type Actor%20Object%20Reference) (OtherComp :type Primitive%20Component%20Object%20Reference) (OtherBodyIndex :type Integer))
  ;[1 1 1] Sets Chased face material
  (if (not (Class|HideNSneakCPPCharacter|IsSeeker))
    (Rendering|Material|SetMaterial (Variables|Character|GetMesh) 2 "/Game/Art/3D/Character/Material/Faces/Hider/M_Hider_Default_Face.M_Hider_Default_Face")))

(event Custom|Waving
  (CallFunction|Wavingpoop))

(event Custom|Wavingpoop
  (bind _mesh (Variables|Character|GetMesh))
  (bind _returnvalue (Components|SkeletalMesh|GetAnimInstance _mesh))
  ;[1 1 1] Simon Animation för wave emote
  (Utilities|FlowControl|Sequence
    (:then_0
      (bind _ashider_anim_bp (Utilities|Casting|CastToHider_Anim_BP _returnvalue))
      (Variables|/Game/Art/3D/Character/Animations/BP/Hider_Anim_BP.Hider_Anim_BP_C|SetisWaving _ashider_anim_bp true)
      (Utilities|FlowControl|Delay 0.1)
      (Variables|/Game/Art/3D/Character/Animations/BP/Hider_Anim_BP.Hider_Anim_BP_C|SetisWaving _ashider_anim_bp false))
    (:then_1
      (bind _asseeker_anim_bp1 (Utilities|Casting|CastToSeeker_Anim_BP1 _returnvalue))
      (Variables|/Game/Art/3D/Character/Animations/BP/Seeker_Anim_BP1.Seeker_Anim_BP1_C|SetisWaving _asseeker_anim_bp1 true)
      (Utilities|FlowControl|Delay 0.1)
      (Variables|/Game/Art/3D/Character/Animations/BP/Seeker_Anim_BP1.Seeker_Anim_BP1_C|SetisWaving _asseeker_anim_bp1 false))))

(event Custom|ClientStopPingingAllPlayers
  ;[1 1 1 1 50] Author:
  ; Co-Authors:
  ; Secondary Authors: Simon Makdesi
  ;;[1 1 1] PING
  (CallFunction|StopPingingAllPlayers))

(event Custom|ClientUpdatePingIcon
  (params (Icon :type Texture%202D%20Object%20Reference))
  ;[1 1 1 1 50] Author:
  ; Co-Authors:
  ; Secondary Authors: Simon Makdesi
  ;;[1 1 1] PING
  (CallFunction|UpdatePingIcon Icon))

(event Custom|UpdatePingIcon
  (params (Icon :type Texture%202D%20Object%20Reference))
  ;[1 1 1 1 50] Author:
  ; Co-Authors:
  ; Secondary Authors: Simon Makdesi
  ;;[1 1 1] PING
  (CallFunction|SetPingIcon Icon))

(event Custom|ClientSpawnSound
  (params (Sound :type Sound%20Base%20Object%20Reference) (Location :type Vector) (VolumeMultiplier :type Float%20%28single-precision%29))
  ;[1 1 1 1 50] Author:
  ; Co-Authors:
  ; Secondary Authors: Simon Makdesi
  ;;[1 1 1] Spawn emitter & sound
  (CallFunction|SpawnSound Sound Location VolumeMultiplier))

(event Custom|ClientSpawnEmitter
  (params (Emitter :type Particle%20System%20Object%20Reference) (Location :type Vector))
  ;[1 1 1 1 50] Author:
  ; Co-Authors:
  ; Secondary Authors: Simon Makdesi
  ;;[1 1 1] Spawn emitter & sound
  (CallFunction|SpawnEmitter Emitter Location))

(event Custom|TurnOfObject
  ;[1 1 1 1 50] Author:
  ; Co-Authors:
  ; Secondary Authors: Simon Makdesi
  ;;[1 1 1] Moving platform interaction
  (Variables|Misc.|SetElevatorReference 0))

(event Custom|ClientStartElevator
  (params (Elevator :type Elevator%20with%20Buttons%20BP%20Object%20Reference))
  ;[1 1 1 1 50] Author:
  ; Co-Authors:
  ; Secondary Authors: Simon Makdesi
  ;;[1 1 1] Moving platform interaction
  (Default|StarttheElevator Elevator))

(event EventEndPlay
  (params (EndPlayReason :type EEndPlayReason%20Enum :default "Destroyed"))
  ;[1 1 1 1 50] Author:
  ; Co-Authors:
  ; Secondary Authors: Simon Makdesi
  (|RemovePlayerFromPlayersArray))

(event EventTick
  (params (DeltaSeconds :type Float%20%28single-precision%29))
  ;[1 1 1 1 50] Author:
  ; Co-Authors:
  ; Secondary Authors: Simon Makdesi
  (Class|HideNSneakCPPCharacter|MoveDecoy))

(event EventSetMeshVisibility
  (params (inVisibility :type Boolean))
  ;[1 1 1 1 50] Author:
  ; Co-Authors:
  ; Secondary Authors: Simon Makdesi
  ;;[1 1 1] Toggle Mesh Visibility
  (CallFunction|MulticastMeshVisibility inVisibility))

(event EventUpdatePowerUpIcon
  (bind _self self)
  ;[1 1 1 1 50] Author:
  ; Co-Authors:
  ; Secondary Authors: Simon Makdesi
  ;;[1 1 1] Power up icons
  ;;;[1 1 1] Set power up icon
  (bind _asbp_hide_nsneak_cppcharacter (Utilities|Casting|CastToBP_HideNSneakCPPCharacter (Pawn|GetControlledPawn (Game|GetPlayerController 0))))
  (if (== _asbp_hide_nsneak_cppcharacter _self)
    (Default|SetPowerUpIcon (Variables|UI|GetUIWidget _self) (Class|HideNSneakCPPCharacter|GetCollectedPowerUpIcon))))

(event EventOnRepIsSeeker
  (bind _returnvalue (Transformation|GetActorLocation))
  (bind _returnvalue_2 (Game|GetPlayerController 0))
  ;[1 1 1 1 50] Author:
  ; Co-Authors:
  ; Secondary Authors: Simon Makdesi
  ;;[1 1 1] Player state transform + seeker interaction with hiders
  (if (Variables|Default|GetbIsSeeker)
    (if (Variables|Default|GetIsDecoy)
      ;;;[1 1 1] Decoy interaction with seeker
      (CallFunction|SpawnEmitter "/Game/Art/VFX/ParticleSystems/P_DecoyDestruction.P_DecoyDestruction" _returnvalue)
      (CallFunction|SpawnSound "/Game/StarterContent/Audio/Explosion01.Explosion01" _returnvalue 0.1)
      (Actor|DestroyActor)
      (else
        (CallFunction|AddTaggerPoints)
        (Utilities|FlowControl|Sequence
          (:then_0
            (CallFunction|SetPingIcon "/Game/Blueprints/Widgets/Materials/Textures/Skull.Skull")
            (CallFunction|ClientPingAllPlayers 0.0))
          (:then_1
            (CallFunction|TurnIntoSeeker)
            ;;;[1 1 1] Change camera perspective when swapping from between character states
            (bind _newtrack_0 (Timeline|CameraSwitch Play)
              (:Update
                (Variables|/Script/Engine.SpringArmComponent|SetTargetArmLength (Variables|Default|GetCameraBoom) (Math|Float|Lerp (Variables|Seeker|GetCameraDistanceAsSeeker) 3e+02 _newtrack_0)))
              (:Finished
                (bind _asbp_round_controller (Utilities|Casting|CastToBP_RoundController (Variables|Misc.|GetRoundControllerInScene)))
                (if (Math|Boolean|ANDBoolean (not (Variables|Misc.|GetIsPlayer)) (Variables|/Game/Blueprints/BP_RoundController.BP_RoundController_C|GetIsTraining _asbp_round_controller) (Class|HideNSneakCPPCharacter|IsSeeker))
                  (Utilities|FlowControl|Delay (Variables|Misc.|GetDummyResetTime))
                  (CallFunction|TurnIntoHider)))))
          (:then_2
            (Input|DisableInput _returnvalue_2)
            (Utilities|FlowControl|Delay 2.0)
            (Input|EnableInput _returnvalue_2)
            (Class|RoundController|BPAddHidertoSeekerTeam (Variables|Misc.|GetRoundControllerInScene) self)))))
    (else
      (CallFunction|TurnIntoHider)
      (Class|RoundController|BPAddHidertoHiderTeam (Variables|Misc.|GetRoundControllerInScene) self)
      (Timeline|CameraSwitch Reverse))))

(event EventClearPowerUpIcon
  (bind _self self)
  ;[1 1 1 1 50] Author:
  ; Co-Authors:
  ; Secondary Authors: Simon Makdesi
  ;;[1 1 1] Power up icons
  ;;;[1 1 1] Clear power up icon
  (bind _asbp_hide_nsneak_cppcharacter (Utilities|Casting|CastToBP_HideNSneakCPPCharacter (Pawn|GetControlledPawn (Game|GetPlayerController 0))))
  (if (== _asbp_hide_nsneak_cppcharacter _self)
    (Default|ClearPowerUpIcon (Variables|UI|GetUIWidget _self))))

(event EventBeginPlay
  (bind _self self)
  ;[1 1 1 1 50] Author:
  ; Co-Authors:
  ; Secondary Authors: Simon Makdesi
  ;;[1 1 1] On player start
  ;;;[1 1 1] Sets the different variables
  (Variables|Misc.|SetPlayerName (Utilities|String|Append "Player " (Utilities|String|ToString(Integer) (Math|Random|RandomIntegerinRange 1 80))))
  (Rendering|Material|SetVectorParameterValue (Variables|Misc.|GetPlayerMaterial) "BodyColor" (Variables|Hider|GetHiderColour) :!class /Script/Engine.MaterialInstanceDynamic)
  (Variables|Misc.|SetIsPlayer (Pawn|IsPlayerControlled))
  (bind _outactors (Actor|GetAllActorsOfClass "/Script/HideNSneakUnreal.RoundController"))
  (Variables|Misc.|SetRoundControllerInScene (Utilities|Array|Get(acopy) _outactors))
  ;;;[1 1 1] Sets the players' spawn location & rotation, ensures that no other player can have the same spawn values
  (bind _asbp_round_controller (Utilities|Casting|CastToBP_RoundController (Variables|Misc.|GetRoundControllerInScene)))
  (Default|SetSpawnLocation _asbp_round_controller self)
  ;;;[1 1 1] Initialize local player's UI, and add ping widget to other players' minimap widgets
  (bind _asbp_hide_nsneak_cppcharacter (Utilities|Casting|CastToBP_HideNSneakCPPCharacter (Pawn|GetControlledPawn (Game|GetPlayerController 0))))
  (if (== _asbp_hide_nsneak_cppcharacter self)
    (bind _returnvalue (UserInterface|CreateWidget "/Game/Blueprints/Widgets/BPW_Player_UI.BPW_Player_UI_C" 0 _asbp_hide_nsneak_cppcharacter))
    (bind _output_get (Variables|UI|SetUIWidget _returnvalue))
    (UserInterface|Viewport|AddtoViewport _output_get 0))
  (bind _uiwidget (CallFunction|GetLocalPlayerUIWidget))
  (Default|AddPointOfInterest (Variables|/Game/Blueprints/Widgets/BPW_Player_UI.BPW_Player_UI_C|GetBPW_Minimap _uiwidget) self)
  (bind _asbp_round_controller_2 (Utilities|Casting|CastToBP_RoundController (Variables|Misc.|GetRoundControllerInScene)))
  (Utilities|FlowControl|Delay 0.2)
  (if (and (not (Variables|Default|GetIsDecoy)) (not (Variables|/Game/Blueprints/BP_RoundController.BP_RoundController_C|GetIsTraining _asbp_round_controller_2)))
    (Class|RoundController|BPAddHidertoHiderTeam (Variables|Misc.|GetRoundControllerInScene) self)
    (if (and (Utilities|IsValid (Variables|Misc.|GetRoundControllerInScene)) (not (Utilities|Array|ContainsItem (Variables|/Script/HideNSneakUnreal.RoundController|GetPlayers (Variables|Misc.|GetRoundControllerInScene)) _self)))
      (Utilities|Array|Add (Variables|/Script/HideNSneakUnreal.RoundController|GetPlayers (Variables|Misc.|GetRoundControllerInScene)) _self)
      (bind _asbp_round_controller_3 (Utilities|Casting|CastToBP_RoundController (Variables|Misc.|GetRoundControllerInScene)))
      (Default|ShowPlayRoundButton _asbp_round_controller_3 (Variables|/Game/Blueprints/BP_RoundController.BP_RoundController_C|GetCharacterWithAuthority _asbp_round_controller_3)))))

(event Input|ActionEvents|InputActionActivateAbility
  (params (Key :type Key%20Structure :default "None"))
  (bind _returnvalue (Utilities|Time|GetGameTimeinSeconds))
  (bind _self self)
  (bind _returnvalue_2 (Transformation|GetActorLocation _self))
  ;[1 1 1 1 50] Author:
  ; Co-Authors:
  ; Secondary Authors: Simon Makdesi
  ;;[1 1 1] Player abilites
  (:Released
    (bind _uiwidget (CallFunction|GetLocalPlayerUIWidget))
    (Default|PLAYANIM; _uiwidget)
    (if (Class|HideNSneakCPPCharacter|IsSeeker)
      ;;;[1 1 1] Seeker ability, Change Hiders material to one that can be seen through walls, reset back to original after delay
      (Math|Float|CompareFloat (Variables|Seeker|GetTimeWhenSeekerAbilityCanBeUsed) _returnvalue
        (:<
          (if (not (Variables|Seeker|GetUsingSeekerAbility)) ; Check to stop the UI from updating incorrectly
            (CallFunction|MakeHidersSeeableThroughWalls)
            (Utilities|FlowControl|Sequence
              (:then_0
                (Variables|Seeker|SetUsingSeekerAbility true))
              (:then_1
                (Utilities|FlowControl|Delay (Variables|Seeker|GetSeekerAbilityDuration))
                (CallFunction|SetBackHidersMaterial)
                (Utilities|FlowControl|Sequence
                  (:then_0
                    (Variables|Seeker|SetUsingSeekerAbility false))
                  (:then_1
                    (Variables|Seeker|SetTimeWhenSeekerAbilityCanBeUsed (+ (Utilities|Time|GetGameTimeinSeconds) (Variables|Seeker|GetSeekerAbilityCooldown))))))
              (:then_2
                (Variables|Seeker|SetTimeWhenSeekerAbilityStops (+ _returnvalue (Variables|Seeker|GetSeekerAbilityDuration))))))))
      (else
        ;;;[1 1 1] Hider ability
        (if (Variables|Default|GetDecoyAvailible)
          (Variables|Hider|SetTimeWhenHiderAbilityCanBeUsed (+ (Utilities|Time|GetGameTimeinSeconds) (Variables|Default|GetDecoyCooldown)))
          (CallFunction|ClientSpawnEmitter "/Game/Art/VFX/ParticleSystems/P_SmokePuff.P_SmokePuff" _returnvalue_2)
          (Class|FMODBlueprintStatics|PlayEventatLocation "/Game/FMOD/Events/Character_Events/Hider/Decoy_Sounds/Activate_Decoy.Activate_Decoy" (Math|Conversions|ToTransform(Vector) _returnvalue_2))
          (Class|HideNSneakCPPCharacter|UseDecoyAbility))))))

(event Input|ActionEvents|InputActionPause
  (params (Key :type Key%20Structure :default "None"))
  (bind _returnvalue (Game|GetPlayerController 0))
  ;[1 1 1 1 50] Author:
  ; Co-Authors:
  ; Secondary Authors: Simon Makdesi
  (:Released
    (if (Variables|Misc.|GetIsInPauseMenu)
      (CallFunction|RemovePauseMenu)
      (CallFunction|RemoveSettingsMenu)
      (Input|SetInputModeGameOnly _returnvalue)
      (Variables|/Script/Engine.PlayerController|SetbShowMouseCursor _returnvalue false)
      (else
        (bind _returnvalue_2 (Game|ConstructObjectfromClass "/Game/Blueprints/Widgets/BPW_PauseMenu.BPW_PauseMenu_C" (Game|GetPlayerController 0)))
        (UserInterface|Viewport|AddtoViewport _returnvalue_2 1)
        (Variables|Misc.|SetIsInPauseMenu true)
        (Variables|UI|SetPauseMenu _returnvalue_2)
        (Input|SetInputModeGameandUI _returnvalue 0 "DoNotLock" false)
        (Variables|/Script/Engine.PlayerController|SetbShowMouseCursor _returnvalue true)))))

(event Input|ActionEvents|InputActionInteractWithEnvironment
  (params (Key :type Key%20Structure :default "None"))
  ;[1 1 1 1 50] Author:
  ; Co-Authors:
  ; Secondary Authors: Simon Makdesi
  ;;[1 1 1] Moving platform interaction
  (:Released
    (if (Utilities|IsValid (Variables|Misc.|GetElevatorReference))
      (CallFunction|ClientStartElevator (Variables|Misc.|GetElevatorReference)))))

(event Input|ActionEvents|InputActionWaveEmote
  (params (Key :type Key%20Structure :default "None"))
  (:Pressed
    (CallFunction|Waving)))

(event Input|KeyboardEvents|Enter
  (params (Key :type Key%20Structure :default "None"))
  ;[1 1 1 1 50] Author:
  ; Co-Authors:
  ; Secondary Authors: Simon Makdesi
  (:Released
    (bind _uiwidget (CallFunction|GetLocalPlayerUIWidget))
    (if (not (Class|Widget|HasKeyboardFocus (Variables|/Game/Blueprints/Widgets/BPW_Player_UI.BPW_Player_UI_C|GetMessageTextBox _uiwidget)))
      (Input|SetInputModeUIOnly (Game|GetPlayerController 0) (Variables|/Game/Blueprints/Widgets/BPW_Player_UI.BPW_Player_UI_C|GetMessageTextBox _uiwidget) "DoNotLock")
      (Widget|SetVisibility (Variables|/Game/Blueprints/Widgets/BPW_Player_UI.BPW_Player_UI_C|GetTextChatCanvas _uiwidget) "Visible"))))

(event Input|KeyboardEvents|G
  (params (Key :type Key%20Structure :default "None"))
  ;[1 1 1 1 50] Author:
  ; Co-Authors:
  ; Secondary Authors: Simon Makdesi
  ;;[1 1 1] PING
  (:Pressed
    (CallFunction|SpawnSound "/Engine/VREditor/Sounds/UI/Camera_Shutter.Camera_Shutter" (Transformation|GetActorLocation) 0.5)
    (CallFunction|ClientUpdatePingIcon "/Game/Blueprints/Widgets/Materials/Textures/Warning_Icon.Warning_Icon")
    (CallFunction|ClientPingAllPlayers 5.0)))

(fn ConstructionScript
  (bind _mesh (Variables|Character|GetMesh))
  ;[1 1 1] Setup dynamic material instance to change color during gameplay
  (bind _returnvalue (Rendering|Material|CreateDynamicMaterialInstance _mesh 0 (Rendering|Material|GetMaterial _mesh 0) "None" :!class /Script/Engine.PrimitiveComponent))
  (Variables|Misc.|SetPlayerMaterial _returnvalue))

(fn MakeHidersSeeableThroughWalls
  (Game|SpawnActorfromClass "/Game/Blueprints/ArtBlueprints/BP_SeekerPing.BP_SeekerPing_C" (Math|Conversions|ToTransform(Vector) (Transformation|GetActorLocation self)) "Undefined" 0 0)
  ;[1 1 1] For all Hiders, set their material to M_SeeThroughWalls
  (bind _asbp_round_controller (Utilities|Casting|CastToBP_RoundController (Variables|Misc.|GetRoundControllerInScene)))
  (for _array_element (Variables|/Script/HideNSneakUnreal.RoundController|GetHiders _asbp_round_controller)
    (bind _asbp_hide_nsneak_cppcharacter (Utilities|Casting|CastToBP_HideNSneakCPPCharacter _array_element))
    (if (not (Class|HideNSneakCPPCharacter|IsSeeker _asbp_hide_nsneak_cppcharacter))
      (if (<= (Math|Vector|VectorLength (- (Transformation|GetActorLocation _asbp_hide_nsneak_cppcharacter) (Transformation|GetActorLocation))) (Variables|Seeker|GetSekerAbilityRange))
        (Rendering|Material|SetMaterial (Variables|/Script/Engine.Character|GetMesh _asbp_hide_nsneak_cppcharacter) 0 "/Game/Art/VFX/Shaders/MI_SeeThroughWalls.MI_SeeThroughWalls")))))

(fn SetBackHidersMaterial
  (bind _asbp_round_controller (Utilities|Casting|CastToBP_RoundController (Variables|Misc.|GetRoundControllerInScene)))
  (for _array_element (Variables|/Script/HideNSneakUnreal.RoundController|GetHiders _asbp_round_controller)
    (bind _asbp_hide_nsneak_cppcharacter (Utilities|Casting|CastToBP_HideNSneakCPPCharacter _array_element))
    (Rendering|Material|SetMaterial (Variables|/Script/Engine.Character|GetMesh _asbp_hide_nsneak_cppcharacter) 0 (Variables|/Game/Blueprints/BP_HideNSneakCPPCharacter.BP_HideNSneakCPPCharacter_C|GetPlayerMaterial _asbp_hide_nsneak_cppcharacter))))

(fn GetLocalPlayerUIWidget
  (bind _asbp_hide_nsneak_cppcharacter (Utilities|Casting|CastToBP_HideNSneakCPPCharacter (Pawn|GetControlledPawn (Game|GetPlayerController 0))))
  (return (Variables|/Game/Blueprints/BP_HideNSneakCPPCharacter.BP_HideNSneakCPPCharacter_C|GetUIWidget _asbp_hide_nsneak_cppcharacter)))

(fn SetPingIcon
  (params (InputPin :type Texture%202D%20Object%20Reference))
  (bind _uiwidget (CallFunction|GetLocalPlayerUIWidget))
  (if (.ReturnValue (Utilities|Map|Find (Variables|/Game/Blueprints/Widgets/BPW_Minimap.BPW_Minimap_C|GetPointsOfInterestByActors (Variables|/Game/Blueprints/Widgets/BPW_Player_UI.BPW_Player_UI_C|GetBPW_Minimap _uiwidget)) self))
    (Appearance|SetBrushfromTexture (Variables|/Game/Blueprints/Widgets/PointOfInterestWidget_BP.PointOfInterestWidget_BP_C|GetCustomImage (.Value (Utilities|Map|Find (Variables|/Game/Blueprints/Widgets/BPW_Minimap.BPW_Minimap_C|GetPointsOfInterestByActors (Variables|/Game/Blueprints/Widgets/BPW_Player_UI.BPW_Player_UI_C|GetBPW_Minimap _uiwidget)) self))) InputPin false)))

(fn TurnIntoSeeker
  (bind _mesh (Variables|Character|GetMesh))
  (bind _charactermovement (Variables|Character|GetCharacterMovement))
  (if (Utilities|IsValid (Variables|Misc.|GetRoundControllerInScene))
    (Variables|/Script/Engine.CharacterMovementComponent|SetMaxWalkSpeed _charactermovement (Variables|Default|GetSeekerBaseSpeed))
    (Variables|/Script/Engine.CharacterMovementComponent|SetJumpZVelocity _charactermovement 1.1e+03)
    (Variables|Seeker|SetTimeWhenSeekerAbilityCanBeUsed 0.0)
    (Utilities|FlowControl|Sequence
      (:then_0
        (bind _asbp_hide_nsneak_cppcharacter (Utilities|Casting|CastToBP_HideNSneakCPPCharacter (Pawn|GetControlledPawn (Game|GetPlayerController 0))))
        (if (== _asbp_hide_nsneak_cppcharacter self)
          (bind _uiwidget (CallFunction|GetLocalPlayerUIWidget))
          (Widget|SetVisibility (Variables|/Game/Blueprints/Widgets/BPW_Player_UI.BPW_Player_UI_C|GetIMGPowerUpIcon _uiwidget) "Collapsed")
          (Default|STOPANIM _uiwidget)))
      (:then_1
        (Class|SkeletalMeshComponent|SetAnimClass _mesh "/Game/Art/3D/Character/Animations/BP/Seeker_Anim_BP1.Seeker_Anim_BP1_C"))
      (:then_2
        (Rendering|Material|SetMaterial _mesh 0 "/Game/Art/3D/Character/Material/M_SeekerBody.M_SeekerBody"))
      (:then_3
        (Rendering|Material|SetMaterial _mesh 2 "/Game/Art/3D/Character/Material/Faces/Seeker/M_Seeker_Default_Face.M_Seeker_Default_Face"))
      (:then_4
        (Rendering|SetVisibility (Variables|Default|GetSpotLight) true false))
      (:then_5
        (Rendering|SetVisibility (Variables|Default|GetSpotLight1) true false))
      (:then_6
        (return)))))

(fn TurnIntoHider
  (bind _mesh (Variables|Character|GetMesh))
  (bind _charactermovement (Variables|Character|GetCharacterMovement))
  (if (Utilities|IsValid (Variables|Misc.|GetRoundControllerInScene))
    (Variables|/Script/Engine.CharacterMovementComponent|SetMaxWalkSpeed _charactermovement (Variables|Default|GetSeekerBaseSpeed))
    (Variables|/Script/Engine.CharacterMovementComponent|SetJumpZVelocity _charactermovement 1.1e+03)
    (Variables|Seeker|SetTimeWhenSeekerAbilityCanBeUsed 0.0)
    (Utilities|FlowControl|Sequence
      (:then_0
        (bind _asbp_hide_nsneak_cppcharacter (Utilities|Casting|CastToBP_HideNSneakCPPCharacter (Pawn|GetControlledPawn (Game|GetPlayerController 0))))
        (if (== _asbp_hide_nsneak_cppcharacter self)
          (bind _uiwidget (CallFunction|GetLocalPlayerUIWidget))
          (Widget|SetVisibility (Variables|/Game/Blueprints/Widgets/BPW_Player_UI.BPW_Player_UI_C|GetIMGPowerUpIcon _uiwidget) "Visible")
          (Default|STOPANIM _uiwidget)))
      (:then_1
        (Class|SkeletalMeshComponent|SetAnimClass _mesh "/Game/Art/3D/Character/Animations/BP/Hider_Anim_BP.Hider_Anim_BP_C"))
      (:then_2
        (Rendering|Material|SetMaterial _mesh 0 "/Game/Art/3D/Character/Material/M_HiderBody.M_HiderBody"))
      (:then_3
        (Rendering|Material|SetMaterial _mesh 2 "/Game/Art/3D/Character/Material/Faces/Hider/M_Hider_Default_Face.M_Hider_Default_Face"))
      (:then_4
        (Rendering|SetVisibility (Variables|Default|GetSpotLight) false false))
      (:then_5
        (Rendering|SetVisibility (Variables|Default|GetSpotLight1) false false))
      (:then_6
        (return)))))

(fn CheckifinTraining
  (bind _asbp_round_controller (Utilities|Casting|CastToBP_RoundController (Variables|Misc.|GetRoundControllerInScene)))
  (return (Variables|/Game/Blueprints/BP_RoundController.BP_RoundController_C|GetIsTraining _asbp_round_controller)))

(fn SetColorBlindMode
  (params (ColorBlindIndex :type Integer))
  (CallFunction|ResetColorBlindMode)
  (switch int ColorBlindIndex
    (:1
      (Rendering|Material|SetScalarParameterValue "/Game/Materials/ColorBlind_MatParam_Collection.ColorBlind_MatParam_Collection" "CB_Protanopia" 1.0 :!class /Script/Engine.KismetMaterialLibrary))
    (:2
      (Rendering|Material|SetScalarParameterValue "/Game/Materials/ColorBlind_MatParam_Collection.ColorBlind_MatParam_Collection" "CB_Deuteranopia" 1.0 :!class /Script/Engine.KismetMaterialLibrary))
    (:3
      (Rendering|Material|SetScalarParameterValue "/Game/Materials/ColorBlind_MatParam_Collection.ColorBlind_MatParam_Collection" "CB_Tritanopia" 1.0 :!class /Script/Engine.KismetMaterialLibrary))
    (:4
      (Rendering|Material|SetScalarParameterValue "/Game/Materials/ColorBlind_MatParam_Collection.ColorBlind_MatParam_Collection" "CB_Monochromacy" 1.0 :!class /Script/Engine.KismetMaterialLibrary))))

(fn AddTaggerPoints
  (bind _roundcontrollerinscene (Variables|Misc.|GetRoundControllerInScene))
  (bind _whotaggedme (Variables|Default|GetWhoTaggedMe))
  (bind _whotaggedme_2 (Variables|Default|GetWhoTaggedMe))
  (bind _roundcontrollerinscene_2 (Variables|Misc.|GetRoundControllerInScene))
  (bind _scoremultiplier (Variables|/Script/HideNSneakUnreal.RoundController|GetScoreMultiplier _roundcontrollerinscene))
  (if (Utilities|IsValid (Variables|Default|GetWhoTaggedMe))
    (if (>= (Utilities|Array|Length (Variables|/Script/HideNSneakUnreal.RoundController|GetPlayers (Variables|Misc.|GetRoundControllerInScene))) 3)
      (Class|HideNSneakCPPCharacter|ClientAddScore _whotaggedme_2 _whotaggedme_2 2 _scoremultiplier)
      (else
        (Class|HideNSneakCPPCharacter|ClientAddScore _whotaggedme _whotaggedme 1 _scoremultiplier)))
    (for _array_element (Variables|/Script/HideNSneakUnreal.RoundController|GetSeekers (Variables|Misc.|GetRoundControllerInScene))
      (Class|HideNSneakCPPCharacter|ClientAddScore _array_element _array_element (Variables|/Script/HideNSneakUnreal.RoundController|GetTagAssistPoint _roundcontrollerinscene_2) (Variables|/Script/HideNSneakUnreal.RoundController|GetScoreMultiplier _roundcontrollerinscene_2))
      (return))))