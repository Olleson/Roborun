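; Round controller for the multiplayer hide-and-seek game, running rounds from host Play button to end screen, plus a training mode with guide arrow and checklist.
; Round start cycles the Seeker role through a copied player list, teleports players, briefly freezes the Seeker and spawns points and optional powerups.
; A one-second timer counts down while Tick checks time and remaining Hiders, awarding winners and the runner-up before the authority shows end screens.
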(event Custom|ServerStartElevator
  (params (MovPlat :type BP%20Moving%20Platform%20NEW%20Object%20Reference))
  (Variables|/Game/Oskar/Blueprints/MovingPlatform/BP_MovingPlatform_NEW.BP_MovingPlatform_NEW_C|SetMoving MovPlat true))

(event Custom|DisplayInstructions
  ;[1 1 1] Author: Pablo
  (bind _foundwidgets (Widget|GetAllWidgetsOfClass "/Game/Blueprints/Widgets/BPW_Player_UI.BPW_Player_UI_C" true))
  (for _array_element _foundwidgets
    (if (Class|HideNSneakCPPCharacter|IsSeeker (Variables|/Game/Blueprints/Widgets/BPW_Player_UI.BPW_Player_UI_C|GetOwner _array_element))
      (Default|DisplayPopUp _array_element "/Game/Art/Textures/UITextures/SeekerInstructions_800x160.SeekerInstructions_800x160")
      (else
        (Default|DisplayPopUp _array_element "/Game/Art/Textures/UITextures/HiderInstructions_800x160.HiderInstructions_800x160")))))

(event Custom|SendMessage
  (params (Player :type BP%20Hide%20N%20Sneak%20CPP%20Character%20Object%20Reference) (PlayerName :type Text) (Message :type Text))
  ;[1 1 1] Updates chat for all players, closes the chat after X seconds
  (bind _uiwidget (Default|GetLocalPlayerUIWidget Player))
  (Default|UpdateChat _uiwidget (Utilities|Text|ToText(String) (Utilities|String|Append (Utilities|String|ToString(Text) PlayerName) ": " (Utilities|String|ToString(Text) Message))))
  (Utilities|FlowControl|Delay (Variables|Numbers|GetChatOpenTime))
  (Widget|SetVisibility (Variables|/Game/Blueprints/Widgets/BPW_Player_UI.BPW_Player_UI_C|GetTextChatCanvas _uiwidget) "Collapsed"))

(event Custom|SetSpawnLocation
  (params (Char :type BP%20Hide%20N%20Sneak%20CPP%20Character%20Object%20Reference))
  ;[1 1 1] Author: Olle Frid
  ; Sets the spawn locations of the players
  (if (not (Variables|Training|GetIsTraining))
    (Utilities|FlowControl|Sequence
      (:then_0
        (Variables|/Game/Blueprints/BP_HideNSneakCPPCharacter.BP_HideNSneakCPPCharacter_C|SetPlayerSpawnLocation Char (Transformation|GetActorLocation (Utilities|Array|Get(acopy) (Variables|Misc.|GetPlayerStarts) (Variables|Numbers|Getlooper)))))
      (:then_1
        (Variables|/Game/Blueprints/BP_HideNSneakCPPCharacter.BP_HideNSneakCPPCharacter_C|SetPlayerSpawnRotation Char (Transformation|GetActorRotation (Utilities|Array|Get(acopy) (Variables|Misc.|GetPlayerStarts) (Variables|Numbers|Getlooper)))))
      (:then_2
        (Variables|Numbers|Setlooper (+ (Variables|Numbers|Getlooper) 1))))))

(event Custom|SpawnPoint
  (bind _pointspawnlocations (Variables|Misc.|GetPointSpawnLocations))
  (bind _returnvalue (Utilities|Array|Length _pointspawnlocations))
  (bind _returnvalue_2 (- _returnvalue 1))
  (bind _returnvalue_3 (Math|Random|RandomIntegerinRange 0 _returnvalue_2))
  (bind _output (Utilities|Array|Get(acopy) _pointspawnlocations _returnvalue_3))
  (bind _rootcomponent (Variables|/Script/Engine.Actor|GetRootComponent _output))
  (bind _returnvalue_4 (Transformation|GetWorldTransform _rootcomponent))
  ;[1 1 1] Section author: Oskar Johansson
  ; Spawn points in the level
  ; Only spawns 100 units above the pivot point of objects with the actor tag "PointSpawn"
  (for _index (range 1 (Variables|Numbers|GetNumberOfPointsToSpawn))
    (if (Utilities|Array|IsValidIndex _pointspawnlocations _returnvalue_3) :!label _label
      (bind _returnvalue_5 (Game|SpawnActorfromClass "/Game/Blueprints/ArtBlueprints/BP_PointPickUp.BP_PointPickUp_C" (Math|Transform|MakeTransform (+ (.location _returnvalue_4) "0,0.000000,100.000000") (.rotation _returnvalue_4) "1,1,1") "AdjustIfPossibleButDontSpawnIfColliding" 0 0))
      (if (not (Utilities|IsValid _returnvalue_5))
        (goto _label))))
  ;;[1 1 1] Set timers when to spawn the point objects again
  (if (Variables|Booleans|GetMIddlePoint)
    (Utilities|Time|SetTimerbyEvent (delegate Custom|SpawnPoint) (Math|Conversions|ToFloat(Integer) (/ (Variables|Numbers|GetRoundTime) 2)))
    (Variables|Booleans|SetMIddlePoint false)
    (elif (Variables|Booleans|GetLastMinute)
      (Utilities|Time|SetTimerbyEvent (delegate Custom|SpawnPoint) (Math|Conversions|ToFloat(Integer) (- (Variables|Numbers|GetRoundTime) 60)))
      (Variables|Booleans|SetLastMinute false))))

(event Custom|ApplySettingsToAllPlayers
  ;[1 1 1] Apply settings to all players
  (bind _assteam_online_game_instance (Utilities|Casting|CastToSteamOnlineGameInstance (Game|GetGameInstance)))
  (for _array_element (Variables|Default|GetPlayers)
    (bind _asbp_hide_nsneak_cppcharacter (Utilities|Casting|CastToBP_HideNSneakCPPCharacter _array_element))
    (Default|InitializePlayerSettings _asbp_hide_nsneak_cppcharacter (Variables|/Script/HideNSneakUnreal.SteamOnlineGameInstance|GetHidersBaseSpeed _assteam_online_game_instance) (Variables|/Script/HideNSneakUnreal.SteamOnlineGameInstance|GetSeekersBaseSpeed _assteam_online_game_instance) (Variables|/Script/HideNSneakUnreal.SteamOnlineGameInstance|GetHidersBaseJumpHeight _assteam_online_game_instance) (Variables|/Script/HideNSneakUnreal.SteamOnlineGameInstance|GetSeekersBaseJumpHeight _assteam_online_game_instance))))

(event Custom|StartRoundEvent
  (bind _randomisedseeker (Variables|Misc.|GetRandomisedSeeker))
  (bind _randomisedseeker_2 (Variables|Misc.|GetRandomisedSeeker))
  (bind _steamonlinegameinstance (Variables|Default|GetSteamOnlinegameInstance))
  (bind _charactermovement (Variables|/Script/Engine.Character|GetCharacterMovement _randomisedseeker))
  ;[1 1 1] Starts the round, makes a random person the Seeker, starts the timer
  (Utilities|FlowControl|Delay 0.1)
  (|StartRoundGraph
    (:Completed
      (Utilities|FlowControl|Delay 0.2)
      (bind _outactors (Actor|GetAllActorswithTag "PointSpawn"))
      (Variables|Misc.|SetPointSpawnLocations _outactors)
      (if (Ability|HasAuthority)
        (CallFunction|SpawnPoint)
        (if (Utilities|IsValid _randomisedseeker_2)
          (Utilities|FlowControl|Delay 1.0)
          (Audio|SpawnSound2D "/Game/Sounds/SoundCues/RoundOver_Cue.RoundOver_Cue" 0.2 1.0 0.0 0)
          (Class|HideNSneakCPPCharacter|ServerBecomeSeeker _randomisedseeker_2)
          (Utilities|FlowControl|Sequence
            (:then_0
              (Utilities|Time|SetTimerbyFunctionName 0 "Detract1FromTimerEverySecond" 1.0 true)
              (Utilities|FlowControl|Delay 0.5)
              (Variables|Misc.|SettempHiders (Variables|Default|GetHiders))
              (if (Variables|Booleans|Getelevators%20started)
                (Variables|Booleans|Setelevators%20started false)
                (bind _outactors_2 (Actor|GetAllActorsOfClass "/Game/Oskar/Blueprints/MovingPlatform/BP_MovingPlatform_NEW.BP_MovingPlatform_NEW_C"))
                (for _array_element _outactors_2
                  (CallFunction|BeginElevator _array_element))))
            (:then_1
              (Utilities|FlowControl|Sequence
                (:then_0
                  (Pawn|Components|CharacterMovement|DisableMovement _charactermovement)
                  (Variables|Booleans|SetCanRandomisedSeekerMove false))
                (:then_1
                  (Utilities|FlowControl|Delay (Variables|Numbers|GetSeekerWaitAtStartTime))
                  (Pawn|Components|CharacterMovement|SetMovementMode _charactermovement "MOVE_Walking" 0)
                  (Variables|Booleans|SetCanRandomisedSeekerMove true))
                (:then_2
                  (for _array_element_2 (Variables|Default|GetHiders)
                    (if (!= _array_element_2 (Variables|Misc.|GetRandomisedSeeker))
                      (Pawn|Components|CharacterMovement|SetMovementMode (Variables|/Script/Engine.Character|GetCharacterMovement _array_element_2) "MOVE_Walking" 0)
                      (Audio|SpawnSound2D "/Game/Sounds/SoundCues/GameStart_Cue.GameStart_Cue" 0.2 1.0 0.0 0))))
                (:then_3
                  (if (Variables|/Script/HideNSneakUnreal.SteamOnlineGameInstance|GetPowerupsEnabled _steamonlinegameinstance)
                    (bind _outactors_3 (Actor|GetAllActorsOfClass "/Game/Blueprints/PowerUps/PowerUpRandomizer_BP.PowerUpRandomizer_BP_C"))
                    (for _array_element_3 _outactors_3
                      (Variables|/Game/Blueprints/PowerUps/PowerUpRandomizer_BP.PowerUpRandomizer_BP_C|SetRespawnTime _array_element_3 (Variables|/Script/HideNSneakUnreal.SteamOnlineGameInstance|GetPowerupSpawnRate _steamonlinegameinstance))
                      (Default|InitializePowerUp _array_element_3))))))
            (:then_2
              (CallFunction|DisplayInstructions))))))))

(event Custom|BeginElevator
  (params (Platform :type BP%20Moving%20Platform%20NEW%20Object%20Reference))
  (Default|StartPlatform Platform))

(event Custom|Server_Show%20End%20Screen
  ;[1 1 1] Tick
  ;;[1 1 1] Author: Olle Frid
  ;; Shows the end screen for all players, called only from the server client
  (for _array_element (Variables|Default|GetPlayers)
    (bind _asbp_hide_nsneak_cppcharacter (Utilities|Casting|CastToBP_HideNSneakCPPCharacter _array_element))
    (bind _uiwidget (Default|GetLocalPlayerUIWidget _asbp_hide_nsneak_cppcharacter))
    (Default|OnRoundEnd _uiwidget)))

(event EventBeginPlay
  (Utilities|FlowControl|Sequence
    (:then_0
      (Networking|SwitchHasAuthority
        (:Authority
          (Utilities|FlowControl|Sequence
            (:then_0
              (Variables|Numbers|SetOrigimalRoundTime (Variables|Numbers|GetRoundTime)))
            (:then_1
              (bind _outactors (Actor|GetAllActorsOfClass "/Game/Blueprints/BP_HideNSneakCPPCharacter.BP_HideNSneakCPPCharacter_C"))
              (for _array_element _outactors
                (if (Ability|HasAuthority _array_element)
                  ;[1 1 1] Shows the PlayButton for the player with authority
                  (bind _output_get (Variables|Misc.|SetCharacterWithAuthority _array_element))
                  ;;[1 1 1] Check to see if the game should be in training mode or not
                  (bind _returnvalue (Game|GetCurrentLevelName true))
                  (if (Utilities|Enum|Equal(Enum) _returnvalue (Variables|Training|GetTrainingLevelName))
                    (Variables|Training|SetIsTraining true)
                    (bind _outactors_2 (Actor|GetAllActorsOfClass "/Game/Oskar/Blueprints/MovingPlatform/BP_MovingPlatform_NEW.BP_MovingPlatform_NEW_C"))
                    (for _array_element_2 _outactors_2
                      (CallFunction|BeginElevator _array_element_2))
                    (else
                      (Utilities|FlowControl|Delay 3.0)
                      (CallFunction|ShowPlayRoundButton _output_get))))))))))
    (:then_1
      ;[1 1 1] Adds all player starts to an array except for the one called SeekerStart
      (if (not (Variables|Training|GetIsTraining))
        (bind _outactors_3 (Actor|GetAllActorsOfClass "/Script/Engine.PlayerStart"))
        (for _array_element_3 _outactors_3
          (if (Utilities|Enum|NotEqual(Enum) (Utilities|GetDisplayName _array_element_3) (Variables|Misc.|GetSeekerStartName))
            (Utilities|Array|Add (Variables|Misc.|GetPlayerStarts) _array_element_3)
            (else
              (Variables|Misc.|SetSeekerStart _array_element_3))))))
    (:then_2
      ;[1 1 1] Gets and sets arrow related things
      (if (Variables|Training|GetIsTraining)
        (Utilities|FlowControl|Sequence
          (:then_0
            (bind _outactors_4 (Actor|GetAllActorsOfClass "/Game/Blueprints/BP_BoxTriggerForUIElements.BP_BoxTriggerForUIElements_C"))
            (bind _output_get_2 (Variables|Training|SetArrowTargets _outactors_4))
            (Variables|Training|SetCurrentArrowTarget (Utilities|Array|Get(acopy) _output_get_2)))
          (:then_1
            (Rendering|SetVisibility (Variables|/Game/Blueprints/BP_HideNSneakCPPCharacter.BP_HideNSneakCPPCharacter_C|GetArrowChild (Variables|Misc.|GetCharacterWithAuthority)) true false)
            (Actor|Tick|SetActorTickEnabled true))
          (:then_2
            (bind _returnvalue_2 (UserInterface|CreateWidget "/Game/Blueprints/Widgets/BPW_TutorialList.BPW_TutorialList_C" (Class|GameplayStatics|GetPlayerControllerfromID)))
            (bind _output_get_3 (Variables|Training|SetCheckList _returnvalue_2))
            (UserInterface|Viewport|AddtoViewport _output_get_3 0)))))
    (:then_3
      (bind _assteam_online_game_instance (Utilities|Casting|CastToSteamOnlineGameInstance (Game|GetGameInstance)))
      (Variables|Default|SetSteamOnlinegameInstance _assteam_online_game_instance))))

(event EventTick
  (params (DeltaSeconds :type Float%20%28single-precision%29))
  (bind _currentarrowtarget (Variables|Training|GetCurrentArrowTarget))
  (bind _characterwithauthority (Variables|Misc.|GetCharacterWithAuthority))
  (bind _returnvalue (Transformation|GetActorLocation _currentarrowtarget))
  (bind _arrowparent (Variables|/Game/Blueprints/BP_HideNSneakCPPCharacter.BP_HideNSneakCPPCharacter_C|GetArrowParent _characterwithauthority))
  (bind _returnvalue_2 (Transformation|GetWorldLocation _arrowparent))
  (bind _returnvalue_3 (Math|Rotator|FindLookatRotation _returnvalue_2 _returnvalue))
  ;[1 1 1] Tick
  (if (Variables|Training|GetIsTraining)
    ;;[1 1 1] Update arrow rotation
    (Transformation|SetWorldRotation _arrowparent (Math|Rotator|MakeRotator (.roll _returnvalue_3) (.pitch _returnvalue_3) (.yaw _returnvalue_3)) false false)
    (else
      (Utilities|FlowControl|Sequence
        (:then_0
          (if (Math|Boolean|ANDBoolean (or (< (Variables|Numbers|GetRoundTime) 1) (== (Utilities|Array|Length (Variables|Default|GetHiders)) (Variables|Default|GetMinimumAmountOfPlayers))) (!= (Utilities|Array|Length (Variables|Default|GetPlayers)) 1) (Variables|Booleans|GetIsRoundActive))
            (Utilities|FlowControl|Delay 0.5)
            (if (Variables|Booleans|GetIsRoundActive)
              (Variables|Booleans|SetIsRoundActive false)
              (Actor|Tick|SetActorTickEnabled false)
              (for _array_element (Variables|Default|GetHiders)
                (bind _asbp_hide_nsneak_cppcharacter (Utilities|Casting|CastToBP_HideNSneakCPPCharacter _array_element))
                (Default|ClientSpawnEmitter _asbp_hide_nsneak_cppcharacter "/Game/Art/VFX/ParticleSystems/P_Victory.P_Victory" (Transformation|GetActorLocation _asbp_hide_nsneak_cppcharacter))
                (Class|FMODBlueprintStatics|PlayEvent2D "/Game/FMOD/Events/GameState/RoundOver.RoundOver")
                (Class|FMODBlueprintStatics|PlayEventatLocation "/Game/FMOD/Events/GameState/GameWinner.GameWinner" (Math|Conversions|ToTransform(Vector) (Transformation|GetActorLocation _asbp_hide_nsneak_cppcharacter)))
                (Class|HideNSneakCPPCharacter|ClientAddScore _asbp_hide_nsneak_cppcharacter _asbp_hide_nsneak_cppcharacter (Variables|Numbers|GetWinningScore) (Variables|Default|GetScoreMultiplier)))
              (Networking|SwitchHasAuthority
                (:Authority
                  (Variables|Numbers|SetCurrentRound (+ (Variables|Numbers|GetCurrentRound) 1))
                  (CallFunction|ServerShowEndScreen)
                  (for _array_element_2 (Variables|Default|GetSeekers)
                    (Rendering|Material|SetMaterial (Variables|/Script/Engine.Character|GetMesh _array_element_2) 2 "/Game/Art/3D/Character/Material/Faces/Seeker/M_Seeker_Happy_Face.M_Seeker_Happy_Face")))))))
        (:then_1
          (|AddPointsForSecondAndThirdPlace))))))

(fn ConstructionScript)

(fn Detract1fromTimerEverySecond
  ;[1 1 1] Checks if the round is over or not
  (if (Variables|Booleans|GetIsRoundActive)
    ;[1 1 1] Starts the timer if the Seeker can move
    (if (Variables|Booleans|GetCanRandomisedSeekerMove)
      ;[1 1 1] Detracts 1 from the Round Time
      (Variables|Numbers|SetRoundTime (- (Variables|Numbers|GetRoundTime) 1)))
    (else
      (return))))

(fn RandomisePlayerinArrayPlayers
  (bind _playerscopy (Variables|Misc.|GetPlayersCopy))
  (bind _output (Utilities|Array|Get(acopy) _playerscopy))
  ;[1 1 1] Randomises the players into a separate array, Players Copy, sets the randomised seeker to the first element in that array, and then removes it.
  ; If the player have left, remove that element from Players Copy and redo the function.
  ; If Players Copy is empty, redo the function
  (if (Variables|Booleans|GetHaveRandomisedArray)
    _
    (else
      (for _array_element (Variables|Default|GetPlayers)
        (bind _asbp_hide_nsneak_cppcharacter (Utilities|Casting|CastToBP_HideNSneakCPPCharacter _array_element))
        (Utilities|Array|Add _playerscopy _asbp_hide_nsneak_cppcharacter))
      (Variables|Booleans|SetHaveRandomisedArray true)))
  (if (> (Utilities|Array|Length _playerscopy) 0)
    (if (Utilities|Array|ContainsItem (Variables|Default|GetPlayers) _output)
      (Variables|Misc.|SetRandomisedSeeker _output)
      (Utilities|Array|RemoveItem _playerscopy _output)
      (return)
      (else
        (Utilities|Array|RemoveItem _playerscopy _output)
        (CallFunction|RandomisePlayerinArrayPlayers)))
    (else
      (Variables|Booleans|SetHaveRandomisedArray false)
      (CallFunction|RandomisePlayerinArrayPlayers))))

(fn StartRoundFunction
  (bind _returnvalue (Utilities|Time|GetGameTimeinSeconds))
  (bind _characterwithauthority (Variables|Misc.|GetCharacterWithAuthority))
  (bind _characterwithauthority_2 (Variables|Misc.|GetCharacterWithAuthority))
  (if (>= (Utilities|Array|Length (Variables|Default|GetPlayers)) (Variables|Numbers|GetAmountOfPlayersToStartAGame))
    (Utilities|FlowControl|Sequence
      (:then_0
        (Variables|Numbers|SetRoundTime (Variables|Numbers|GetOrigimalRoundTime)))
      (:then_1
        (Variables|Booleans|SetIsRoundActive true)
        (Widget|SetVisibility (Variables|/Game/Blueprints/Widgets/BPW_Player_UI.BPW_Player_UI_C|GetB_LobbySettings (Variables|/Game/Blueprints/BP_HideNSneakCPPCharacter.BP_HideNSneakCPPCharacter_C|GetUIWidget _characterwithauthority)) "Hidden"))
      (:then_2
        (bind _asplayer_controller (Utilities|Casting|CastToPlayerController (Pawn|GetController _characterwithauthority)))
        (Variables|/Script/Engine.PlayerController|SetbShowMouseCursor _asplayer_controller false)
        (Class|HideNSneakCPPCharacter|ServerResetPlayerstoHiders _characterwithauthority_2)
        (CallFunction|HidePlayRoundButton _characterwithauthority_2))
      (:then_3
        (CallFunction|RandomisePlayerinArrayPlayers)
        (Actor|Tick|SetActorTickEnabled true))
      (:then_4
        (for _array_element (Variables|Default|GetPlayers)
          (bind _asbp_hide_nsneak_cppcharacter (Utilities|Casting|CastToBP_HideNSneakCPPCharacter _array_element))
          (Utilities|FlowControl|Sequence
            (:then_0
              (Variables|/Game/Blueprints/BP_HideNSneakCPPCharacter.BP_HideNSneakCPPCharacter_C|SetTimeWhenHiderAbilityCanBeUsed _asbp_hide_nsneak_cppcharacter _returnvalue))
            (:then_1
              (Variables|/Game/Blueprints/BP_HideNSneakCPPCharacter.BP_HideNSneakCPPCharacter_C|SetTimeWhenSeekerAbilityCanBeUsed _asbp_hide_nsneak_cppcharacter _returnvalue))
            (:then_2
              (if (!= (Variables|Misc.|GetRandomisedSeeker) _asbp_hide_nsneak_cppcharacter)
                (Transformation|SetActorTransform _asbp_hide_nsneak_cppcharacter (Math|Transform|MakeTransform (Variables|/Game/Blueprints/BP_HideNSneakCPPCharacter.BP_HideNSneakCPPCharacter_C|GetPlayerSpawnLocation _asbp_hide_nsneak_cppcharacter) (Variables|/Game/Blueprints/BP_HideNSneakCPPCharacter.BP_HideNSneakCPPCharacter_C|GetPlayerSpawnRotation _asbp_hide_nsneak_cppcharacter) "1,1,1"))
                (else
                  (Transformation|SetActorTransform _asbp_hide_nsneak_cppcharacter (Transformation|GetActorTransform (Variables|Misc.|GetSeekerStart))))))))))))

(fn ShowPlayRoundButton
  (params (GameMaster :type BP%20Hide%20N%20Sneak%20CPP%20Character%20Object%20Reference))
  (if (Math|Boolean|ANDBoolean (>= (Utilities|Array|Length (Variables|Default|GetPlayers)) (Variables|Numbers|GetAmountOfPlayersToStartAGame)) (not (Variables|Booleans|GetIsRoundActive)) (Utilities|IsValid GameMaster))
    (bind _uiwidget (Default|GetLocalPlayerUIWidget GameMaster))
    (if (not (Widget|IsVisible (Variables|/Game/Blueprints/Widgets/BPW_Player_UI.BPW_Player_UI_C|GetPlayButton _uiwidget)))
      (Widget|SetVisibility (Variables|/Game/Blueprints/Widgets/BPW_Player_UI.BPW_Player_UI_C|GetPlayButton _uiwidget) "Visible")
      (Variables|/Script/Engine.PlayerController|SetbShowMouseCursor (Class|GameplayStatics|GetPlayerControllerfromID) true))))

(fn HidePlayRoundButton
  (params (Game%20Master :type BP%20Hide%20N%20Sneak%20CPP%20Character%20Object%20Reference))
  (if (Utilities|IsValid Game%20Master)
    (bind _uiwidget (Default|GetLocalPlayerUIWidget Game%20Master))
    (Widget|SetVisibility (Variables|/Game/Blueprints/Widgets/BPW_Player_UI.BPW_Player_UI_C|GetPlayButton _uiwidget) "Collapsed")
    (Variables|/Script/Engine.PlayerController|SetbShowMouseCursor (Class|GameplayStatics|GetPlayerControllerfromID) false)))