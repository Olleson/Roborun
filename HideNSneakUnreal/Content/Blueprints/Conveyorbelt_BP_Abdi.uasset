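; Spline-based conveyor belt whose surface is a loop of moving BeltPart_BP actors.
; The construction script tiles spline meshes along the spline, sizing sections by forward-axis bounds, with an optional end mesh.
; BeginPlay spawns flattened parts at overlapping intervals.
; Tick advances each by Speed plus DeltaSeconds (not multiplied) and snaps it to the spline, wrapping to the start with collision switched off at the jump.
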(event Custom|Populatebelt
  (while (< (Variables|Default|GetCurrentposition) (Variables|Default|GetSplineLength))
    (CallFunction|SpawnObject (Variables|Default|GetCurrentposition))
    (Variables|Default|SetCurrentposition (+ (- (Variables|Default|GetSize) (Variables|Default|GetOverlap)) (Variables|Default|GetCurrentposition))))
  (Actor|Tick|SetActorTickEnabled true))

(event Custom|SpawnObject
  (params (SpawnPosition :type Float%20%28single-precision%29))
  (bind _spline (Variables|Default|GetSpline))
  (bind _returnvalue (Game|SpawnActorfromClass "/Game/Blueprints/BeltPart_BP.BeltPart_BP_C" (Math|Transform|MakeTransform (Spline|GetLocationatDistanceAlongSpline _spline SpawnPosition "World") (Math|Rotator|MakeRotator 0.0 1.0 (.yaw (Spline|GetRotationatDistanceAlongSpline _spline SpawnPosition "World"))) "1.900000,1.900000,0.010000") "AlwaysSpawn" 0 0))
  (if (Utilities|IsValid _returnvalue)
    (bind _output_get (Variables|/Game/Blueprints/BeltPart_BP.BeltPart_BP_C|SetSpawnAtPosOnSpline _returnvalue SpawnPosition))
    (Variables|/Game/Blueprints/BeltPart_BP.BeltPart_BP_C|SetCurrentLocation _returnvalue _output_get)
    (Utilities|Array|Add (Variables|Default|GetBeltParts) _returnvalue)))

(event EventBeginPlay
  (Variables|Default|SetSplineLength (Spline|GetSplineLength (Variables|Default|GetSpline)))
  (Variables|Default|SetSize 1.9e+02)
  (CallFunction|Populatebelt))

(event EventTick
  (params (DeltaSeconds :type Float%20%28single-precision%29))
  (bind _spline (Variables|Default|GetSpline))
  (for _array_element (Variables|Default|GetBeltParts)
    (bind _asbelt_part_bp (Utilities|Casting|CastToBeltPart_BP _array_element))
    (if (> (+ (+ DeltaSeconds (Variables|Default|GetSpeed)) (Variables|/Game/Blueprints/BeltPart_BP.BeltPart_BP_C|GetCurrentLocation _asbelt_part_bp)) (Variables|Default|GetSplineLength))
      (Variables|/Game/Blueprints/BeltPart_BP.BeltPart_BP_C|SetCurrentLocation _asbelt_part_bp 0.0)
      (Collision|SetActorEnableCollision _array_element false)
      (Utilities|FlowControl|Delay 0.1)
      (else
        (Variables|/Game/Blueprints/BeltPart_BP.BeltPart_BP_C|SetCurrentLocation _asbelt_part_bp (+ (+ DeltaSeconds (Variables|Default|GetSpeed)) (Variables|/Game/Blueprints/BeltPart_BP.BeltPart_BP_C|GetCurrentLocation _asbelt_part_bp)))))
    (if (Utilities|IsValid (Variables|/Script/Engine.Actor|GetRootComponent _array_element))
      (Transformation|SetWorldLocationAndRotation (Variables|/Script/Engine.Actor|GetRootComponent _array_element) (Math|Vector|MakeVector (.x (Spline|GetLocationatDistanceAlongSpline _spline (Variables|/Game/Blueprints/BeltPart_BP.BeltPart_BP_C|GetCurrentLocation _asbelt_part_bp) "World")) (.y (Spline|GetLocationatDistanceAlongSpline _spline (Variables|/Game/Blueprints/BeltPart_BP.BeltPart_BP_C|GetCurrentLocation _asbelt_part_bp) "World")) (+ (.z (Spline|GetLocationatDistanceAlongSpline _spline (Variables|/Game/Blueprints/BeltPart_BP.BeltPart_BP_C|GetCurrentLocation _asbelt_part_bp) "World")) 8.0)) (Spline|GetRotationatDistanceAlongSpline _spline (Variables|/Game/Blueprints/BeltPart_BP.BeltPart_BP_C|GetCurrentLocation _asbelt_part_bp) "World") false false)
      (Collision|SetActorEnableCollision _array_element true))))

(fn ConstructionScript
  (bind _mesh (Variables|Default|GetMesh))
  (bind _endmesh (Variables|Default|GetEndMesh))
  (bind _spline (Variables|Default|GetSpline))
  (bind _returnvalue (StaticMesh|GetBoundingBox _mesh))
  (Variables|Default|SetSplineLength (Spline|GetSplineLength (Variables|Default|GetSpline)))
  (if (Utilities|IsValid (Variables|Default|GetMesh))
    (if (Utilities|Enum|Equal(Enum) (Utilities|String|ToString(Byte) (Variables|Default|GetForward%20axis)) "0")
      (Variables|Default|SetSectionLength (.x (.max _returnvalue)))
      (for _index (range 0 (- (Math|Float|Truncate (/ (Variables|Default|GetSplineLength) (Variables|Default|GetSectionLength))) 1)) :!label _label
        (bind _returnvalue_2 (AddComponent|AddSplineMeshComponent false))
        (if (Utilities|IsValid _endmesh)
          (if (== _index (- (Math|Float|Truncate (/ (Variables|Default|GetSplineLength) (Variables|Default|GetSectionLength))) 1))
            (Components|StaticMesh|SetStaticMesh _returnvalue_2 _endmesh)
            (else
              (Components|StaticMesh|SetStaticMesh _returnvalue_2 (Variables|Default|GetMesh) :!label _label_2)))
          (else
            (goto _label_2)))
        (SplineMesh|SetForwardAxis _returnvalue_2 (Variables|Default|GetForward%20axis) true)
        (SplineMesh|SetStartandEnd _returnvalue_2 (Spline|GetLocationatDistanceAlongSpline _spline (* _index (Variables|Default|GetSectionLength)) "Local") (Math|Vector|ClampVectorSize (Spline|GetTangentatDistanceAlongSpline _spline (* _index (Variables|Default|GetSectionLength)) "Local") 0.0 (Variables|Default|GetSectionLength)) (Spline|GetLocationatDistanceAlongSpline _spline (* (+ _index 1) (Variables|Default|GetSectionLength)) "Local") (Math|Vector|ClampVectorSize (Spline|GetTangentatDistanceAlongSpline _spline (* (+ _index 1) (Variables|Default|GetSectionLength)) "Local") 0.0 (Variables|Default|GetSectionLength)) true :!class /Script/Engine.SplineMeshComponent)
        (Collision|SetCollisionEnabled _returnvalue_2 "QueryAndPhysics"))
      (elif (Utilities|Enum|Equal(Enum) (Utilities|String|ToString(Byte) (Variables|Default|GetForward%20axis)) "1")
        (Variables|Default|SetSectionLength (.y (.max _returnvalue)))
        (goto _label)
        (elif true
          (Variables|Default|SetSectionLength (.z (.max _returnvalue)))
          (goto _label))))))