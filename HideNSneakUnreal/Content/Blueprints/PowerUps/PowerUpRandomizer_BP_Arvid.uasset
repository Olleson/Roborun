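; Power-up spawner actor that spawns a random pickup class from its array at its own transform.
; InitializePowerUp caches the RoundController and starts a delayed spawn, registering each spawned pickup in the controller's PickUps list.
; The pickup's picked-up delegate restarts the RespawnTime delay, forming a continuous respawn loop.
; Index selection is a separate event, commented as server-side, followed by a short delay before spawning.
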(event Custom|SpawnPowerUp
  (bind _self self)
  ;[1 1 1] Author: Oskar Johansson
  ; Co-Authors: Alexander Aulin, Olle Frid
  ;;[1 1 1] Spawn a powerup at the loctaion of this actor
  (CallFunction|DeterminePowerUpArrayIndex)
  (Utilities|FlowControl|Delay 0.2)
  ;;;[1 1 1] Spawn a powerup and set the currentPowerUp to be a reference to the spawned one
  (bind _returnvalue (Game|SpawnActorfromClass (Utilities|Array|Get(acopy) (Variables|Default|GetPowerUpArray) (Variables|Default|GetPowerUpIndex)) (Transformation|GetWorldTransform (Variables|Default|GetDefaultSceneRoot _self)) "AlwaysSpawn" _self 0))
  (bind _aspickup (Utilities|Casting|CastToPickup _returnvalue))
  (bind _output_get (Variables|Default|SetCurrentPowerUp _aspickup))
  (EventDispatchers|BindEventtoPickedUpDelegate _output_get (delegate Custom|SpawnNewPowerUp))
  (Utilities|Array|Add (Variables|/Game/Blueprints/BP_RoundController.BP_RoundController_C|GetPickUps (Variables|Default|GetRoundController)) _returnvalue))

(event Custom|DeterminePowerUpArrayIndex
  (bind _poweruparray (Variables|Default|GetPowerUpArray))
  (bind _returnvalue (Utilities|Array|Length _poweruparray))
  (bind _returnvalue_2 (Math|Random|RandomInteger _returnvalue))
  ;[1 1 1] Author: Oskar Johansson
  ; Co-Authors: Alexander Aulin, Olle Frid
  ;;[1 1 1] Randomly choose which powerup to spawn on the server, hopefully this will sync up with the clients
  (if (Utilities|Array|IsValidIndex _poweruparray _returnvalue_2)
    (Variables|Default|SetPowerUpIndex _returnvalue_2)))

(event Custom|InitializePowerUp
  ;[1 1 1] Author: Oskar Johansson
  ; Co-Authors: Alexander Aulin, Olle Frid
  ;;[1 1 1] Begin play
  (CallFunction|SpawnNewPowerUp)
  (bind _outactors (Actor|GetAllActorsOfClass "/Game/Blueprints/BP_RoundController.BP_RoundController_C"))
  (Variables|Default|SetRoundController (Utilities|Array|Get(acopy) _outactors)))

(event Custom|SpawnNewPowerUp
  ;[1 1 1] Author: Oskar Johansson
  ; Co-Authors: Alexander Aulin, Olle Frid
  ;;[1 1 1] Spawn a powerup at the loctaion of this actor
  ;;;[1 1 1] Spawns a new powerUp after a set delay
  (Utilities|FlowControl|Delay (Variables|Default|GetRespawnTime))
  (CallFunction|SpawnPowerUp))

(fn ConstructionScript)