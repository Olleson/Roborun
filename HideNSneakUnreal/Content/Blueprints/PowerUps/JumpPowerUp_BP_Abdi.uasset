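; Jump power-up pickup Blueprint that handles the visual and audio presentation of spawning and being picked up.
; On spawn, a separate animated mesh plays for a second, then gives way to the looping idle mesh and particles.
; On pickup, it hides the mesh, plays a sound and runs a one-second collect effect, which Tick steers toward the instigator through a point-attraction parameter.
; BeginPlay repositions the box component to work around incorrect placement.
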(event EventBeginPlay
  ;[1 1 1] I can't get the damn box to spawn in the correct location, this fixes that
  (Transformation|SetRelativeLocation (Variables|Default|GetBoxComponent) "0, 0,70.000000" false true))

(event Collision|EventActorBeginOverlap
  (params (OtherActor :type Actor%20Object%20Reference)))

(event EventTick
  (params (DeltaSeconds :type Float%20%28single-precision%29))
  (bind _pickupinstigator (Variables|Default|GetPickupInstigator))
  (if (Components|Activation|IsActive (Variables|Default|GetP_NutsNBoltsCollide))
    (Utilities|IsValid _pickupinstigator
      (:Is%20Valid
        (Effects|Components|ParticleSystem|SetVectorParameter (Variables|Default|GetP_NutsNBoltsCollide) "PointAttractionPos" (Transformation|GetActorLocation _pickupinstigator))))))

(event EventOnSpawn
  (bind _skeletalmeshcomponent (Variables|Default|GetSkeletalMeshComponent))
  (bind _spawnmesh (Variables|Default|GetSpawnMesh))
  ;[1 1 1] Use this to set up functionality for when the powerup is spawned
  (Rendering|SetVisibility (Variables|Default|GetSkeletalMeshComponent) false false)
  (Components|Activation|Activate (Variables|Default|GetP_NutsNBoltsSpawn) false)
  (Rendering|SetVisibility _spawnmesh true false)
  (Components|Animation|PlayAnimation _spawnmesh "/Game/Art/3D/ACTUALWORLD/PowerUp/PowerUpSpawn/I_PowerUp_Spawn_anim_Anim.I_PowerUp_Spawn_anim_Anim" false)
  (Utilities|FlowControl|Delay 1.0)
  (Rendering|SetVisibility _spawnmesh false false)
  (Rendering|SetVisibility _skeletalmeshcomponent true false)
  (Components|Animation|PlayAnimation _skeletalmeshcomponent "/Game/Art/3D/ACTUALWORLD/PowerUp/PowerUpIdle/I_PowerUp_Idle_anim_Anim.I_PowerUp_Idle_anim_Anim" true)
  (Components|Activation|Activate (Variables|Default|GetP_NutsNBolts) false)
  (Components|Activation|Deactivate (Variables|Default|GetP_NutsNBoltsCollide)))

(event EventOnPickedUp
  (bind _skeletalmeshcomponent (Variables|Default|GetSkeletalMeshComponent))
  (bind _p_nutsnboltscollide (Variables|Default|GetP_NutsNBoltsCollide))
  ;[1 1 1] Use this to set up functionality for when the powerup is picked up
  (Rendering|SetVisibility _skeletalmeshcomponent false false)
  (Components|Activation|Deactivate (Variables|Default|GetP_NutsNBolts))
  (Components|Activation|Activate _p_nutsnboltscollide false)
  (Class|FMODBlueprintStatics|PlayEventatLocation "/Game/FMOD/Events/Character_Events/Pickup_Sounds/Pickup_the_pickup.Pickup_the_pickup" (Transformation|GetWorldTransform _skeletalmeshcomponent))
  (Utilities|FlowControl|Delay 1.0)
  (Components|Activation|Deactivate _p_nutsnboltscollide))

(fn ConstructionScript)