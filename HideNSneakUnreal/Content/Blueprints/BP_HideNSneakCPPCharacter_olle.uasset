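; Player character for a hide-and-seek game, switching between hider and seeker roles registered with the RoundController.
; BeginPlay sets up the local UI, minimap markers and authority-only round buttons.
; OnRepIsSeeker swaps team, color, speed and camera distance; TurnIntoHider and TurnIntoSeeker do the opposite of their names.
; E triggers the hider decoy or a timed seeker see-through-walls material on nearby hiders, while G pings the minimap.
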(event Custom|ClientPingAllPlayers
  (params (PingDuration :type Float%20%28single-precision%29))
  ;[1 1 1] PING
  (CallFunction|PingAllPlayers PingDuration))

(event Custom|PingAllPlayers
  (params (PingDuration :type Float%20%28single-precision%29))
  ;[1 1 1] Initialize local player's UI, and add ping widget to other players' minimap widgets
  (Default|SetPointOfInterestVisibility (Variables|/Game/Blueprints/Widgets/BPW_Player_UI.BPW_Player_UI_C|GetBPW_Minimap (Variables|/Game/Blueprints/BP_HideNSneakCPPCharacter.BP_HideNSneakCPPCharacter_C|GetUIWidget (stale EventBeginPlay _asbp_hide_nsneak_cppcharacter))) self true)
  (Utilities|FlowControl|Delay PingDuration)
  (CallFunction|StopPingingAllPlayers))

(event Custom|StopPingingAllPlayers
  ;[1 1 1] Initialize local player's UI, and add ping widget to other players' minimap widgets
  (Default|SetPointOfInterestVisibility (Variables|/Game/Blueprints/Widgets/BPW_Player_UI.BPW_Player_UI_C|GetBPW_Minimap (Variables|/Game/Blueprints/BP_HideNSneakCPPCharacter.BP_HideNSneakCPPCharacter_C|GetUIWidget (stale EventBeginPlay _asbp_hide_nsneak_cppcharacter))) self false))

(event Custom|ClientStopPingingAllPlayers
  ;[1 1 1] PING
  (CallFunction|StopPingingAllPlayers))

(event Custom|ClientUpdatePingIcon
  (params (Icon :type Texture%202D%20Object%20Reference))
  ;[1 1 1] PING
  (CallFunction|UpdatePingIcon Icon))

(event Custom|UpdatePingIcon
  (params (Icon :type Texture%202D%20Object%20Reference))
  ;[1 1 1] PING
  (CallFunction|SetPingIcon Icon))

(event EventBeginPlay
  (Utilities|FlowControl|Sequence
    (:then_0
      ;[1 1 1] Initialize local player's UI, and add ping widget to other players' minimap widgets
      (bind _asbp_hide_nsneak_cppcharacter (Utilities|Casting|CastToBP_HideNSneakCPPCharacter (Pawn|GetControlledPawn (Game|GetPlayerController 0))))
      (Utilities|FlowControl|Sequence
        (:then_0
          (if (not (Variables|/Game/Blueprints/BP_HideNSneakCPPCharacter.BP_HideNSneakCPPCharacter_C|GetHasWidget _asbp_hide_nsneak_cppcharacter))
            (Variables|/Game/Blueprints/BP_HideNSneakCPPCharacter.BP_HideNSneakCPPCharacter_C|SetHasWidget _asbp_hide_nsneak_cppcharacter true)
            (bind _returnvalue (UserInterface|CreateWidget "/Game/Blueprints/Widgets/BPW_Player_UI.BPW_Player_UI_C" 0 _asbp_hide_nsneak_cppcharacter))
            (bind _output_get (Variables|Default|SetUIWidget _returnvalue))
            (UserInterface|Viewport|AddtoViewport _output_get 0)))
        (:then_1
          (Default|AddPointOfInterest (Variables|/Game/Blueprints/Widgets/BPW_Player_UI.BPW_Player_UI_C|GetBPW_Minimap (Variables|/Game/Blueprints/BP_HideNSneakCPPCharacter.BP_HideNSneakCPPCharacter_C|GetUIWidget _asbp_hide_nsneak_cppcharacter)) self))))
    (:then_1
      (Rendering|Material|SetVectorParameterValue (Variables|Default|GetPlayerMaterial) "BodyColor" (Variables|Default|GetHiderColour) :!class /Script/Engine.MaterialInstanceDynamic)
      (if (Ability|HasAuthority)
        (Utilities|FlowControl|Sequence
          (:then_0
            ;[1 1 1] Creates a unique play button for each player with authority
            (bind _returnvalue_2 (UserInterface|CreateWidget "/Game/Blueprints/UI/StartRoundButton.StartRoundButton_C"))
            (bind _output_get_2 (Variables|Default|SetThisPlayersStartRoundButton _returnvalue_2))
            (Widget|SetVisibility _output_get_2 "Collapsed"))
          (:then_1
            (bind _returnvalue_3 (UserInterface|CreateWidget "/Game/Blueprints/UI/PlayAgainButton.PlayAgainButton_C"))
            (bind _output_get_3 (Variables|Default|SetThisPlayersPlayAgainButton _returnvalue_3))
            (Widget|SetVisibility _output_get_3 "Collapsed")
            ;[1 1 1] Sets the Round Controller for the character
            (bind _outactors (Actor|GetAllActorsOfClass "/Script/HideNSneakUnreal.RoundController" :!label _label))
            (for _array_element _outactors
              (bind _output_get_4 (Variables|Default|SetRoundControllerInScene _array_element))
              (Class|RoundController|BPAddHidertoHiderTeam _output_get_4 self))))
        (else
          (goto _label))))
    (:then_2
      ;[1 1 1] If player is not in array Players, add it
      (if (not (Utilities|Array|ContainsItem (Variables|/Script/HideNSneakUnreal.RoundController|GetPlayers (Variables|Default|GetRoundControllerInScene)) self))
        (Utilities|Array|Add (Variables|/Script/HideNSneakUnreal.RoundController|GetPlayers (Variables|Default|GetRoundControllerInScene)) 0)))))

(event EventTick
  (params (DeltaSeconds :type Float%20%28single-precision%29))
  (Class|HideNSneakCPPCharacter|MoveDecoy))

(event EventOnRepIsSeeker
  ;[1 1 1] Make characters change color when they become seekers
  (if (Variables|Default|GetbIsSeeker)
    (Utilities|FlowControl|Sequence
      (:then_0
        (CallFunction|SetPingIcon "/Game/Blueprints/Widgets/Materials/Textures/Skull.Skull")
        (CallFunction|PingAllPlayers 5.0))
      (:then_1
        (bind (_playermaterial _charactermovement) (CallFunction|TurnIntoHider))
        (bind _newtrack_0 (Timeline|CameraSwitch Play)
          (:Update
            (Variables|/Script/Engine.SpringArmComponent|SetTargetArmLength (Variables|Default|GetCameraBoom) (Math|Float|Lerp 0.0 (Variables|Default|GetCameraDistanceAsSeeker) _newtrack_0))))))
    (else
      (CallFunction|TurnIntoSeeker _playermaterial _charactermovement)
      (Timeline|CameraSwitch Reverse))))

(event Input|KeyboardEvents|E
  (params (Key :type Key%20Structure))
  (bind _returnvalue (Utilities|Time|GetGameTimeinSeconds))
  (bind _hiderabilityduration (Variables|Default|GetHiderAbilityDuration))
  (:Pressed
    (if (Class|HideNSneakCPPCharacter|IsSeeker)
      ;[1 1 1] Seeker Ability - Change Hiders material to one that can be seen through walls, reset back to original after delay
      (Math|Float|CompareFloat (Variables|Default|GetTimeWhenSeekerAbilityCanBeUsed) _returnvalue
        (:<
          (Utilities|FlowControl|Sequence
            (:then_0
              (Variables|Default|SetTimeWhenSeekerAbilityStops (+ _returnvalue _hiderabilityduration)))
            (:then_1
              (Variables|Default|SetUsingSeekerAbility true))
            (:then_2
              (CallFunction|MakeHidersSeeableThroughWalls)
              (Utilities|FlowControl|Delay _hiderabilityduration)
              (Utilities|FlowControl|Sequence
                (:then_0
                  (Variables|Default|SetTimeWhenSeekerAbilityCanBeUsed (+ (Utilities|Time|GetGameTimeinSeconds) (Variables|Default|GetSeekerAbilityCooldown))))
                (:then_1
                  (Variables|Default|SetUsingSeekerAbility false))
                (:then_2
                  (CallFunction|SetBackHidersMaterial)))))))
      (else
        ;[1 1 1] Hider ability
        (if (Variables|Default|GetDecoyAvailible)
          (Utilities|FlowControl|Sequence
            (:then_0
              (Variables|Default|SetHasUsedHiderAbility true))
            (:then_1
              (Variables|Default|SetTimeWhenHiderAbilityCanBeUsed (+ (Utilities|Time|GetGameTimeinSeconds) (Variables|Default|GetDecoyCooldown)))
              (Class|HideNSneakCPPCharacter|UseDecoyAbility)))
          (else
            (Variables|Default|SetHasUsedHiderAbility false)))))))

(event Input|MouseEvents|RightMouseButton
  (params (Key :type Key%20Structure))
  (bind _returnvalue (Game|GetPlayerController 0))
  ;[1 1 1] Make it so the player can click on UI elements
  (:Released
    (if (Variables|Default|GetInputIsGameOnly)
      (Variables|/Script/Engine.PlayerController|SetbShowMouseCursor _returnvalue true)
      (Input|SetInputModeGameandUI _returnvalue (Variables|Default|GetUIWidget) "LockAlways" false)
      (Variables|Default|SetInputIsGameOnly false)
      (else
        (Variables|/Script/Engine.PlayerController|SetbShowMouseCursor _returnvalue false)
        (Input|SetInputModeGameOnly _returnvalue)
        (Variables|Default|SetInputIsGameOnly true)))))

(event Input|KeyboardEvents|G
  (params (Key :type Key%20Structure))
  ;[1 1 1] PING
  (:Pressed
    (CallFunction|ClientUpdatePingIcon "/Game/Blueprints/Widgets/Materials/Textures/Warning_Icon.Warning_Icon")
    (CallFunction|ClientPingAllPlayers 5.0)))

(fn ConstructionScript
  (bind _mesh (Variables|Character|GetMesh))
  ;[1 1 1] Setup dynamic material instance to change color during gameplay
  (bind _returnvalue (Rendering|Material|CreateDynamicMaterialInstance _mesh 0 (Rendering|Material|GetMaterial _mesh 0) "None" :!class /Script/Engine.PrimitiveComponent))
  (Variables|Default|SetPlayerMaterial _returnvalue))

(fn MakeHidersSeeableThroughWalls
  ;[1 1 1] For all Hiders, set their material to M_SeeThroughWalls
  (bind _outactors (Actor|GetAllActorsOfClass "/Game/Blueprints/BP_HideNSneakCPPCharacter.BP_HideNSneakCPPCharacter_C"))
  (for _array_element _outactors
    (if (not (Class|HideNSneakCPPCharacter|IsSeeker _array_element))
      (if (<= (Math|Vector|VectorLength (- (Transformation|GetActorLocation _array_element) (Transformation|GetActorLocation))) (Variables|Default|GetSekerAbilityRange))
        (Rendering|Material|SetMaterial (Variables|/Script/Engine.Character|GetMesh _array_element) 0 "/Game/Art/Materials/M_SeeThroughWalls.M_SeeThroughWalls")))))

(fn SetBackHidersMaterial
  (bind _outactors (Actor|GetAllActorsOfClass "/Game/Blueprints/BP_HideNSneakCPPCharacter.BP_HideNSneakCPPCharacter_C"))
  (for _array_element _outactors
    (Rendering|Material|SetMaterial (Variables|/Script/Engine.Character|GetMesh _array_element) 0 (Variables|/Game/Blueprints/BP_HideNSneakCPPCharacter.BP_HideNSneakCPPCharacter_C|GetPlayerMaterial _array_element))))

(fn GetLocalPlayerUIWidget
  (bind _asbp_hide_nsneak_cppcharacter (Utilities|Casting|CastToBP_HideNSneakCPPCharacter (Pawn|GetControlledPawn (Game|GetPlayerController 0))))
  (return (Variables|/Game/Blueprints/BP_HideNSneakCPPCharacter.BP_HideNSneakCPPCharacter_C|GetUIWidget _asbp_hide_nsneak_cppcharacter)))

(fn SetPingIcon
  (params (InputPin :type Texture%202D%20Object%20Reference))
  (bind _uiwidget (CallFunction|GetLocalPlayerUIWidget))
  (if (.ReturnValue (Utilities|Map|Find (Variables|/Game/Blueprints/Widgets/BPW_Minimap.BPW_Minimap_C|GetPointsOfInterestByActors (Variables|/Game/Blueprints/Widgets/BPW_Player_UI.BPW_Player_UI_C|GetBPW_Minimap _uiwidget)) self))
    (Appearance|SetBrushfromTexture (Variables|/Game/Blueprints/Widgets/PointOfInterestWidget_BP.PointOfInterestWidget_BP_C|GetCustomImage (.Value (Utilities|Map|Find (Variables|/Game/Blueprints/Widgets/BPW_Minimap.BPW_Minimap_C|GetPointsOfInterestByActors (Variables|/Game/Blueprints/Widgets/BPW_Player_UI.BPW_Player_UI_C|GetBPW_Minimap _uiwidget)) self))) InputPin false)))

(fn TurnIntoHider
  (bind _playermaterial (Variables|Default|GetPlayerMaterial))
  (bind _charactermovement (Variables|Character|GetCharacterMovement))
  (Class|RoundController|BPAddHidertoSeekerTeam (Variables|Default|GetRoundControllerInScene) self)
  (Rendering|Material|SetVectorParameterValue _playermaterial "BodyColor" (Variables|Default|GetSeekerColour) :!class /Script/Engine.MaterialInstanceDynamic)
  (Variables|/Script/Engine.CharacterMovementComponent|SetMaxWalkSpeed _charactermovement (Variables|Default|GetSeekerBaseSpeed))
  (Variables|Default|SetTimeWhenSeekerAbilityCanBeUsed 0.0)
  (return _playermaterial _charactermovement))

(fn TurnIntoSeeker
  (params (self2 :type Material%20Instance%20Dynamic%20Object%20Reference) (self3 :type Character%20Movement%20Component%20Object%20Reference))
  (Class|RoundController|BPAddHidertoHiderTeam (Variables|Default|GetRoundControllerInScene) self)
  (Rendering|Material|SetVectorParameterValue self2 "BodyColor" (Variables|Default|GetHiderColour) :!class /Script/Engine.MaterialInstanceDynamic)
  (Variables|/Script/Engine.CharacterMovementComponent|SetMaxWalkSpeed self3 (Variables|Default|GetHiderBaseSpeed))
  (Variables|Default|SetTimeWhenHiderAbilityCanBeUsed 0.0))