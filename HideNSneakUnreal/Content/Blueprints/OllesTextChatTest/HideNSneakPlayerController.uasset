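; HideNSneakPlayerController is a player controller that carries text chat messages between players.
; On BeginPlay it builds a random "Player" name with a numeric suffix.
; SendMessage prefixes text with that name and calls ReceiveMessage on every controller of this class found in the world, including itself.
; ReceiveMessage casts the HUD to HideNSneakHUD and passes the text to its ChatWindow to update the chat.
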(event Custom|SendMessage
  (params (Message :type Text))
  (bind _outactors (Actor|GetAllActorsOfClass "HideNSneakPlayerController_C"))
  (for _array_element _outactors
    (CallFunction|ReceiveMessage _array_element (Utilities|Text|ToText(String) (Utilities|String|Append (Variables|Default|GetPlayerName) ": " (Utilities|String|ToString(Text) Message))))))

(event Custom|ReceiveMessage
  (params (Message :type Text))
  (bind _ashide_nsneak_hud (Utilities|Casting|CastToHideNSneakHUD (HUD|GetHUD)))
  (Default|UpdateChat (Variables|/Game/Blueprints/OllesTextChatTest/HideNSneakHUD.HideNSneakHUD_C|GetChatWindow _ashide_nsneak_hud) Message))

(event EventBeginPlay
  (Variables|Default|SetPlayerName (Utilities|String|Append "Player " (Utilities|String|ToString(Integer) (Math|Random|RandomIntegerinRange 1 5164312)))))

(fn ConstructionScript)