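; Player character for a hide-and-seek game with hider and seeker roles, minimap pings and a seeker reveal ability.
; BeginPlay creates the local player's UI and registers each character on its minimap, where G shows a timed warning ping.
; OnRepIsSeeker changes dynamic-material colour, speed and camera distance, pinging new seekers with a skull.
; E temporarily swaps nearby hiders to a see-through-walls material on a cooldown; right-click toggles UI cursor input.
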(event Custom|ClientPingAllPlayers
  (params (PingDuration :type Float%20%28single-precision%29))
  (CallFunction|PingAllPlayers PingDuration))

(event Custom|PingAllPlayers
  (params (PingDuration :type Float%20%28single-precision%29))
  ;[1 1 1] Initialize local player's UI, and add ping widget to other players' minimap widgets
  (Default|SetPointOfInterestVisibility (Variables|/Game/Blueprints/Widgets/BPW_Player_UI.BPW_Player_UI_C|GetBPW_Minimap (Variables|/Game/Blueprints/BP_HideNSneakCPPCharacter.BP_HideNSneakCPPCharacter_C|GetUIWidget (stale EventBeginPlay _asbp_hide_nsneak_cppcharacter))) self true)
  (Utilities|FlowControl|Delay PingDuration)
  (CallFunction|StopPingingAllPlayers))

(event Custom|StopPingingAllPlayers
  ;[1 1 1] Initialize local player's UI, and add ping widget to other players' minimap widgets
  (Default|SetPointOfInterestVisibility (Variables|/Game/Blueprints/Widgets/BPW_Player_UI.BPW_Player_UI_C|GetBPW_Minimap (Variables|/Game/Blueprints/BP_HideNSneakCPPCharacter.BP_HideNSneakCPPCharacter_C|GetUIWidget (stale EventBeginPlay _asbp_hide_nsneak_cppcharacter))) self false))

(event Custom|ClientStopPingingAllPlayers
  (CallFunction|StopPingingAllPlayers))

(event Custom|ClientUpdatePingIcon
  (params (Icon :type Texture%202D%20Object%20Reference))
  (CallFunction|UpdatePingIcon Icon))

(event Custom|UpdatePingIcon
  (params (Icon :type Texture%202D%20Object%20Reference))
  (CallFunction|SetPingIcon Icon))

(event EventBeginPlay
  ;[1 1 1] Initialize local player's UI, and add ping widget to other players' minimap widgets
  (bind _asbp_hide_nsneak_cppcharacter (Utilities|Casting|CastToBP_HideNSneakCPPCharacter (Pawn|GetControlledPawn (Game|GetPlayerController 0))))
  (Utilities|FlowControl|Sequence
    (:then_0
      (if (not (Variables|/Game/Blueprints/BP_HideNSneakCPPCharacter.BP_HideNSneakCPPCharacter_C|GetHasWidget _asbp_hide_nsneak_cppcharacter))
        (Variables|/Game/Blueprints/BP_HideNSneakCPPCharacter.BP_HideNSneakCPPCharacter_C|SetHasWidget _asbp_hide_nsneak_cppcharacter true)
        (bind _returnvalue (UserInterface|CreateWidget "/Game/Blueprints/Widgets/BPW_Player_UI.BPW_Player_UI_C" 0 _asbp_hide_nsneak_cppcharacter))
        (bind _output_get (Variables|Default|SetUIWidget _returnvalue))
        (UserInterface|Viewport|AddtoViewport _output_get 0)))
    (:then_1
      (Default|AddPointOfInterest (Variables|/Game/Blueprints/Widgets/BPW_Player_UI.BPW_Player_UI_C|GetBPW_Minimap (Variables|/Game/Blueprints/BP_HideNSneakCPPCharacter.BP_HideNSneakCPPCharacter_C|GetUIWidget _asbp_hide_nsneak_cppcharacter)) self))))

(event EventOnRepIsSeeker
  (bind _playermaterial (Variables|Default|GetPlayerMaterial))
  (bind _charactermovement (Variables|Character|GetCharacterMovement))
  ;[1 1 1] Make characters change color when they become seekers
  (if (Variables|Default|GetbIsSeeker)
    (Utilities|FlowControl|Sequence
      (:then_0
        (CallFunction|SetPingIcon "/Game/Blueprints/Widgets/Materials/Textures/Skull.Skull")
        (CallFunction|PingAllPlayers 5.0))
      (:then_1
        (Rendering|Material|SetVectorParameterValue _playermaterial "BodyColor" (Variables|Default|GetSeekerColour) :!class /Script/Engine.MaterialInstanceDynamic)
        (Variables|/Script/Engine.CharacterMovementComponent|SetMaxWalkSpeed _charactermovement (Variables|Default|GetSeekerSpeed))
        (bind _newtrack_0 (Timeline|CameraSwitch Play)
          (:Update
            (Variables|/Script/Engine.SpringArmComponent|SetTargetArmLength (Variables|Default|GetCameraBoom) (Math|Float|Lerp (Variables|Default|GetCameraDistanceAsSeeker) 3e+02 _newtrack_0))))))
    (else
      (Rendering|Material|SetVectorParameterValue _playermaterial "BodyColor" (Variables|Default|GetHiderColour) :!class /Script/Engine.MaterialInstanceDynamic)
      (Variables|/Script/Engine.CharacterMovementComponent|SetMaxWalkSpeed _charactermovement (Variables|Default|GetHiderSpeed))
      (Timeline|CameraSwitch Reverse))))

(event Input|KeyboardEvents|E
  (params (Key :type Key%20Structure :default "None"))
  (:Pressed
    (if (Class|HideNSneakCPPCharacter|IsSeeker)
      ;[1 1 1] Change Hiders material to one that can be seen through walls, reset back to original after delay
      (Math|Float|CompareFloat (Variables|Default|GetTimeWhenSeekerAbilityCanBeUsed) (Utilities|Time|GetGameTimeinSeconds)
        (:<
          (CallFunction|MakeHidersSeeableThroughWalls)
          (Utilities|FlowControl|Delay (Variables|Default|GetHiderAbilityDuration))
          (CallFunction|SetBackHidersMaterial)
          (Variables|Default|SetTimeWhenSeekerAbilityCanBeUsed (+ (Utilities|Time|GetGameTimeinSeconds) (Variables|Default|GetSeekerAbilityCooldown))))))))

(event Input|MouseEvents|RightMouseButton
  (params (Key :type Key%20Structure :default "None"))
  (bind _returnvalue (Game|GetPlayerController 0))
  ;[1 1 1] Make it so the player can click on UI elements
  (:Released
    (if (Variables|Default|GetInputIsGameOnly)
      (Variables|/Script/Engine.PlayerController|SetbShowMouseCursor _returnvalue true)
      (Input|SetInputModeGameandUI _returnvalue (Variables|Default|GetUIWidget) "LockAlways" false)
      (Variables|Default|SetInputIsGameOnly false)
      (else
        (Variables|/Script/Engine.PlayerController|SetbShowMouseCursor _returnvalue false)
        (Input|SetInputModeGameOnly _returnvalue)
        (Variables|Default|SetInputIsGameOnly true)))))

(event Input|KeyboardEvents|G
  (params (Key :type Key%20Structure :default "None"))
  (:Released
    (CallFunction|ClientUpdatePingIcon "/Game/Blueprints/Widgets/Materials/Textures/Warning_Icon.Warning_Icon")
    (CallFunction|ClientPingAllPlayers 5.0)))

(fn ConstructionScript
  (bind _mesh (Variables|Character|GetMesh))
  ;[1 1 1] Setup dynamic material instance to change color during gameplay
  (bind _returnvalue (Rendering|Material|CreateDynamicMaterialInstance _mesh 0 (Rendering|Material|GetMaterial _mesh 0) "None" :!class /Script/Engine.PrimitiveComponent))
  (Variables|Default|SetPlayerMaterial _returnvalue))

(fn MakeHidersSeeableThroughWalls
  ;[1 1 1] For all Hiders, set their material to M_SeeThroughWalls
  (bind _outactors (Actor|GetAllActorsOfClass "/Game/Blueprints/BP_HideNSneakCPPCharacter.BP_HideNSneakCPPCharacter_C"))
  (for _array_element _outactors
    (if (not (Class|HideNSneakCPPCharacter|IsSeeker _array_element))
      (if (<= (Math|Vector|VectorLength (- (Transformation|GetActorLocation _array_element) (Transformation|GetActorLocation))) (Variables|Default|GetSekerAbilityRange))
        (Rendering|Material|SetMaterial (Variables|/Script/Engine.Character|GetMesh _array_element) 0 "/Game/Art/Materials/M_SeeThroughWalls.M_SeeThroughWalls")))))

(fn SetBackHidersMaterial
  (bind _outactors (Actor|GetAllActorsOfClass "/Game/Blueprints/BP_HideNSneakCPPCharacter.BP_HideNSneakCPPCharacter_C"))
  (for _array_element _outactors
    (Rendering|Material|SetMaterial (Variables|/Script/Engine.Character|GetMesh _array_element) 0 (Variables|/Game/Blueprints/BP_HideNSneakCPPCharacter.BP_HideNSneakCPPCharacter_C|GetPlayerMaterial _array_element))))

(fn SetPingIcon
  (params (Icon :type Texture%202D%20Object%20Reference))
  (bind _widget (CallFunction|GetLocalPlayerUIWidget))
  (if (.ReturnValue (Utilities|Map|Find (Variables|/Game/Blueprints/Widgets/BPW_Minimap.BPW_Minimap_C|GetPointsOfInterestByActors (Variables|/Game/Blueprints/Widgets/BPW_Player_UI.BPW_Player_UI_C|GetBPW_Minimap _widget)) self))
    (Appearance|SetBrushfromTexture (Variables|/Game/Blueprints/Widgets/PointOfInterestWidget_BP.PointOfInterestWidget_BP_C|GetCustomImage (.Value (Utilities|Map|Find (Variables|/Game/Blueprints/Widgets/BPW_Minimap.BPW_Minimap_C|GetPointsOfInterestByActors (Variables|/Game/Blueprints/Widgets/BPW_Player_UI.BPW_Player_UI_C|GetBPW_Minimap _widget)) self))) Icon false)))

(fn GetLocalPlayerUIWidget
  (bind _asbp_hide_nsneak_cppcharacter (Utilities|Casting|CastToBP_HideNSneakCPPCharacter (Pawn|GetControlledPawn (Game|GetPlayerController 0))))
  (return (Variables|/Game/Blueprints/BP_HideNSneakCPPCharacter.BP_HideNSneakCPPCharacter_C|GetUIWidget _asbp_hide_nsneak_cppcharacter)))