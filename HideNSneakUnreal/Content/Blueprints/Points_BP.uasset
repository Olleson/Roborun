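; Points_BP is a score pickup for hiders in a hide-and-sneak game.
; On BeginPlay it caches a reference to the BP_RoundController in the level.
; When a character overlaps its collider and is neither a seeker nor a decoy, it awards its point value with the round controller's score multiplier, then destroys itself.
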(event OnComponentBeginOverlap(Collider)
  (params (OverlappedComponent :type Primitive%20Component%20Object%20Reference) (OtherActor :type Actor%20Object%20Reference) (OtherComp :type Primitive%20Component%20Object%20Reference) (OtherBodyIndex :type Integer) (bFromSweep :type Boolean) (SweepResult :type Hit%20Result%20Structure%20%28by%20ref%29))
  (bind _asbp_hide_nsneak_cppcharacter (Utilities|Casting|CastToBP_HideNSneakCPPCharacter OtherActor))
  (if (not (Class|HideNSneakCPPCharacter|IsSeeker _asbp_hide_nsneak_cppcharacter))
    (if (not (Variables|/Script/HideNSneakUnreal.HideNSneakCPPCharacter|GetIsDecoy _asbp_hide_nsneak_cppcharacter))
      (Default|AddScore _asbp_hide_nsneak_cppcharacter (Variables|Default|GetPointValue) (Variables|/Script/HideNSneakUnreal.RoundController|GetScoreMultiplier (Variables|Default|GetRoundController)))
      (Actor|DestroyActor))))

(event EventBeginPlay
  (bind _outactors (Actor|GetAllActorsOfClass "/Game/Blueprints/BP_RoundController.BP_RoundController_C"))
  (for _array_element _outactors
    (Variables|Default|SetRoundController _array_element)))

(fn ConstructionScript)