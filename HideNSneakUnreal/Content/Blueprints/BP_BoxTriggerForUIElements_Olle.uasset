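; Tutorial trigger box that shows a title, description and video widget when the player reaches it during training rounds.
; On BeginPlay it finds the round controller, builds the widget, or destroys itself outside training.
; Overlap by the player character only counts when this box is the current arrow target.
; It then shows the widget, updates the checklist item matching its display name, and advances the arrow target, hiding the arrow after the last.
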(event EventBeginPlay
  (Utilities|FlowControl|Delay 0.2)
  (bind _outactors (Actor|GetAllActorsOfClass "/Game/Blueprints/BP_RoundController.BP_RoundController_C"))
  (bind _output_get (Variables|Default|SetRoundControllerInScene (Utilities|Array|Get(acopy) _outactors)))
  (if (Variables|/Game/Blueprints/BP_RoundController.BP_RoundController_C|GetIsTraining _output_get)
    (bind _returnvalue (UserInterface|CreateWidget "/Game/Blueprints/Widgets/TrainingOrTutorial/BPW_DefaultTutWidget.BPW_DefaultTutWidget_C"))
    (Utilities|FlowControl|Sequence
      (:then_0
        (Default|ChangeTitleText _returnvalue (Variables|Default|GetWidgetTitle)))
      (:then_1
        (Default|ChangeDescriptionText _returnvalue (Variables|Default|GetWidgetText)))
      (:then_2
        (Default|ChangeImageVideo _returnvalue (Variables|Default|GetWidgetVideo)))
      (:then_3
        (Variables|Default|SetWidgetToShow _returnvalue)))
    (else
      (Actor|DestroyActor))))

(event Collision|EventActorBeginOverlap
  (params (OtherActor :type Actor%20Object%20Reference))
  (bind _roundcontrollerinscene (Variables|Default|GetRoundControllerInScene))
  (bind _roundcontrollerinscene_2 (Variables|Default|GetRoundControllerInScene))
  (bind _arrowtargets (Variables|/Game/Blueprints/BP_RoundController.BP_RoundController_C|GetArrowTargets _roundcontrollerinscene_2))
  (bind _asbp_hide_nsneak_cppcharacter (Utilities|Casting|CastToBP_HideNSneakCPPCharacter OtherActor))
  (Utilities|IsValid _asbp_hide_nsneak_cppcharacter
    (:Is%20Valid
      (if (== self (Variables|/Game/Blueprints/BP_RoundController.BP_RoundController_C|GetCurrentArrowTarget _roundcontrollerinscene))
        (Utilities|FlowControl|Sequence
          (:then_0
            (UserInterface|Viewport|AddtoViewport (Variables|Default|GetWidgetToShow) 0))
          (:then_1
            (for _array_element (Class|PanelWidget|GetAllChildren (Variables|/Game/Blueprints/Widgets/BPW_TutorialList.BPW_TutorialList_C|GetListScrollBox (Variables|/Game/Blueprints/BP_RoundController.BP_RoundController_C|GetCheckList _roundcontrollerinscene)))
              (bind _asbpw_tutorial_list_item (Utilities|Casting|CastToBPW_TutorialListItem _array_element))
              (if (Utilities|Enum|Equal(Enum) (Utilities|GetDisplayName self) (Variables|/Game/Blueprints/Widgets/BPW_TutorialListItem.BPW_TutorialListItem_C|GetNewText _asbpw_tutorial_list_item))
                (Default|ChangeImageonWidget _asbpw_tutorial_list_item))))
          (:then_2
            (if (not (Variables|Default|GetHasChangedArrowtarget))
              (Variables|Default|SetHasChangedArrowtarget true)
              (if (Utilities|IsValid (Utilities|Array|Get(acopy) _arrowtargets (+ (Utilities|Array|FindItem _arrowtargets (Variables|/Game/Blueprints/BP_RoundController.BP_RoundController_C|GetCurrentArrowTarget _roundcontrollerinscene_2)) 1)))
                (Variables|/Game/Blueprints/BP_RoundController.BP_RoundController_C|SetCurrentArrowTarget _roundcontrollerinscene_2 (Utilities|Array|Get(acopy) _arrowtargets (+ (Utilities|Array|FindItem _arrowtargets (Variables|/Game/Blueprints/BP_RoundController.BP_RoundController_C|GetCurrentArrowTarget _roundcontrollerinscene_2)) 1)))
                (else
                  (Development|SetHiddeninGame (Variables|/Game/Blueprints/BP_HideNSneakCPPCharacter.BP_HideNSneakCPPCharacter_C|GetArrowChild _asbp_hide_nsneak_cppcharacter) true false)
                  (Actor|Tick|SetActorTickEnabled _roundcontrollerinscene_2))))))))))

(fn ConstructionScript)