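; Spline mesh generator Blueprint that tiles a chosen mesh along a spline in its construction script.
; Section length comes from the mesh bounding box's max on the forward axis, and only whole sections spawn to avoid squashed pieces.
; Each spline mesh component takes positions and tangents from the spline, with tangents clamped to section length, and gets query-only collision.
; An optional end mesh replaces the last piece.
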(fn ConstructionScript
  (bind _mesh (Variables|Default|GetMesh))
  (bind _endmesh (Variables|Default|GetEndMesh))
  (bind _spline (Variables|Default|GetSpline))
  (bind _returnvalue (StaticMesh|GetBoundingBox _mesh))
  ;[1 1 1] Author: Oskar Johansson
  ;;[1 1 1] Set the length of the spline and check if the mesh is valid
  (Variables|Default|SetSplineLength (Spline|GetSplineLength (Variables|Default|GetSpline)))
  (if (Utilities|IsValid (Variables|Default|GetMesh))
    ;;[1 1 1] Sets how long the mesh should be depending on wich axis is forward to prevent stretching the meshes
    (if (Utilities|Enum|Equal(Enum) (Utilities|String|ToString(Byte) (Variables|Default|GetForward%20axis)) "0")
      (Variables|Default|SetSectionLength (.x (.max _returnvalue)))
      ;;[1 1 1] Loop through the numbers and spawn meshes accordingly
      (for _index (range 0 (- (Math|Float|Truncate (/ (Variables|Default|GetSplineLength) (Variables|Default|GetSectionLength))) 1)) :!label _label
        (bind _returnvalue_2 (AddComponent|AddSplineMeshComponent false))
        ;;[1 1 1] If an endmesh is selected spawn one as the last piece
        (if (== (- (Math|Float|Truncate (/ (Variables|Default|GetSplineLength) (Variables|Default|GetSectionLength))) 1) _index)
          (if (Utilities|IsValid _endmesh)
            (Components|StaticMesh|SetStaticMesh _returnvalue_2 _endmesh)
            (else
              (Components|StaticMesh|SetStaticMesh _returnvalue_2 (Variables|Default|GetMesh) :!label _label_2)))
          (else
            (goto _label_2)))
        (SplineMesh|SetForwardAxis _returnvalue_2 (Variables|Default|GetForward%20axis) true)
        (SplineMesh|SetStartandEnd _returnvalue_2 (Spline|GetLocationatDistanceAlongSpline _spline (* _index (Variables|Default|GetSectionLength)) "Local") (Math|Vector|ClampVectorSize (Spline|GetTangentatDistanceAlongSpline _spline (* _index (Variables|Default|GetSectionLength)) "Local") 0.0 (Variables|Default|GetSectionLength)) (Spline|GetLocationatDistanceAlongSpline _spline (* (+ _index 1) (Variables|Default|GetSectionLength)) "Local") (Math|Vector|ClampVectorSize (Spline|GetTangentatDistanceAlongSpline _spline (* (+ _index 1) (Variables|Default|GetSectionLength)) "Local") 0.0 (Variables|Default|GetSectionLength)) true :!class /Script/Engine.SplineMeshComponent)
        (Collision|SetCollisionEnabled _returnvalue_2 "QueryOnly"))
      (elif (Utilities|Enum|Equal(Enum) (Utilities|String|ToString(Byte) (Variables|Default|GetForward%20axis)) "1")
        (Variables|Default|SetSectionLength (.y (.max _returnvalue)))
        (goto _label)
        (elif true
          (Variables|Default|SetSectionLength (.z (.max _returnvalue)))
          (goto _label))))))