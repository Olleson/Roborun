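; Round controller for a multiplayer hide-and-seek game, running each match from start button to scoring.
; Starting a round resets players to hiders and their spawns, picks a random seeker who is briefly frozen, and begins a countdown.
; Tick ends the round on timeout or minimum hider count, awarding remaining hiders points and showing Play Again.
; The authority also spawns point pickups at random tagged locations, with timed respawns based on round length.
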(event Custom|ApplySettingsToAllPlayers
  ;[1 1 1] Apply settings to all players
  (for _array_element (Variables|Default|GetPlayers)
    (bind _asbp_hide_nsneak_cppcharacter (Utilities|Casting|CastToBP_HideNSneakCPPCharacter _array_element))
    (Default|InitializePlayerSettings _asbp_hide_nsneak_cppcharacter (Variables|Default|GetHidersBaseSpeed) (Variables|Default|GetSeekersBaseSpeed) (Variables|Default|GetPlayersBaseJumpHeight))))

(event Custom|StartRound
  (bind _randomisedseeker (Variables|Default|GetRandomisedSeeker))
  ;[1 1 1] Starts the round, makes a random person the Seeker, starts the timer
  (Utilities|FlowControl|Delay 0.01)
  (CallFunction|StartRound)
  (Utilities|FlowControl|Delay 0.01)
  (if (Utilities|IsValid _randomisedseeker)
    (Class|HideNSneakCPPCharacter|ServerBecomeSeeker _randomisedseeker)
    (Utilities|FlowControl|Sequence
      (:then_0
        (Utilities|Time|SetTimerbyFunctionName 0 "Detract1FromTimerEverySecond" 1.0 true))
      (:then_1
        (for _array_element (Variables|Default|GetSeekers)
          (Utilities|FlowControl|Sequence
            (:then_0
              (Pawn|Components|CharacterMovement|DisableMovement (Variables|/Script/Engine.Character|GetCharacterMovement _array_element)))
            (:then_1
              (Utilities|FlowControl|Delay (Variables|Default|GetSeekerWaitAtStartTime))
              (Pawn|Components|CharacterMovement|SetMovementMode (Variables|/Script/Engine.Character|GetCharacterMovement _array_element) "MOVE_Walking" 0)))))
      (:then_2
        (Actor|Tick|SetActorTickEnabled true)
        (Development|PrintString "Hello")))))

(event Custom|SetStartButton
  (CallFunction|MakeButtonVisible (Variables|/Game/Blueprints/BP_HideNSneakCPPCharacter.BP_HideNSneakCPPCharacter_C|GetThisPlayersStartRoundButton (Variables|Default|GetCharacterWithAuthority))))

(event Custom|SpawnPoint
  (bind _pointspawnlocations (Variables|Default|GetPointSpawnLocations))
  (bind _pointspawnlocations_2 (Variables|Default|GetPointSpawnLocations))
  (bind _returnvalue (Utilities|Array|Length _pointspawnlocations))
  (bind _returnvalue_2 (- _returnvalue 1))
  (bind _returnvalue_3 (Math|Random|RandomIntegerinRange 0 _returnvalue_2))
  (bind _output (Utilities|Array|Get(acopy) _pointspawnlocations_2 _returnvalue_3))
  (bind _rootcomponent (Variables|/Script/Engine.Actor|GetRootComponent _output))
  (bind _returnvalue_4 (Transformation|GetWorldTransform _rootcomponent))
  ;[1 1 1] Section author: Oskar Johansson
  ; Spawn points in the level
  ; Only spawns 100 units above the pivot point of objects with the actor tag "PointSpawn"
  (for _index (range 1 (Variables|Default|GetNumberOfPointsToSpawn))
    (if (Utilities|Array|IsValidIndex _pointspawnlocations_2 _returnvalue_3) :!label _label
      (bind _returnvalue_5 (Game|SpawnActorfromClass "/Game/Blueprints/Points_BP.Points_BP_C" (Math|Transform|MakeTransform (+ (.location _returnvalue_4) "0,0.000000,100.000000") (.rotation _returnvalue_4) (.scale _returnvalue_4)) "AdjustIfPossibleButDontSpawnIfColliding" 0 0))
      (Development|PrintString (Utilities|String|Append "LoopNumber = " (Utilities|String|ToString(Integer) _index)) true true "(R=0.000000,G=0.660000,B=1.000000,A=1.000000)" 6.0)
      (if (not (Utilities|IsValid _returnvalue_5))
        (goto _label))
      (else
        (Development|PrintString "no point spawn locations in the world"))))
  ;;[1 1 1] Set timers when to spawn the point objects again
  (if (Variables|Default|GetMIddlePoint)
    (Utilities|Time|SetTimerbyEvent (delegate Custom|SpawnPoint) (Math|Conversions|ToFloat(Integer) (/ (Variables|RoundController|GetRoundTime) 2)))
    (Variables|Default|SetMIddlePoint false)
    (Development|PrintString "timer set" true true "(R=0.000000,G=0.660000,B=1.000000,A=1.000000)" 5.0)
    (elif (Variables|Default|GetLastMinute)
      (Utilities|Time|SetTimerbyEvent (delegate Custom|SpawnPoint) (Math|Conversions|ToFloat(Integer) (- (Variables|RoundController|GetRoundTime) 60)))
      (Variables|Default|SetLastMinute false)
      (Development|PrintString "HalfTime"))))

(event EventBeginPlay
  (Utilities|FlowControl|Sequence
    (:then_0
      (bind _outactors (Actor|GetAllActorswithTag "PointSpawn"))
      (Variables|Default|SetPointSpawnLocations _outactors)
      (if (Ability|HasAuthority)
        (CallFunction|SpawnPoint)))
    (:then_1
      ;[1 1 1] Check to see if the game should be in training mode or not
      (bind _returnvalue (Game|GetCurrentLevelName true))
      (if (Utilities|Enum|Equal(Enum) _returnvalue (Variables|Default|GetTrainingLevelName))
        _
        (else
          _))
      (Networking|SwitchHasAuthority
        (:Authority
          (Utilities|FlowControl|Sequence
            (:then_0
              (Variables|RoundController|SetOrigimalRoundTime (Variables|RoundController|GetRoundTime)))
            (:then_1
              (bind _outactors_2 (Actor|GetAllActorsOfClass "/Game/Blueprints/BP_HideNSneakCPPCharacter.BP_HideNSneakCPPCharacter_C"))
              (if (Ability|HasAuthority (Utilities|Array|Get(acopy) _outactors_2))
                (Variables|Default|SetCharacterWithAuthority (Utilities|Array|Get(acopy) _outactors_2))
                (Utilities|FlowControl|Delay 3.0)
                (CallFunction|SetStartButton)))
            (:then_2
              (bind _outactors_3 (Actor|GetAllActorsOfClass "/Game/Oskar/Blueprints/MovingPlatform/AlwaysMovingPlatform.AlwaysMovingPlatform_C"))
              (for _array_element _outactors_3
                (Actor|Tick|SetActorTickEnabled _array_element true)))))))
    (:then_2
      (bind _outactors_4 (Actor|GetAllActorsOfClass "/Script/Engine.PlayerStart"))
      (for _array_element_2 _outactors_4
        (Utilities|Array|Add (Variables|Default|GetPlayerStarts_0) _array_element_2)))))

(event EventTick
  (params (DeltaSeconds :type Float%20%28single-precision%29))
  (bind _characterwithauthority (Variables|Default|GetCharacterWithAuthority))
  (bind _thisplayersplayagainbutton (Variables|/Game/Blueprints/BP_HideNSneakCPPCharacter.BP_HideNSneakCPPCharacter_C|GetThisPlayersPlayAgainButton _characterwithauthority))
  ;[1 1 1] Tick
  (if (and (or (< (Variables|RoundController|GetRoundTime) 1) (== (Utilities|Array|Length (Variables|Default|GetHiders)) (Variables|Default|GetMinimumAmountOfPlayers))) (!= (Utilities|Array|Length (Variables|Default|GetPlayers)) 1))
    (Actor|Tick|SetActorTickEnabled false)
    (Variables|RoundController|SetIsRoundActive false)
    (for _array_element (Variables|Default|GetHiders)
      (bind _returnvalue (Class|HideNSneakCPPCharacter|AddScore _array_element (Variables|Default|GetWinningScore) (Variables|Default|GetScoreMultiplier)))
      (Development|PrintString (Utilities|String|Append (Utilities|GetDisplayName _array_element) " Won and now has  " (Utilities|String|ToString(Integer) _returnvalue) " points") true true "(R=0.000000,G=0.660000,B=1.000000,A=1.000000)" 15.0)
      (bind _outactors (Actor|GetAllActorsOfClass "/Game/Blueprints/BP_HideNSneakCPPCharacter.BP_HideNSneakCPPCharacter_C"))
      (for _array_element_2 _outactors
        (Development|PrintString (Utilities|String|Append (Utilities|GetDisplayName _array_element_2) " has " (Utilities|String|ToString(Integer) (Variables|/Script/HideNSneakUnreal.HideNSneakCPPCharacter|GetScore _array_element_2)) " points") true true "(R=1.000000,G=0.000000,B=0.051249,A=1.000000)" 3e+01)))
    (Widget|SetVisibility _thisplayersplayagainbutton "Visible")
    (Variables|/Script/Engine.PlayerController|SetbShowMouseCursor (Class|GameplayStatics|GetPlayerControllerfromID) true)
    (if (UserInterface|Viewport|IsinViewport _thisplayersplayagainbutton)
      (Widget|SetVisibility _thisplayersplayagainbutton "Visible")
      (else
        (UserInterface|Viewport|AddtoViewport _thisplayersplayagainbutton 0)))))

(fn ConstructionScript)

(fn Detract1fromTimerEverySecond
  ;[1 1 1] Checks if the round is over or not
  (if (Variables|RoundController|GetIsRoundActive)
    ;[1 1 1] Detracts 1 from the Round Time
    (Variables|RoundController|SetRoundTime (- (Variables|RoundController|GetRoundTime) 1))
    (else
      (return))))

(fn MakeButtonVisible
  (params (InputPin :type Start%20Round%20Button%20Object%20Reference))
  (Widget|SetVisibility InputPin "Visible")
  (Variables|/Script/Engine.PlayerController|SetbShowMouseCursor (Class|GameplayStatics|GetPlayerControllerfromID) true)
  (Variables|Default|SetStartRoundButton InputPin)
  (if (UserInterface|Viewport|IsinViewport InputPin)
    (Widget|SetVisibility InputPin "Visible")
    (else
      (UserInterface|Viewport|AddtoViewport InputPin 0))))

(fn RandomisePlayerinArrayPlayers
  (bind _players (Variables|Default|GetPlayers))
  (bind _output_get (Variables|Default|SetRandom%20Number (Math|Random|RandomIntegerinRange 0 (- (Utilities|Array|Length _players) 1))))
  (for (_array_element _array_index) _players
    (if (== _array_index _output_get)
      (bind _asbp_hide_nsneak_cppcharacter (Utilities|Casting|CastToBP_HideNSneakCPPCharacter _array_element))
      (Variables|Default|SetRandomisedSeeker _asbp_hide_nsneak_cppcharacter)))
  (return))

(fn StartRound
  (bind _returnvalue (Utilities|Time|GetGameTimeinSeconds))
  (bind _characterwithauthority (Variables|Default|GetCharacterWithAuthority))
  (if (>= (Utilities|Array|Length (Variables|Default|GetPlayers)) (Variables|Default|GetAmountOfPlayersToStart))
    (Utilities|FlowControl|Sequence
      (:then_0
        (Variables|RoundController|SetRoundTime (Variables|RoundController|GetOrigimalRoundTime)))
      (:then_1
        (Variables|RoundController|SetIsRoundActive true)
        (Widget|SetVisibility (Variables|/Game/Blueprints/Widgets/BPW_Player_UI.BPW_Player_UI_C|GetB_LobbySettings (Variables|/Game/Blueprints/BP_HideNSneakCPPCharacter.BP_HideNSneakCPPCharacter_C|GetUIWidget (Variables|Default|GetCharacterWithAuthority))) "Hidden"))
      (:then_2
        (bind _asplayer_controller (Utilities|Casting|CastToPlayerController (Pawn|GetController (Variables|Default|GetCharacterWithAuthority))))
        (Variables|/Script/Engine.PlayerController|SetbShowMouseCursor _asplayer_controller false)
        (Class|HideNSneakCPPCharacter|ServerResetPlayerstoHiders _characterwithauthority)
        (Widget|SetVisibility (Variables|/Game/Blueprints/BP_HideNSneakCPPCharacter.BP_HideNSneakCPPCharacter_C|GetThisPlayersStartRoundButton _characterwithauthority) "Collapsed"))
      (:then_3
        (CallFunction|RandomisePlayerinArrayPlayers)
        (Actor|Tick|SetActorTickEnabled true)
        (Development|PrintString "im now ticking"))
      (:then_4
        (for _array_element (Variables|Default|GetPlayers)
          (bind _asbp_hide_nsneak_cppcharacter (Utilities|Casting|CastToBP_HideNSneakCPPCharacter _array_element))
          (Utilities|FlowControl|Sequence
            (:then_0
              (Variables|/Game/Blueprints/BP_HideNSneakCPPCharacter.BP_HideNSneakCPPCharacter_C|SetTimeWhenHiderAbilityCanBeUsed _asbp_hide_nsneak_cppcharacter _returnvalue))
            (:then_1
              (Variables|/Game/Blueprints/BP_HideNSneakCPPCharacter.BP_HideNSneakCPPCharacter_C|SetTimeWhenSeekerAbilityCanBeUsed _asbp_hide_nsneak_cppcharacter _returnvalue))
            (:then_2
              (Transformation|SetActorTransform _asbp_hide_nsneak_cppcharacter (Math|Transform|MakeTransform (Variables|/Game/Blueprints/BP_HideNSneakCPPCharacter.BP_HideNSneakCPPCharacter_C|GetPlayerSpawnLocation _asbp_hide_nsneak_cppcharacter) (Variables|/Game/Blueprints/BP_HideNSneakCPPCharacter.BP_HideNSneakCPPCharacter_C|GetPlayerSpawnRotation _asbp_hide_nsneak_cppcharacter) "1,1,1")))))))
    (else
      (CallFunction|SetStartButton))))