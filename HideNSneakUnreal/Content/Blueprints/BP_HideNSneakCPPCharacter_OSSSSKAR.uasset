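; Player character for a hide-and-seek tag game, switching between hider and seeker roles, with decoys as a variant.
; The IsSeeker rep-notify swaps team, speed, anim class, materials and camera distance, scores the tagger, and destroys tagged decoys.
; Abilities give seekers timed see-through-wall materials on nearby hiders and hiders a decoy.
; It also handles round-controller registration, local UI, minimap pings, elevators, power-up icons and chat.
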(event Custom|AddToUI
  (params (WidgetToShow :type User%20Widget%20Class%20Reference))
  ;[1 1 1] Add element to player UI
  (bind _returnvalue (UserInterface|CreateWidget WidgetToShow))
  (UserInterface|Viewport|AddtoViewport _returnvalue 0))

(event Custom|PingAllPlayers
  (params (PingDuration :type Float%20%28single-precision%29))
  ;[1 1 1] On player start
  ;;[1 1 1] Initialize local player's UI, and add ping widget to other players' minimap widgets
  (if (Pawn|IsPlayerControlled)
    (Default|SetPointOfInterestVisibility (Variables|/Game/Blueprints/Widgets/BPW_Player_UI.BPW_Player_UI_C|GetBPW_Minimap (Variables|/Game/Blueprints/BP_HideNSneakCPPCharacter.BP_HideNSneakCPPCharacter_C|GetUIWidget (stale EventBeginPlay _asbp_hide_nsneak_cppcharacter))) self true)
    (Utilities|FlowControl|Delay PingDuration)
    (CallFunction|StopPingingAllPlayers)))

(event Custom|ActivateObject
  (params (Elevator :type Elevator%20with%20Buttons%20BP%20Object%20Reference))
  ;[1 1 1] Moving platform interaction
  (Variables|Misc.|SetElevatorReference Elevator))

(event Custom|InitializePlayerSettings
  (params (HiderBaseSpeed :type Float%20%28single-precision%29) (SeekerBaseSpeed :type Float%20%28single-precision%29) (PlayerBaseJumpHeight :type Float%20%28single-precision%29))
  ;[1 1 1] Initialize Player Settings
  (bind _output_get (Variables|Default|SetHiderBaseSpeed HiderBaseSpeed))
  (Variables|/Script/Engine.CharacterMovementComponent|SetMaxWalkSpeed (Variables|Character|GetCharacterMovement) _output_get)
  (Variables|Default|SetSeekerBaseSpeed SeekerBaseSpeed)
  (bind _output_get_2 (Variables|Default|SetBaseJumpHeight PlayerBaseJumpHeight))
  (Variables|/Script/Engine.CharacterMovementComponent|SetJumpZVelocity (Variables|Character|GetCharacterMovement) _output_get_2))

(event Custom|ClientPingAllPlayers
  (params (PingDuration :type Float%20%28single-precision%29))
  ;[1 1 1] PING
  (CallFunction|PingAllPlayers PingDuration))

(event Custom|StopPingingAllPlayers
  ;[1 1 1] On player start
  ;;[1 1 1] Initialize local player's UI, and add ping widget to other players' minimap widgets
  (if (Pawn|IsPlayerControlled)
    (Default|SetPointOfInterestVisibility (Variables|/Game/Blueprints/Widgets/BPW_Player_UI.BPW_Player_UI_C|GetBPW_Minimap (Variables|/Game/Blueprints/BP_HideNSneakCPPCharacter.BP_HideNSneakCPPCharacter_C|GetUIWidget (stale EventBeginPlay _asbp_hide_nsneak_cppcharacter))) self false)))

(event Custom|ServerSendMessage
  (params (Player :type BP%20Hide%20N%20Sneak%20CPP%20Character%20Object%20Reference) (PlayerName :type Text) (Message :type Text))
  ;[1 1 1] Owning client replicates players' messages
  (bind _asbp_round_controller (Utilities|Casting|CastToBP_RoundController (Variables|Misc.|GetRoundControllerInScene)))
  (Default|SendMessage _asbp_round_controller Player PlayerName Message))

(event Custom|ClientStopPingingAllPlayers
  ;[1 1 1] PING
  (CallFunction|StopPingingAllPlayers))

(event Custom|ClientUpdatePingIcon
  (params (Icon :type Texture%202D%20Object%20Reference))
  ;[1 1 1] PING
  (CallFunction|UpdatePingIcon Icon))

(event Custom|UpdatePingIcon
  (params (Icon :type Texture%202D%20Object%20Reference))
  ;[1 1 1] PING
  (CallFunction|SetPingIcon Icon))

(event Custom|Spawn%20sound
  (params (Sound :type Sound%20Base%20Object%20Reference) (Location :type Vector))
  ;[1 1 1] Spawn emitter & sound
  (Audio|SpawnSoundatLocation Sound Location "0, 0, 0" 0.7 1.0 0.0 0 0))

(event Custom|Spawn%20emitter
  (params (Emitter :type Particle%20System%20Object%20Reference) (Location :type Vector))
  ;[1 1 1] Spawn emitter & sound
  (Effects|SpawnEmitteratLocation Emitter Location))

(event Custom|TurnOfObject
  ;[1 1 1] Moving platform interaction
  (Variables|Misc.|SetElevatorReference 0))

(event Custom|ClientStartElevator
  (params (Elevator :type Elevator%20with%20Buttons%20BP%20Object%20Reference))
  ;[1 1 1] Moving platform interaction
  (Default|StarttheElevator Elevator))

(event Custom|SetSilentFootsteps_1
  (params (inSilentFootsteps :type Boolean))
  ;[1 1 1] Toggles footsteps to be audible or silent
  (bind _ashider_anim_bp (Utilities|Casting|CastToHider_Anim_BP (Components|SkeletalMesh|GetAnimInstance (Variables|Character|GetMesh))))
  (Variables|/Game/Art/3D/Character/Animations/BP/Hider_Anim_BP.Hider_Anim_BP_C|SetHasSilentFootsteps _ashider_anim_bp inSilentFootsteps))

(event EventEndPlay
  (params (EndPlayReason :type EEndPlayReason%20Enum :default "Destroyed"))
  (|RemovePlayerFromPlayersArray))

(event EventBeginPlay
  (bind _self self)
  (bind _self_2 self)
  ;[1 1 1] On player start
  (Utilities|FlowControl|Sequence
    (:then_0
      ;;[1 1 1] Initialize local player's UI, and add ping widget to other players' minimap widgets
      (if (Pawn|IsPlayerControlled)
        (bind _asbp_hide_nsneak_cppcharacter (Utilities|Casting|CastToBP_HideNSneakCPPCharacter (Pawn|GetControlledPawn (Game|GetPlayerController 0))))
        (Utilities|FlowControl|Sequence
          (:then_0
            (if (not (Variables|/Game/Blueprints/BP_HideNSneakCPPCharacter.BP_HideNSneakCPPCharacter_C|GetHasWidget _asbp_hide_nsneak_cppcharacter))
              (Variables|/Game/Blueprints/BP_HideNSneakCPPCharacter.BP_HideNSneakCPPCharacter_C|SetHasWidget _asbp_hide_nsneak_cppcharacter true)
              (bind _returnvalue (UserInterface|CreateWidget "/Game/Blueprints/Widgets/BPW_Player_UI.BPW_Player_UI_C" 0 _asbp_hide_nsneak_cppcharacter))
              (bind _output_get (Variables|UI|SetUIWidget _returnvalue))
              (UserInterface|Viewport|AddtoViewport _output_get 0)))
          (:then_1
            (Default|AddPointOfInterest (Variables|/Game/Blueprints/Widgets/BPW_Player_UI.BPW_Player_UI_C|GetBPW_Minimap (Variables|/Game/Blueprints/BP_HideNSneakCPPCharacter.BP_HideNSneakCPPCharacter_C|GetUIWidget _asbp_hide_nsneak_cppcharacter)) self)))))
    (:then_1
      ;;[1 1 1] Button Setting functions
      (Rendering|Material|SetVectorParameterValue (Variables|Misc.|GetPlayerMaterial) "BodyColor" (Variables|Hider|GetHiderColour) :!class /Script/Engine.MaterialInstanceDynamic)
      (Utilities|FlowControl|Delay 0.2)
      (if (not (Variables|Default|GetIsDecoy))
        ;;;[1 1 1] Sets the Round Controller for the character
        (bind _outactors (Actor|GetAllActorsOfClass "/Script/HideNSneakUnreal.RoundController"))
        (bind _output_get_2 (Variables|Misc.|SetRoundControllerInScene (Utilities|Array|Get(acopy) _outactors)))
        (if (not (Variables|Default|GetIsDecoy _self_2))
          (Class|RoundController|BPAddHidertoHiderTeam _output_get_2 _self_2))))
    (:then_2
      ;;[1 1 1] Sets the players' spawn location & rotation, ensures that no other player can have the same spawn values
      (Utilities|FlowControl|Delay 2.0)
      (bind _asbp_round_controller (Utilities|Casting|CastToBP_RoundController (Variables|Misc.|GetRoundControllerInScene)))
      (if (not (Variables|/Game/Blueprints/BP_RoundController.BP_RoundController_C|GetIsTraining _asbp_round_controller))
        (Utilities|FlowControl|Sequence
          (:then_0
            (Variables|Misc.|SetPlayerSpawnLocation (Transformation|GetActorLocation (Utilities|Array|Get(acopy) (Variables|/Game/Blueprints/BP_RoundController.BP_RoundController_C|GetPlayerStarts _asbp_round_controller) (Math|Random|RandomInteger (Utilities|Array|Length (Variables|/Game/Blueprints/BP_RoundController.BP_RoundController_C|GetPlayerStarts _asbp_round_controller)))))))
          (:then_1
            (Variables|Misc.|SetPlayerSpawnRotation (Transformation|GetActorRotation (Utilities|Array|Get(acopy) (Variables|/Game/Blueprints/BP_RoundController.BP_RoundController_C|GetPlayerStarts _asbp_round_controller) (Math|Random|RandomInteger (Utilities|Array|Length (Variables|/Game/Blueprints/BP_RoundController.BP_RoundController_C|GetPlayerStarts _asbp_round_controller)))))))
          (:then_2
            (Utilities|Array|RemoveItem (Variables|/Game/Blueprints/BP_RoundController.BP_RoundController_C|GetPlayerStarts _asbp_round_controller) (Utilities|Array|Get(acopy) (Variables|/Game/Blueprints/BP_RoundController.BP_RoundController_C|GetPlayerStarts _asbp_round_controller) (Math|Random|RandomInteger (Utilities|Array|Length (Variables|/Game/Blueprints/BP_RoundController.BP_RoundController_C|GetPlayerStarts _asbp_round_controller)))))))))
    (:then_3
      (Variables|Misc.|SetPlayerName (Utilities|String|Append "Player " (Utilities|String|ToString(Integer) (Math|Random|RandomIntegerinRange 1 80)))))
    (:then_4
      ;;[1 1 1] Adds this player to the players array if they are valid
      (Utilities|FlowControl|Delay 0.2)
      (if (not (Variables|Default|GetIsDecoy))
        (if (Utilities|IsValid (Variables|Misc.|GetRoundControllerInScene))
          (if (not (Utilities|Array|ContainsItem (Variables|/Script/HideNSneakUnreal.RoundController|GetPlayers (Variables|Misc.|GetRoundControllerInScene)) _self))
            (Utilities|Array|Add (Variables|/Script/HideNSneakUnreal.RoundController|GetPlayers (Variables|Misc.|GetRoundControllerInScene)) _self)))))))

(event EventTick
  (params (DeltaSeconds :type Float%20%28single-precision%29))
  (Class|HideNSneakCPPCharacter|MoveDecoy))

(event EventOnRepIsSeeker
  (bind _returnvalue (Transformation|GetActorLocation))
  (bind _returnvalue_2 (Game|GetPlayerController 0))
  ;[1 1 1] NEW
  ;[1 1 1] Player state transform + seeker interaction with hiders
  (if (Variables|Default|GetRanAlready)
    (Variables|Default|SetRanAlready false)
    (if (Variables|Default|GetbIsSeeker)
      (if (Variables|Default|GetIsDecoy)
        ;;[1 1 1] Decoy interaction with seeker
        (CallFunction|SpawnEmitter "/Game/Art/VFX/ParticleSystems/P_DecoyDestruction.P_DecoyDestruction" _returnvalue)
        (CallFunction|SpawnSound "/Game/StarterContent/Audio/Explosion01.Explosion01" _returnvalue)
        (Actor|DestroyActor)
        (Variables|Default|SetRanAlready true :!label _label)
        (else
          (CallFunction|AddTaggerPoints)
          (Utilities|FlowControl|Sequence
            (:then_0
              (CallFunction|SetPingIcon "/Game/Blueprints/Widgets/Materials/Textures/Skull.Skull")
              (CallFunction|PingAllPlayers 5.0))
            (:then_1
              (Input|DisableInput _returnvalue_2)
              (Utilities|FlowControl|Delay 2.0)
              (Input|EnableInput _returnvalue_2))
            (:then_2
              (bind _charactermovement (CallFunction|TurnIntoSeeker))
              ;;[1 1 1] Change camera perspective when swapping from between character states
              (bind _newtrack_0 (Timeline|CameraSwitch Play)
                (:Update
                  (Variables|/Script/Engine.SpringArmComponent|SetTargetArmLength (Variables|Default|GetCameraBoom) (Math|Float|Lerp 0.0 (Variables|Seeker|GetCameraDistanceAsSeeker) _newtrack_0))
                  (if (and (not (Pawn|IsPlayerControlled)) (Class|HideNSneakCPPCharacter|IsSeeker))
                    (Utilities|FlowControl|Delay (Variables|Misc.|GetDummyResetTime))
                    (CallFunction|TurnIntoHider (Variables|Character|GetCharacterMovement))))
                (:Finished
                  (goto _label)))))))
      (else
        (CallFunction|TurnIntoHider _charactermovement)
        (Timeline|CameraSwitch Reverse)))))

(event EventUpdatePowerUpIcon
  (bind _self self)
  ;[1 1 1] Power up icons
  ;;[1 1 1] Set power up icon
  (bind _asbp_hide_nsneak_cppcharacter (Utilities|Casting|CastToBP_HideNSneakCPPCharacter (Pawn|GetControlledPawn (Game|GetPlayerController 0))))
  (if (== _asbp_hide_nsneak_cppcharacter _self)
    (Default|SetPowerUpIcon (Variables|UI|GetUIWidget _self) (Class|HideNSneakCPPCharacter|GetCollectedPowerUpIcon))))

(event EventClearPowerUpIcon
  (bind _self self)
  ;[1 1 1] Power up icons
  ;;[1 1 1] Clear power up icon
  (bind _asbp_hide_nsneak_cppcharacter (Utilities|Casting|CastToBP_HideNSneakCPPCharacter (Pawn|GetControlledPawn (Game|GetPlayerController 0))))
  (if (== _asbp_hide_nsneak_cppcharacter _self)
    (Default|ClearPowerUpIcon (Variables|UI|GetUIWidget _self))))

(event Input|ActionEvents|InputActionActivateAbility
  (params (Key :type Key%20Structure :default "None"))
  (bind _returnvalue (Utilities|Time|GetGameTimeinSeconds))
  (bind _self self)
  (bind _returnvalue_2 (Transformation|GetActorLocation _self))
  ;[1 1 1] Player abilites
  (:Released
    (if (Class|HideNSneakCPPCharacter|IsSeeker)
      ;;[1 1 1] Seeker ability, Change Hiders material to one that can be seen through walls, reset back to original after delay
      (Math|Float|CompareFloat (Variables|Seeker|GetTimeWhenSeekerAbilityCanBeUsed) _returnvalue
        (:<
          (if (not (Variables|Seeker|GetUsingSeekerAbility)) ; Check to stop the UI from updating incorrectly
            (CallFunction|MakeHidersSeeableThroughWalls)
            (Utilities|FlowControl|Sequence
              (:then_0
                (Variables|Seeker|SetUsingSeekerAbility true))
              (:then_1
                (Utilities|FlowControl|Delay (Variables|Seeker|GetSeekerAbilityDuration))
                (CallFunction|SetBackHidersMaterial)
                (Utilities|FlowControl|Sequence
                  (:then_0
                    (Variables|Seeker|SetUsingSeekerAbility false))
                  (:then_1
                    (Variables|Seeker|SetTimeWhenSeekerAbilityCanBeUsed (+ (Utilities|Time|GetGameTimeinSeconds) (Variables|Seeker|GetSeekerAbilityCooldown))))))
              (:then_2
                (Variables|Seeker|SetTimeWhenSeekerAbilityStops (+ _returnvalue (Variables|Seeker|GetSeekerAbilityDuration))))))))
      (else
        ;;[1 1 1] Hider ability
        (if (Variables|Default|GetDecoyAvailible)
          (Utilities|FlowControl|Sequence
            (:then_0
              (Variables|Hider|SetHasUsedHiderAbility true))
            (:then_1
              (Variables|Hider|SetTimeWhenHiderAbilityCanBeUsed (+ (Utilities|Time|GetGameTimeinSeconds) (Variables|Default|GetDecoyCooldown)))
              (CallFunction|SpawnEmitter "/Game/Art/VFX/ParticleSystems/P_SmokePuff.P_SmokePuff" _returnvalue_2)
              (CallFunction|SpawnSound "/Game/Sounds/Powers/Powerups/38704__elanhickler__archi-sonar-05.38704__elanhickler__archi-sonar-05" _returnvalue_2)
              (Class|HideNSneakCPPCharacter|UseDecoyAbility)))
          (else
            (Variables|Hider|SetHasUsedHiderAbility false)))))))

(event Input|MouseEvents|RightMouseButton
  (params (Key :type Key%20Structure :default "None"))
  (bind _returnvalue (Game|GetPlayerController 0))
  (bind _uiwidget (Variables|UI|GetUIWidget))
  (bind _b_customizecontrols (Variables|/Game/Blueprints/Widgets/BPW_Player_UI.BPW_Player_UI_C|GetB_CustomizeControls _uiwidget))
  ;[1 1 1] Make it so the player can click on UI elements
  (:Released
    (if (Variables|Misc.|GetInputIsGameOnly)
      (Variables|/Script/Engine.PlayerController|SetbShowMouseCursor _returnvalue true)
      (Input|SetInputModeGameandUI _returnvalue _uiwidget "LockAlways" false)
      (Variables|Misc.|SetInputIsGameOnly false)
      (Widget|SetVisibility _b_customizecontrols "Visible")
      (else
        (Variables|/Script/Engine.PlayerController|SetbShowMouseCursor _returnvalue false)
        (Input|SetInputModeGameOnly _returnvalue)
        (Variables|Misc.|SetInputIsGameOnly true)
        (Widget|SetVisibility _b_customizecontrols "Hidden")))))

(event Input|KeyboardEvents|G
  (params (Key :type Key%20Structure :default "None"))
  ;[1 1 1] PING
  (:Pressed
    (CallFunction|ClientUpdatePingIcon "/Game/Blueprints/Widgets/Materials/Textures/Warning_Icon.Warning_Icon")
    (CallFunction|ClientPingAllPlayers 5.0)))

(event Input|KeyboardEvents|1
  (params (Key :type Key%20Structure :default "None"))
  ;[1 1 1] Moving platform interaction
  (:Pressed
    (if (Utilities|IsValid (Variables|Misc.|GetElevatorReference))
      (CallFunction|ClientStartElevator (Variables|Misc.|GetElevatorReference)))))

(fn ConstructionScript
  (bind _mesh (Variables|Character|GetMesh))
  ;[1 1 1] Setup dynamic material instance to change color during gameplay
  (bind _returnvalue (Rendering|Material|CreateDynamicMaterialInstance _mesh 0 (Rendering|Material|GetMaterial _mesh 0) "None" :!class /Script/Engine.PrimitiveComponent))
  (Variables|Misc.|SetPlayerMaterial _returnvalue))

(fn MakeHidersSeeableThroughWalls
  (Game|SpawnActorfromClass "/Game/Blueprints/ArtBlueprints/BP_SeekerPing.BP_SeekerPing_C" (Math|Conversions|ToTransform(Vector) (Transformation|GetActorLocation self)) "Undefined" 0 0)
  ;[1 1 1] For all Hiders, set their material to M_SeeThroughWalls
  (bind _outactors (Actor|GetAllActorsOfClass "/Game/Blueprints/BP_HideNSneakCPPCharacter.BP_HideNSneakCPPCharacter_C"))
  (for _array_element _outactors
    (if (not (Class|HideNSneakCPPCharacter|IsSeeker _array_element))
      (if (<= (Math|Vector|VectorLength (- (Transformation|GetActorLocation _array_element) (Transformation|GetActorLocation))) (Variables|Seeker|GetSekerAbilityRange))
        (Rendering|Material|SetMaterial (Variables|/Script/Engine.Character|GetMesh _array_element) 0 "/Game/Art/VFX/Shaders/MI_SeeThroughWalls.MI_SeeThroughWalls")))))

(fn SetBackHidersMaterial
  (bind _outactors (Actor|GetAllActorsOfClass "/Game/Blueprints/BP_HideNSneakCPPCharacter.BP_HideNSneakCPPCharacter_C"))
  (for _array_element _outactors
    (Rendering|Material|SetMaterial (Variables|/Script/Engine.Character|GetMesh _array_element) 0 (Variables|/Game/Blueprints/BP_HideNSneakCPPCharacter.BP_HideNSneakCPPCharacter_C|GetPlayerMaterial _array_element))))

(fn GetLocalPlayerUIWidget
  (bind _asbp_hide_nsneak_cppcharacter (Utilities|Casting|CastToBP_HideNSneakCPPCharacter (Pawn|GetControlledPawn (Game|GetPlayerController 0))))
  (return (Variables|/Game/Blueprints/BP_HideNSneakCPPCharacter.BP_HideNSneakCPPCharacter_C|GetUIWidget _asbp_hide_nsneak_cppcharacter)))

(fn SetPingIcon
  (params (InputPin :type Texture%202D%20Object%20Reference))
  (bind _uiwidget (CallFunction|GetLocalPlayerUIWidget))
  (if (.ReturnValue (Utilities|Map|Find (Variables|/Game/Blueprints/Widgets/BPW_Minimap.BPW_Minimap_C|GetPointsOfInterestByActors (Variables|/Game/Blueprints/Widgets/BPW_Player_UI.BPW_Player_UI_C|GetBPW_Minimap _uiwidget)) self))
    (Appearance|SetBrushfromTexture (Variables|/Game/Blueprints/Widgets/PointOfInterestWidget_BP.PointOfInterestWidget_BP_C|GetCustomImage (.Value (Utilities|Map|Find (Variables|/Game/Blueprints/Widgets/BPW_Minimap.BPW_Minimap_C|GetPointsOfInterestByActors (Variables|/Game/Blueprints/Widgets/BPW_Player_UI.BPW_Player_UI_C|GetBPW_Minimap _uiwidget)) self))) InputPin false)))

(fn TurnIntoSeeker
  (bind _mesh (Variables|Character|GetMesh))
  (bind _roundcontrollerinscene (Variables|Misc.|GetRoundControllerInScene))
  (bind _charactermovement (Variables|Character|GetCharacterMovement))
  (if (Utilities|IsValid _roundcontrollerinscene)
    (Class|RoundController|BPAddHidertoSeekerTeam _roundcontrollerinscene self)
    (Variables|/Script/Engine.CharacterMovementComponent|SetMaxWalkSpeed _charactermovement (Variables|Default|GetSeekerBaseSpeed))
    (Variables|Seeker|SetTimeWhenSeekerAbilityCanBeUsed 0.0)
    (Utilities|FlowControl|Sequence
      (:then_0
        (Class|SkeletalMeshComponent|SetAnimClass _mesh "/Game/Art/3D/Character/Animations/BP/Seeker_Anim_BP1.Seeker_Anim_BP1_C"))
      (:then_1
        (Rendering|Material|SetMaterial _mesh 0 "/Game/Art/3D/Character/Material/M_SeekerBody.M_SeekerBody"))
      (:then_2
        (Rendering|Material|SetMaterial _mesh 2 "/Game/Art/3D/Character/Material/M_Seeker_Face.M_Seeker_Face"))
      (:then_3
        (Rendering|SetVisibility (Variables|Default|GetSpotLight) true false))
      (:then_4
        (Rendering|SetVisibility (Variables|Default|GetSpotLight1) true false))
      (:then_5
        (return _charactermovement)))))

(fn TurnIntoHider
  (params (self3 :type Character%20Movement%20Component%20Object%20Reference))
  (bind _self self)
  (bind _mesh (Variables|Character|GetMesh))
  (bind _roundcontrollerinscene (Variables|Misc.|GetRoundControllerInScene))
  (if (and (Utilities|IsValid _roundcontrollerinscene) (not (Variables|Default|GetIsDecoy _self)))
    (Class|RoundController|BPAddHidertoHiderTeam _roundcontrollerinscene _self)
    (Variables|/Script/Engine.CharacterMovementComponent|SetMaxWalkSpeed self3 (Variables|Default|GetHiderBaseSpeed))
    (Variables|Hider|SetTimeWhenHiderAbilityCanBeUsed 0.0)
    (Utilities|FlowControl|Sequence
      (:then_0
        (Class|SkeletalMeshComponent|SetAnimClass _mesh "/Game/Art/3D/Character/Animations/BP/Hider_Anim_BP.Hider_Anim_BP_C"))
      (:then_1
        (Rendering|Material|SetMaterial _mesh 0 "/Game/Art/3D/Character/Material/M_HiderBody.M_HiderBody"))
      (:then_2
        (Rendering|Material|SetMaterial _mesh 2 "/Game/Art/3D/Character/Material/M_Hider_Face.M_Hider_Face"))
      (:then_3
        (Rendering|SetVisibility (Variables|Default|GetSpotLight) false false))
      (:then_4
        (Rendering|SetVisibility (Variables|Default|GetSpotLight1) false false)))))

(fn CheckifinTraining
  (bind _asbp_round_controller (Utilities|Casting|CastToBP_RoundController (Variables|Misc.|GetRoundControllerInScene)))
  (return (Variables|/Game/Blueprints/BP_RoundController.BP_RoundController_C|GetIsTraining _asbp_round_controller)))

(fn AddTaggerPoints
  (bind _roundcontrollerinscene (Variables|Misc.|GetRoundControllerInScene))
  (bind _whotaggedme (Variables|Default|GetWhoTaggedMe))
  (bind _whotaggedme_2 (Variables|Default|GetWhoTaggedMe))
  (bind _roundcontrollerinscene_2 (Variables|Misc.|GetRoundControllerInScene))
  (bind _scoremultiplier (Variables|/Script/HideNSneakUnreal.RoundController|GetScoreMultiplier _roundcontrollerinscene))
  (if (Utilities|IsValid (Variables|Default|GetWhoTaggedMe))
    (Development|PrintString "it worked")
    (if (>= (Utilities|Array|Length (Variables|/Script/HideNSneakUnreal.RoundController|GetPlayers (Variables|Misc.|GetRoundControllerInScene))) 3)
      (Class|HideNSneakCPPCharacter|ClientAddScore _whotaggedme_2 _whotaggedme_2 2 _scoremultiplier)
      (else
        (Class|HideNSneakCPPCharacter|ClientAddScore _whotaggedme _whotaggedme 1 _scoremultiplier)))
    (for _array_element (Variables|/Script/HideNSneakUnreal.RoundController|GetSeekers (Variables|Misc.|GetRoundControllerInScene))
      (Class|HideNSneakCPPCharacter|ClientAddScore _array_element _array_element (Variables|/Script/HideNSneakUnreal.RoundController|GetTagAssistPoint _roundcontrollerinscene_2) (Variables|/Script/HideNSneakUnreal.RoundController|GetScoreMultiplier _roundcontrollerinscene_2))
      (return))
    (else
      (Development|PrintString "it didnt work"))))