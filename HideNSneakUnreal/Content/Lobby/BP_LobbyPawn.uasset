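; BP_LobbyPawn is the lobby pawn that delivers chat messages to the local player's chat box.
; Client-prefixed events forward to ReceiveMessage and UpdateStat, which look up the pawn controlled by player controller 0 instead of using their own instance.
; ReceiveMessage updates that pawn's ChatBox when valid, while UpdateStat only performs the lookup and does not apply the stat.
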(event Custom|ClientReceiveMessage
  (params (Message :type Text))
  (CallFunction|ReceiveMessage Message))

(event Custom|ReceiveMessage
  (params (ReceivedMessage :type Text))
  (bind _localplayer (CallFunction|GetLocalPlayer))
  (Utilities|IsValid (Variables|BP_LobbyPawn_C|GetChatBox _localplayer)
    (:Is%20Valid
      (Default|UpdateChat (Variables|BP_LobbyPawn_C|GetChatBox _localplayer) ReceivedMessage))))

(event Custom|ClientUpdateStat
  (params (Index :type Integer) (UpdatedText :type Text))
  (CallFunction|UpdateStat Index UpdatedText))

(event Custom|Update%20Stat
  (params (Index :type Integer) (UpdatedStat :type Text))
  (CallFunction|GetLocalPlayer))

(fn ConstructionScript)

(fn GetLocalPlayer
  (bind _asbp_lobby_pawn (Utilities|Casting|CastToBP_LobbyPawn (Pawn|GetControlledPawn (Game|GetPlayerController 0))))
  (return _asbp_lobby_pawn))