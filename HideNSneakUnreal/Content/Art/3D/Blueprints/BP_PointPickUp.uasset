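; BP_PointPickUp is a looping animated pickup that reacts when the Hide N Sneak player character overlaps it.
; Overlap hides the mesh, disables collision, activates a nuts-and-bolts particle effect and destroys the actor after five seconds.
; Tick tracks the stored player's location and, when it changes, feeds it into the effect's PointAttractorPos parameter, so particles follow the player.
; No score is awarded here.
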(event OnComponentBeginOverlap(Collider)
  (params (OverlappedComponent :type Primitive%20Component%20Object%20Reference) (OtherActor :type Actor%20Object%20Reference) (OtherComp :type Primitive%20Component%20Object%20Reference) (OtherBodyIndex :type Integer) (bFromSweep :type Boolean) (SweepResult :type Hit%20Result%20Structure%20%28by%20ref%29))
  (bind _p_nutsnboltscollide (Variables|Default|GetP_NutsNBoltsCollide))
  (Utilities|FlowControl|Sequence
    (:then_0
      (bind _asbp_hide_nsneak_cppcharacter (Utilities|Casting|CastToBP_HideNSneakCPPCharacter OtherActor))
      (Utilities|FlowControl|Sequence
        (:then_0
          (Rendering|SetVisibility (Variables|Default|GetI_PointPickUp_anim) false false)
          (Collision|SetCollisionEnabled (Variables|Default|GetCollider) "NoCollision")
          (Components|Activation|Activate _p_nutsnboltscollide false)
          (Effects|Components|ParticleSystem|SetVectorParameter _p_nutsnboltscollide "PointAttractorPos" (stale _output_get))
          (Utilities|FlowControl|Delay 5.0)
          (Actor|DestroyActor))
        (:then_1
          (bind _output_get (Variables|Default|SetPlayerLocationOld (Transformation|GetActorLocation _asbp_hide_nsneak_cppcharacter))))))
    (:then_1
      (bind _output_get_2 (Variables|Default|SetPlayerVar OtherActor)))))

(event EventBeginPlay
  (Utilities|FlowControl|Sequence
    (:then_1
      (Components|Activation|Deactivate (Variables|Default|GetP_NutsNBoltsCollide)))
    (:then_2
      (Components|Animation|PlayAnimation (Variables|Default|GetI_PointPickUp_anim) "/Game/Art/3D/Interactable/Meshes/PointPickUp/I_PointPickUp_anim_Anim.I_PointPickUp_anim_Anim" true))
    (:then_3
      (Collision|SetCollisionEnabled (Variables|Default|GetCollider) "QueryAndPhysics"))))

(event EventTick
  (params (DeltaSeconds :type Float%20%28single-precision%29))
  (bind _playervar (Variables|Default|GetPlayerVar))
  (bind _rootcomponent (Variables|/Script/Engine.Actor|GetRootComponent _playervar))
  (bind _returnvalue (Transformation|GetWorldLocation _rootcomponent))
  (Utilities|Casting|CastToBP_HideNSneakCPPCharacter (stale OnComponentBeginOverlap(Collider) _output_get_2))
  (if (not (Math|Vector|Equal(Vector) _returnvalue (Variables|Default|GetPlayerLocationOld) 0.0001))
    (Variables|Default|SetPlayerLocationOld _returnvalue)
    (Effects|Components|ParticleSystem|SetVectorParameter (Variables|Default|GetP_NutsNBoltsCollide) "PointAttractorPos" (stale OnComponentBeginOverlap(Collider) _output_get))
    (Utilities|FlowControl|Delay 5.0)
    (Actor|DestroyActor)))

(fn ConstructionScript)